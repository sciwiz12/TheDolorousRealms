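; BP_Money is a money pickup that gambles with the player's currency when a BP_Character overlaps its Box component.
; A random roll at roughly even odds either adds to or subtracts from Currency on GI_Main, with the loss slightly larger than the gain.
; The total is changed directly on the game instance without clamping, and the actor destroys itself after a short delay.
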(event OnComponentBeginOverlap(Box)
  (params (OverlappedComponent :type Primitive%20Component%20Object%20Reference) (OtherActor :type Actor%20Object%20Reference) (OtherComp :type Primitive%20Component%20Object%20Reference) (OtherBodyIndex :type Integer) (bFromSweep :type Boolean) (SweepResult :type Hit%20Result%20Structure%20%28by%20ref%29))
  (Utilities|Casting|CastToBP_Character OtherActor)
  (bind _asgi_main (Utilities|Casting|CastToGI_Main (Game|GetGameInstance)))
  (Variables|Default|SetRandomValue (Math|Random|RandomIntegerinRange 0 50))
  (if (>= (Variables|Default|GetRandomValue) 25)
    (Variables|/Game/Blueprints/GI_Main.GI_Main_C|SetCurrency _asgi_main (+ (Variables|/Game/Blueprints/GI_Main.GI_Main_C|GetCurrency _asgi_main) 25))
    (else
      (Variables|/Game/Blueprints/GI_Main.GI_Main_C|SetCurrency _asgi_main (- (Variables|/Game/Blueprints/GI_Main.GI_Main_C|GetCurrency _asgi_main) 30))))
  (Utilities|FlowControl|Delay 0.2)
  (Actor|DestroyActor))

(fn ConstructionScript)