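; BP_LevelManager_CircleOne is the level manager for Circle One, handling player setup and camera height.
; On BeginPlay, BeginLevel resets the player camera and copies monster roster, inventory and stored monsters from GI_Main into the character and first BP_MonsterStorage.
; Tick moves the camera's relative height from an axis value, clamped to a range.
; EncounterBeasts and EncounterVirgil are empty event stubs.
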(event Custom|BeginLevel
  (bind _asbp_character (Utilities|Casting|CastToBP_Character (Game|GetPlayerCharacter 0)))
  (bind _output_get (Variables|Default|SetCharacter _asbp_character))
  (Transformation|SetRelativeLocation (Variables|/Game/Blueprints/Avatar/BP_Character.BP_Character_C|GetCamera _output_get) "15.832092, 0,1000.000000" false false)
  (bind _asgi_main (Utilities|Casting|CastToGI_Main (Game|GetGameInstance)))
  (bind _asbp_character_2 (Utilities|Casting|CastToBP_Character (Game|GetPlayerCharacter 0)))
  (Variables|/Game/Blueprints/MonsterAssets/BP_Component_MonsterRoster.BP_Component_MonsterRoster_C|SetMonsterRosterStruct (Variables|/Game/Blueprints/Avatar/BP_Character.BP_Character_C|GetMonsterRoster _asbp_character_2) (Variables|/Game/Blueprints/GI_Main.GI_Main_C|Getmonster%20struct%20roster _asgi_main))
  (Variables|/Game/Blueprints/InventorySystem/BP_Inventory.BP_Inventory_C|SetStructInventory (Variables|/Game/Blueprints/Avatar/BP_Character.BP_Character_C|GetBP_Inventory _asbp_character_2) (Variables|/Game/Blueprints/GI_Main.GI_Main_C|GetStruct%20Inventory _asgi_main))
  (bind _outactors (Actor|GetAllActorsOfClass "/Game/Blueprints/InventorySystem/BP_MonsterStorage.BP_MonsterStorage_C"))
  (Variables|/Game/Blueprints/InventorySystem/BP_MonsterStorage.BP_MonsterStorage_C|SetMonsters (Utilities|Array|Get(acopy) _outactors) (Variables|/Game/Blueprints/GI_Main.GI_Main_C|GetMonsters _asgi_main)))

(event Custom|EncounterBeasts)

(event Custom|EncounterVirgil)

(event EventBeginPlay
  (CallFunction|BeginLevel))

(event Collision|EventActorBeginOverlap
  (params (OtherActor :type Actor%20Object%20Reference)))

(event EventTick
  (params (DeltaSeconds :type Float%20%28single-precision%29))
  (bind _output_get (Variables|Default|SetNew%20Location%20Z (Math|Float|Clamp(Float) (+ (Variables|Default|GetNew%20Location%20Z) (* (Variables|Default|GetAxisValue) -1e+02)) 1e+02 3e+03)))
  (Transformation|SetRelativeLocation (Variables|/Game/Blueprints/Avatar/BP_Character.BP_Character_C|GetCamera (Variables|Default|GetCharacter)) (Math|Vector|MakeVector 15.832092 0.0 _output_get) false false))

(fn ConstructionScript)