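; Move executer component that carries out field moves (Cut, Strength, Dispel, Command, SuperSight, Climb) on referenced world objects.
; BeginPlay fills a name list, and DetermineMove uses a move's index in it to pick the handler.
; Handlers destroy obstacles, flag the player for boulder pushing, open gates of defeated guardians or toggle climbing.
; Dispel branches on illusion type to destroy, unfreeze, correct or reveal, though End Battle only casts.
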(event EventBeginPlay
  (Utilities|Array|Add (Variables|Default|GetMoveNames) "Cut")
  (Utilities|Array|Add (Variables|Default|GetMoveNames) "Strength")
  (Utilities|Array|Add (Variables|Default|GetMoveNames) "Dispel")
  (Utilities|Array|Add (Variables|Default|GetMoveNames) "Command")
  (Utilities|Array|Add (Variables|Default|GetMoveNames) "SuperSight")
  (Utilities|Array|Add (Variables|Default|GetMoveNames) "Climb"))

(event EventTick
  (params (DeltaSeconds :type Float%20%28single-precision%29)))

(fn ExecuteCut
  (Utilities|IsValid (Variables|Default|GetLog)
    (:Is%20Valid
      (Actor|DestroyActor (Variables|Default|GetLog)))))

(fn DetermineMove
  (params (Move :type Struct%20Move%20Structure))
  (switch int (Utilities|Array|FindItem (Variables|Default|GetMoveNames) (.MoveName (Utilities|Struct|BreakStruct_Move Move)))
    (:0
      (CallFunction|ExecuteCut))
    (:1
      (CallFunction|ExecuteStrength))
    (:2
      (CallFunction|ExecuteDispel))
    (:3
      (CallFunction|ExecuteCommand))
    (:4
      (CallFunction|ExecuteSuperSight))
    (:5
      (CallFunction|ExecuteClimb))))

(fn ExecuteStrength
  (Utilities|IsValid (Variables|Default|GetBoulder)
    (:Is%20Valid
      (bind _asbp_character (Utilities|Casting|CastToBP_Character (Game|GetPlayerCharacter 0)))
      (Variables|/Game/Blueprints/Avatar/BP_Character.BP_Character_C|SetMoveBoulder _asbp_character true))))

(fn ExecuteDispel
  (Utilities|IsValid (Variables|Default|GetIllusion)
    (:Is%20Valid
      (switch Utilities|FlowControl|Switch|SwitchonEnum_IllusionType (Variables|/Game/Blueprints/InventorySystem/MoveScrolls/BP_Illusion.BP_Illusion_C|GetIllusionType (Variables|Default|GetIllusion))
        (:NewEnumerator0
          (Development|PrintString "Illusion Not Set"))
        (:NewEnumerator1
          (Actor|DestroyActor (Variables|Default|GetIllusion)))
        (:NewEnumerator2
          (Utilities|Casting|CastToBP_Illusion_FalseEnemy (Variables|Default|GetIllusion)))
        (:NewEnumerator3
          (bind _asbp_illusion_freeze (Utilities|Casting|CastToBP_Illusion_Freeze (Variables|Default|GetIllusion)))
          (Default|Unfreeze _asbp_illusion_freeze))
        (:NewEnumerator4
          (bind _asbp_illusion_reverse (Utilities|Casting|CastToBP_Illusion_Reverse (Variables|Default|GetIllusion)))
          (Default|CorrectMovement _asbp_illusion_reverse))
        (:NewEnumerator5
          (bind _asbp_illusion_invisible_bridge (Utilities|Casting|CastToBP_Illusion_InvisibleBridge (Variables|Default|GetIllusion)))
          (Development|SetHiddeninGame (Variables|/Game/Blueprints/InventorySystem/MoveScrolls/BP_Illusion_InvisibleBridge.BP_Illusion_InvisibleBridge_C|GetPaperSprite _asbp_illusion_invisible_bridge) false false))))))

(fn ExecuteCommand
  (bind _gate (Variables|Default|GetGate))
  (bind _gate_guardian (Variables|Default|GetGate%20Guardian))
  (Utilities|IsValid _gate_guardian
    (:Is%20Valid
      (Default|CheckifDeafeated _gate_guardian)
      (if (Variables|/Game/Blueprints/NPCs/BP_NPC_GateGuardian.BP_NPC_GateGuardian_C|GetIsDefeated _gate_guardian)
        (Utilities|IsValid _gate
          (:Is%20Valid
            (Default|DestroyDoor _gate)))))))

(fn ExecuteSuperSight
  (Utilities|IsValid (Variables|Default|GetSuperSight)
    (:Is%20Valid
      (Actor|DestroyActor (Variables|Default|GetSuperSight)))))

(fn ExecuteClimb
  (bind _climb (Variables|Default|GetClimb))
  (Utilities|IsValid _climb
    (:Is%20Valid
      (Utilities|FlowControl|FlipFlop
        (:A
          (Variables|/Game/Blueprints/BP_Climb.BP_Climb_C|SetIsClimbing _climb true)
          (Default|Climb _climb))
        (:B
          (Variables|/Game/Blueprints/BP_Climb.BP_Climb_C|SetIsClimbing _climb false))))
    (:Is%20Not%20Valid
      (Development|PrintString "IsnotValid"))))

(fn Moveboulder
  (Default|MoveBoulder (Variables|Default|GetBoulder)))