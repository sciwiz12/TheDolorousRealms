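; Pushable boulder that slides away from the player along a single world axis.
; An overlap box marks the player in range and registers the boulder with the character's BPComponentMoveExecuter; two others choose the axis (XOnly moves along Y, YOnly along X).
; MoveBoulder enables movement, then Tick offsets the actor by a fixed unswept step, showing Niagara dust, until a frame counter reaches Threshold.
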(event OnComponentBeginOverlap(Box1)
  (params (OverlappedComponent :type Primitive%20Component%20Object%20Reference) (OtherActor :type Actor%20Object%20Reference) (OtherComp :type Primitive%20Component%20Object%20Reference) (OtherBodyIndex :type Integer) (bFromSweep :type Boolean) (SweepResult :type Hit%20Result%20Structure%20%28by%20ref%29))
  (Utilities|Casting|CastToBP_Character OtherActor)
  (Variables|Default|SetXOnly true)
  (Variables|Default|SetYOnly false))

(event OnComponentBeginOverlap(Box)
  (params (OverlappedComponent :type Primitive%20Component%20Object%20Reference) (OtherActor :type Actor%20Object%20Reference) (OtherComp :type Primitive%20Component%20Object%20Reference) (OtherBodyIndex :type Integer) (bFromSweep :type Boolean) (SweepResult :type Hit%20Result%20Structure%20%28by%20ref%29))
  (bind _asbp_character (Utilities|Casting|CastToBP_Character OtherActor))
  (Variables|Default|SetInRange true)
  (Variables|Default|SetAs%20BP%20Character _asbp_character)
  (Variables|/Game/Blueprints/Moves/BP_Component_MoveExecuter.BP_Component_MoveExecuter_C|SetBoulder (Variables|/Game/Blueprints/Avatar/BP_Character.BP_Character_C|GetBP_Component_MoveExecuter (Variables|Default|GetAs%20BP%20Character)) self))

(event OnComponentEndOverlap(Box)
  (params (OverlappedComponent :type Primitive%20Component%20Object%20Reference) (OtherActor :type Actor%20Object%20Reference) (OtherComp :type Primitive%20Component%20Object%20Reference) (OtherBodyIndex :type Integer))
  (Utilities|Casting|CastToBP_Character OtherActor)
  (Variables|Default|SetInRange false))

(event OnComponentBeginOverlap(Sphere)
  (params (OverlappedComponent :type Primitive%20Component%20Object%20Reference) (OtherActor :type Actor%20Object%20Reference) (OtherComp :type Primitive%20Component%20Object%20Reference) (OtherBodyIndex :type Integer) (bFromSweep :type Boolean) (SweepResult :type Hit%20Result%20Structure%20%28by%20ref%29)))

(event OnComponentBeginOverlap(Box2)
  (params (OverlappedComponent :type Primitive%20Component%20Object%20Reference) (OtherActor :type Actor%20Object%20Reference) (OtherComp :type Primitive%20Component%20Object%20Reference) (OtherBodyIndex :type Integer) (bFromSweep :type Boolean) (SweepResult :type Hit%20Result%20Structure%20%28by%20ref%29))
  (Utilities|Casting|CastToBP_Character OtherActor)
  (Variables|Default|SetYOnly true)
  (Variables|Default|SetXOnly false))

(event EventTick
  (params (DeltaSeconds :type Float%20%28single-precision%29))
  (bind _returnvalue (Game|GetPlayerCharacter 0))
  (bind _returnvalue_2 (Transformation|GetActorLocation))
  (bind _returnvalue_3 (Game|GetPlayerCharacter 0))
  (bind _returnvalue_4 (Transformation|GetActorLocation))
  (bind _returnvalue_5 (Transformation|GetActorLocation _returnvalue))
  (bind _returnvalue_6 (Transformation|GetActorLocation _returnvalue_3))
  (bind _returnvalue_7 (Math|Vector|GetUnitDirection(Vector) (Math|Vector|MakeVector (.x _returnvalue_4) (.y _returnvalue_6) (.z _returnvalue_4)) (Math|Vector|MakeVector (.x _returnvalue_4) (.y _returnvalue_4) (.z _returnvalue_4))))
  (bind _returnvalue_8 (Math|Vector|GetUnitDirection(Vector) (Math|Vector|MakeVector (.x _returnvalue_5) (.y _returnvalue_2) (.z _returnvalue_2)) (Math|Vector|MakeVector (.x _returnvalue_2) (.y _returnvalue_2) (.z _returnvalue_2))))
  (Rendering|SetVisibility (Variables|Default|GetNS_boulderDust) false false)
  (if (Variables|Default|GetInRange)
    (if (Variables|Default|GetMoveEnable)
      (if (Variables|Default|GetXOnly)
        (Transformation|AddActorWorldOffset (Math|Vector|Lerp(Vector) _returnvalue_7 (* _returnvalue_7 2.5) 1.0))
        (Rendering|SetVisibility (Variables|Default|GetNS_boulderDust) true false)
        (bind _result (Math|Integer|IncrementInt (Variables|Default|GetCounter))
          (:%20%20
            (Variables|Default|SetCounter _result)
            (if (>= (Variables|Default|GetCounter) (Variables|Default|GetThreshold))
              (Variables|Default|SetMoveEnable false)
              (Variables|Default|SetCounter 0))))
        (elif (Variables|Default|GetYOnly)
          (Transformation|AddActorWorldOffset (Math|Vector|Lerp(Vector) _returnvalue_8 (* _returnvalue_8 2.5) 1.0))
          (bind _result_2 (Math|Integer|IncrementInt (Variables|Default|GetCounter))
            (:%20%20
              (Variables|Default|SetCounter _result_2)
              (Rendering|SetVisibility (Variables|Default|GetNS_boulderDust) true false)
              (if (>= (Variables|Default|GetCounter) (Variables|Default|GetThreshold))
                (Variables|Default|SetMoveEnable false)
                (Variables|Default|SetCounter 0)))))))))

(fn ConstructionScript)

(fn MoveBoulder
  (Variables|Default|SetMoveEnable true)
  (Development|PrintString "ISWORKING 
"))