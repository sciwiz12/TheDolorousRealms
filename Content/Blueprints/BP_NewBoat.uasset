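; BP_NewBoat is a drivable boat that moves along its forward vector on Move Up and yaws on Move Right.
; Its BoatSphere overlap sets IsNearBoat on the player controller while a BP_Character is inside.
; Two seconds after BeginPlay, it copies the monster roster from GI_Main into its roster component and prints the second monster's name on screen.
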(event OnComponentBeginOverlap(BoatSphere)
  (params (OverlappedComponent :type Primitive%20Component%20Object%20Reference) (OtherActor :type Actor%20Object%20Reference) (OtherComp :type Primitive%20Component%20Object%20Reference) (OtherBodyIndex :type Integer) (bFromSweep :type Boolean) (SweepResult :type Hit%20Result%20Structure%20%28by%20ref%29))
  (Utilities|Casting|CastToBP_Character OtherActor)
  (bind _asbp_controller_character (Utilities|Casting|CastToBP_Controller_Character (Game|GetPlayerController 0)))
  (Variables|/Game/Blueprints/Avatar/BP_Controller_Character.BP_Controller_Character_C|SetIsNearBoat _asbp_controller_character true))

(event OnComponentEndOverlap(BoatSphere)
  (params (OverlappedComponent :type Primitive%20Component%20Object%20Reference) (OtherActor :type Actor%20Object%20Reference) (OtherComp :type Primitive%20Component%20Object%20Reference) (OtherBodyIndex :type Integer))
  (Utilities|Casting|CastToBP_Character OtherActor)
  (bind _asbp_controller_character (Utilities|Casting|CastToBP_Controller_Character (Game|GetPlayerController 0)))
  (Variables|/Game/Blueprints/Avatar/BP_Controller_Character.BP_Controller_Character_C|SetIsNearBoat _asbp_controller_character false))

(event EventBeginPlay
  (Utilities|FlowControl|Delay 2.0)
  (bind _asgi_main (Utilities|Casting|CastToGI_Main (Game|GetGameInstance)))
  (bind _output_get (Variables|/Game/Blueprints/MonsterAssets/BP_Component_MonsterRoster.BP_Component_MonsterRoster_C|SetMonsterRosterStruct (Variables|Default|GetBP_Component_MonsterRoster) (Variables|/Game/Blueprints/GI_Main.GI_Main_C|Getmonster%20struct%20roster _asgi_main)))
  (Development|PrintString (.name (.MonsterDetails (Utilities|Struct|BreakStruct_Monster (.Monster_2 (Utilities|Struct|BreakStruct_MonsterRoster _output_get))))) true true "(R=0.000000,G=0.660000,B=1.000000,A=1.000000)" 1e+01))

(event Input|AxisEvents|InputAxisMoveUp
  (params (AxisValue :type Float%20%28single-precision%29))
  ;[1 1 1] BoatMovement
  (Pawn|Input|AddMovementInput (Math|Vector|GetForwardVector (Transformation|GetActorRotation)) AxisValue true))

(event Input|AxisEvents|InputAxisMoveRight
  (params (AxisValue :type Float%20%28single-precision%29))
  ;[1 1 1] BoatMovement
  (Class|Actor|AddActorWorldRotation (Math|Rotator|MakeRotator 0.0 0.0 AxisValue)))

(fn ConstructionScript)