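; BP_RouteNameTrigger is a trigger actor that briefly shows a route name on screen when the player character enters it.
; On overlap by a BP_Character, it creates a GUI_RouteName widget for player 0, passes in its RouteName and adds it to the viewport.
; The widget is removed after a short delay, and a search for existing top-level instances prevents stacking a second one while one is showing.
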(event OnComponentBeginOverlap(CollisionComponent)
  (params (OverlappedComponent :type Primitive%20Component%20Object%20Reference) (OtherActor :type Actor%20Object%20Reference) (OtherComp :type Primitive%20Component%20Object%20Reference) (OtherBodyIndex :type Integer) (bFromSweep :type Boolean) (SweepResult :type Hit%20Result%20Structure%20%28by%20ref%29))
  (Utilities|Casting|CastToBP_Character OtherActor)
  (bind _foundwidgets (Widget|GetAllWidgetsOfClass "/Game/Blueprints/GUIs/GUI_RouteName.GUI_RouteName_C" true))
  (Utilities|IsValid (Utilities|Array|Get(acopy) _foundwidgets)
    (:Is%20Not%20Valid
      (bind _returnvalue (UserInterface|CreateWidget "/Game/Blueprints/GUIs/GUI_RouteName.GUI_RouteName_C" (Game|GetPlayerController 0)))
      (Variables|Default|SetRouteWidget _returnvalue)
      (Variables|/Game/Blueprints/GUIs/GUI_RouteName.GUI_RouteName_C|SetRouteName (Variables|Default|GetRouteWidget) (Variables|Default|GetRouteName))
      (UserInterface|Viewport|AddtoViewport (Variables|Default|GetRouteWidget) 0)
      (Utilities|FlowControl|Delay 5.0)
      (Widget|RemovefromParent (Variables|Default|GetRouteWidget)))))

(event EventBeginPlay)

(event Collision|EventActorBeginOverlap
  (params (OtherActor :type Actor%20Object%20Reference)))

(event EventTick
  (params (DeltaSeconds :type Float%20%28single-precision%29)))

(fn ConstructionScript)