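; Component that holds the player's six-slot monster party and handles XP, leveling, evolution, healing and ID assignment.
; RunThroughRoster splits battle XP among monsters flagged as Battled, levels them up with base-stat growth, then clears the flags.
; Reaching the evolution threshold on level-up opens a GUI_Evolve widget unless one already exists.
; Monsters live in a roster struct edited by reference, mirrored into MonsterArray by SetOrder, which also stamps slot order.
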(event EventBeginPlay)

(event EventTick
  (params (DeltaSeconds :type Float%20%28single-precision%29)))

(fn CheckEvolution
  (params (Monster :type Struct%20Monster%20Structure))
  (LocalVariables|SetMonLocal Monster)
  (if (and (Utilities|IsValidClass (.EvolutionReference (Utilities|Struct|BreakStruct_Evolution (.Evolutions (Utilities|Struct|BreakStruct_LevelXP (.LevelandXP (Utilities|Struct|BreakStruct_Monster (LocalVariables|GetMonLocal)))))))) (!= (.EvolutionReference (Utilities|Struct|BreakStruct_Evolution (.Evolutions (Utilities|Struct|BreakStruct_LevelXP (.LevelandXP (Utilities|Struct|BreakStruct_Monster (LocalVariables|GetMonLocal))))))) (.ClassReference (Utilities|Struct|BreakStruct_MonsterDetails (.MonsterDetails (Utilities|Struct|BreakStruct_Monster (LocalVariables|GetMonLocal)))))))
    (if (>= (.Level (Utilities|Struct|BreakStruct_LevelXP (.LevelandXP (Utilities|Struct|BreakStruct_Monster (LocalVariables|GetMonLocal))))) (.LevelThreshold (Utilities|Struct|BreakStruct_Evolution (.Evolutions (Utilities|Struct|BreakStruct_LevelXP (.LevelandXP (Utilities|Struct|BreakStruct_Monster (LocalVariables|GetMonLocal))))))))
      (bind _foundwidgets (Widget|GetAllWidgetsOfClass "/Game/Blueprints/GUIs/GUI_Evolve.GUI_Evolve_C" false))
      (Utilities|IsValid (Utilities|Array|Get(acopy) _foundwidgets)
        (:Is%20Not%20Valid
          (bind _outputmon (CallFunction|Evolve (LocalVariables|GetMonLocal)))
          (LocalVariables|SetMonLocal _outputmon)))))
  (return (LocalVariables|GetMonLocal)))

(fn LevelUp
  (params (Monster :type Struct%20Monster%20Structure))
  (LocalVariables|SetMonLocal Monster)
  (bind _result (Math|Integer|IncrementInt (.Level (Utilities|Struct|BreakStruct_LevelXP (.LevelandXP (Utilities|Struct|BreakStruct_Monster (LocalVariables|GetMonLocal))))))
    (:%20%20
      (|SetBy-RefVar (.Level (Utilities|Struct|BreakStruct_LevelXP (.LevelandXP (Utilities|Struct|BreakStruct_Monster (LocalVariables|GetMonLocal))))) _result)
      (|SetBy-RefVar (.XPtoLevelUp (Utilities|Struct|BreakStruct_LevelXP (.LevelandXP (Utilities|Struct|BreakStruct_Monster (LocalVariables|GetMonLocal))))) (Math|Conversions|ToFloat(Integer) (* (.Level (Utilities|Struct|BreakStruct_LevelXP (.LevelandXP (Utilities|Struct|BreakStruct_Monster (LocalVariables|GetMonLocal))))) 10)))
      (|SetBy-RefVar (.Stats (Utilities|Struct|BreakStruct_Monster (LocalVariables|GetMonLocal))) (Utilities|Struct|MakeStruct_Stats (+ (.Health (Utilities|Struct|BreakStruct_Stats (.Stats (Utilities|Struct|BreakStruct_Monster (LocalVariables|GetMonLocal))))) (Math|Conversions|ToFloat(Integer) (+ (/ (.Level (Utilities|Struct|BreakStruct_LevelXP (.LevelandXP (Utilities|Struct|BreakStruct_Monster (LocalVariables|GetMonLocal))))) 10) (Math|Float|Truncate (* (.Factor (Utilities|Struct|BreakStruct_Stats_Base (.BaseStats (Utilities|Struct|BreakStruct_Monster (LocalVariables|GetMonLocal))))) (.Health (Utilities|Struct|BreakStruct_Stats_Base (.BaseStats (Utilities|Struct|BreakStruct_Monster (LocalVariables|GetMonLocal)))))))))) (+ (.TotalHealth (Utilities|Struct|BreakStruct_Stats (.Stats (Utilities|Struct|BreakStruct_Monster (LocalVariables|GetMonLocal))))) (Math|Conversions|ToFloat(Integer) (+ (/ (.Level (Utilities|Struct|BreakStruct_LevelXP (.LevelandXP (Utilities|Struct|BreakStruct_Monster (LocalVariables|GetMonLocal))))) 10) (Math|Float|Truncate (* (.Factor (Utilities|Struct|BreakStruct_Stats_Base (.BaseStats (Utilities|Struct|BreakStruct_Monster (LocalVariables|GetMonLocal))))) (.TotalHealth (Utilities|Struct|BreakStruct_Stats_Base (.BaseStats (Utilities|Struct|BreakStruct_Monster (LocalVariables|GetMonLocal)))))))))) (+ (.Speed (Utilities|Struct|BreakStruct_Stats (.Stats (Utilities|Struct|BreakStruct_Monster (LocalVariables|GetMonLocal))))) (+ (/ (.Level (Utilities|Struct|BreakStruct_LevelXP (.LevelandXP (Utilities|Struct|BreakStruct_Monster (LocalVariables|GetMonLocal))))) 10) (Math|Float|Truncate (* (.Speed (Utilities|Struct|BreakStruct_Stats_Base (.BaseStats (Utilities|Struct|BreakStruct_Monster (LocalVariables|GetMonLocal))))) (.Factor (Utilities|Struct|BreakStruct_Stats_Base (.BaseStats (Utilities|Struct|BreakStruct_Monster (LocalVariables|GetMonLocal))))))))) (+ (.Attack (Utilities|Struct|BreakStruct_Stats (.Stats (Utilities|Struct|BreakStruct_Monster (LocalVariables|GetMonLocal))))) (+ (/ (.Level (Utilities|Struct|BreakStruct_LevelXP (.LevelandXP (Utilities|Struct|BreakStruct_Monster (LocalVariables|GetMonLocal))))) 10) (Math|Float|Truncate (* (.Attack (Utilities|Struct|BreakStruct_Stats_Base (.BaseStats (Utilities|Struct|BreakStruct_Monster (LocalVariables|GetMonLocal))))) (.Factor (Utilities|Struct|BreakStruct_Stats_Base (.BaseStats (Utilities|Struct|BreakStruct_Monster (LocalVariables|GetMonLocal))))))))) (+ (.SpecialAttack (Utilities|Struct|BreakStruct_Stats (.Stats (Utilities|Struct|BreakStruct_Monster (LocalVariables|GetMonLocal))))) (+ (/ (.Level (Utilities|Struct|BreakStruct_LevelXP (.LevelandXP (Utilities|Struct|BreakStruct_Monster (LocalVariables|GetMonLocal))))) 10) (Math|Float|Truncate (* (.SpecialAttack (Utilities|Struct|BreakStruct_Stats_Base (.BaseStats (Utilities|Struct|BreakStruct_Monster (LocalVariables|GetMonLocal))))) (.Factor (Utilities|Struct|BreakStruct_Stats_Base (.BaseStats (Utilities|Struct|BreakStruct_Monster (LocalVariables|GetMonLocal))))))))) (+ (.Defense (Utilities|Struct|BreakStruct_Stats (.Stats (Utilities|Struct|BreakStruct_Monster (LocalVariables|GetMonLocal))))) (+ (/ (.Level (Utilities|Struct|BreakStruct_LevelXP (.LevelandXP (Utilities|Struct|BreakStruct_Monster (LocalVariables|GetMonLocal))))) 10) (Math|Float|Truncate (* (.Defense (Utilities|Struct|BreakStruct_Stats_Base (.BaseStats (Utilities|Struct|BreakStruct_Monster (LocalVariables|GetMonLocal))))) (.Factor (Utilities|Struct|BreakStruct_Stats_Base (.BaseStats (Utilities|Struct|BreakStruct_Monster (LocalVariables|GetMonLocal))))))))) (+ (.SpecialDefense (Utilities|Struct|BreakStruct_Stats (.Stats (Utilities|Struct|BreakStruct_Monster (LocalVariables|GetMonLocal))))) (+ (/ (.Level (Utilities|Struct|BreakStruct_LevelXP (.LevelandXP (Utilities|Struct|BreakStruct_Monster (LocalVariables|GetMonLocal))))) 10) (Math|Float|Truncate (* (.SpecialDefense (Utilities|Struct|BreakStruct_Stats_Base (.BaseStats (Utilities|Struct|BreakStruct_Monster (LocalVariables|GetMonLocal))))) (.Factor (Utilities|Struct|BreakStruct_Stats_Base (.BaseStats (Utilities|Struct|BreakStruct_Monster (LocalVariables|GetMonLocal))))))))) (+ (.Evasion (Utilities|Struct|BreakStruct_Stats (.Stats (Utilities|Struct|BreakStruct_Monster (LocalVariables|GetMonLocal))))) (+ (/ (.Level (Utilities|Struct|BreakStruct_LevelXP (.LevelandXP (Utilities|Struct|BreakStruct_Monster (LocalVariables|GetMonLocal))))) 10) (Math|Float|Truncate (* (.Evasion (Utilities|Struct|BreakStruct_Stats_Base (.BaseStats (Utilities|Struct|BreakStruct_Monster (LocalVariables|GetMonLocal))))) (.Factor (Utilities|Struct|BreakStruct_Stats_Base (.BaseStats (Utilities|Struct|BreakStruct_Monster (LocalVariables|GetMonLocal)))))))))))
      (bind _outputmonster (CallFunction|CheckEvolution (LocalVariables|GetMonLocal)))
      (LocalVariables|SetMonLocal _outputmonster)
      (return (LocalVariables|GetMonLocal)))))

(fn IncreaseXP
  (params (Monster :type Struct%20Monster%20Structure))
  (LocalVariables|SetMonLocal Monster)
  (|SetBy-RefVar (.XP (Utilities|Struct|BreakStruct_LevelXP (.LevelandXP (Utilities|Struct|BreakStruct_Monster (LocalVariables|GetMonLocal))))) (+ (.XP (Utilities|Struct|BreakStruct_LevelXP (.LevelandXP (Utilities|Struct|BreakStruct_Monster (LocalVariables|GetMonLocal))))) (/ (Variables|Default|GetTotal%20XP) (Math|Conversions|ToFloat(Integer) (Variables|Default|GetNumWhoBattled)))))
  (if (>= (.XP (Utilities|Struct|BreakStruct_LevelXP (.LevelandXP (Utilities|Struct|BreakStruct_Monster (LocalVariables|GetMonLocal))))) (.XPtoLevelUp (Utilities|Struct|BreakStruct_LevelXP (.LevelandXP (Utilities|Struct|BreakStruct_Monster (LocalVariables|GetMonLocal))))))
    (|SetBy-RefVar (.XP (Utilities|Struct|BreakStruct_LevelXP (.LevelandXP (Utilities|Struct|BreakStruct_Monster (LocalVariables|GetMonLocal))))) 0.0)
    (bind _outputmon (CallFunction|LevelUp (LocalVariables|GetMonLocal)))
    (LocalVariables|SetMonLocal _outputmon))
  (return (LocalVariables|GetMonLocal)))

(fn Evolve
  (params (Monster :type Struct%20Monster%20Structure))
  (LocalVariables|SetMonLocal Monster)
  (bind _returnvalue (UserInterface|CreateWidget "/Game/Blueprints/GUIs/GUI_Evolve.GUI_Evolve_C" (Game|GetPlayerController 0)))
  (UserInterface|Viewport|AddtoViewport _returnvalue 0)
  (Variables|/Game/Blueprints/GUIs/GUI_Evolve.GUI_Evolve_C|SetMonster _returnvalue (LocalVariables|GetMonLocal))
  (return (LocalVariables|GetMonLocal)))

(fn RunThroughRoster
  (params (TotalXP :type Float%20%28single-precision%29))
  (bind _monsterrosterstruct (Variables|Default|GetMonsterRosterStruct))
  (bind _monsterrosterstruct_2 (Variables|Default|GetMonsterRosterStruct))
  (bind _monsterrosterstruct_3 (Variables|Default|GetMonsterRosterStruct))
  (bind _monsterrosterstruct_4 (Variables|Default|GetMonsterRosterStruct))
  (bind _monsterrosterstruct_5 (Variables|Default|GetMonsterRosterStruct))
  (bind _monsterrosterstruct_6 (Variables|Default|GetMonsterRosterStruct))
  (Variables|Default|SetTotal%20XP TotalXP)
  (for _array_element (Variables|Default|GetMonsterArray)
    (if (.Battled (Utilities|Struct|BreakStruct_Monster _array_element))
      (bind _result (Math|Integer|IncrementInt (Variables|Default|GetNumWhoBattled))
        (:%20%20
          (Variables|Default|SetNumWhoBattled _result)))))
  (bind _outputmon (CallFunction|CheckMonValid (.monster_1 _monsterrosterstruct_5)))
  (|SetBy-RefVar (.monster_1 _monsterrosterstruct_5) _outputmon)
  (bind _outputmon_2 (CallFunction|CheckMonValid (.monster_2 _monsterrosterstruct_6)))
  (|SetBy-RefVar (.monster_2 _monsterrosterstruct_6) _outputmon_2)
  (bind _outputmon_3 (CallFunction|CheckMonValid (.monster_3 _monsterrosterstruct_2)))
  (|SetBy-RefVar (.monster_3 _monsterrosterstruct_2) _outputmon_3)
  (bind _outputmon_4 (CallFunction|CheckMonValid (.monster_4 _monsterrosterstruct_3)))
  (|SetBy-RefVar (.monster_4 _monsterrosterstruct_3) _outputmon_4)
  (bind _outputmon_5 (CallFunction|CheckMonValid (.monster_5 _monsterrosterstruct_4)))
  (|SetBy-RefVar (.monster_5 _monsterrosterstruct_4) _outputmon_5)
  (bind _outputmon_6 (CallFunction|CheckMonValid (.monster_6 _monsterrosterstruct)))
  (|SetBy-RefVar (.monster_6 _monsterrosterstruct) _outputmon_6)
  (Variables|Default|SetNumWhoBattled 0)
  (CallFunction|SetAllBattled false))

(fn CheckMonValid
  (params (InputPin :type Struct%20Monster%20Structure))
  (LocalVariables|SetMonLocal InputPin)
  (if (Utilities|Enum|NotEqual(Enum) (.Name (Utilities|Struct|BreakStruct_MonsterDetails (.MonsterDetails (Utilities|Struct|BreakStruct_Monster (LocalVariables|GetMonLocal))))) "")
    (if (.Battled (Utilities|Struct|BreakStruct_Monster (LocalVariables|GetMonLocal)))
      (bind _outputmon (CallFunction|IncreaseXP (LocalVariables|GetMonLocal)))
      (LocalVariables|SetMonLocal _outputmon)
      (else
        (Development|PrintString (Utilities|String|ToString(Integer) (Variables|Default|GetNumWhoBattled))))))
  (return (LocalVariables|GetMonLocal)))

(fn SetOrder
  (bind _monsterrosterstruct (Variables|Default|GetMonsterRosterStruct))
  (|SetBy-RefVar (.PlaceInRoster (Utilities|Struct|BreakStruct_MonsterDetails (.MonsterDetails (Utilities|Struct|BreakStruct_Monster (.monster_1 (Variables|Default|GetMonsterRosterStruct)))))) "NewEnumerator0")
  (|SetBy-RefVar (.PlaceInRoster (Utilities|Struct|BreakStruct_MonsterDetails (.MonsterDetails (Utilities|Struct|BreakStruct_Monster (.monster_2 (Variables|Default|GetMonsterRosterStruct)))))) "NewEnumerator1")
  (|SetBy-RefVar (.PlaceInRoster (Utilities|Struct|BreakStruct_MonsterDetails (.MonsterDetails (Utilities|Struct|BreakStruct_Monster (.monster_3 (Variables|Default|GetMonsterRosterStruct)))))) "NewEnumerator2")
  (|SetBy-RefVar (.PlaceInRoster (Utilities|Struct|BreakStruct_MonsterDetails (.MonsterDetails (Utilities|Struct|BreakStruct_Monster (.monster_4 (Variables|Default|GetMonsterRosterStruct)))))) "NewEnumerator3")
  (|SetBy-RefVar (.PlaceInRoster (Utilities|Struct|BreakStruct_MonsterDetails (.MonsterDetails (Utilities|Struct|BreakStruct_Monster (.monster_5 (Variables|Default|GetMonsterRosterStruct)))))) "NewEnumerator4")
  (|SetBy-RefVar (.PlaceInRoster (Utilities|Struct|BreakStruct_MonsterDetails (.MonsterDetails (Utilities|Struct|BreakStruct_Monster (.monster_6 (Variables|Default|GetMonsterRosterStruct)))))) "NewEnumerator5")
  (CallFunction|AddtoArray (.monster_1 _monsterrosterstruct) (.monster_2 _monsterrosterstruct) (.monster_3 _monsterrosterstruct) (.monster_4 _monsterrosterstruct) (.monster_5 _monsterrosterstruct) (.monster_6 _monsterrosterstruct)))

(fn AssignUniqueID
  (params (Struct_Monster :type Struct%20Monster%20Structure%20%28by%20ref%29))
  (bind _monsterdetails (Utilities|Struct|BreakStruct_Monster Struct_Monster))
  (bind _uniqueid (Utilities|Struct|BreakStruct_MonsterDetails _monsterdetails))
  (if (<= _uniqueid 9999.0)
    (|SetBy-RefVar _uniqueid (Math|Random|RandomFloatinRange 1e+03 1e+04))))

(fn AssignPartyIDs
  (bind _monsterrosterstruct (Variables|Default|GetMonsterRosterStruct))
  (CallFunction|AssignUniqueID (.monster_1 _monsterrosterstruct))
  (CallFunction|AssignUniqueID (.monster_2 _monsterrosterstruct))
  (CallFunction|AssignUniqueID (.monster_3 _monsterrosterstruct))
  (CallFunction|AssignUniqueID (.monster_4 _monsterrosterstruct))
  (CallFunction|AssignUniqueID (.monster_5 _monsterrosterstruct))
  (CallFunction|AssignUniqueID (.monster_6 _monsterrosterstruct)))

(fn AddtoArray
  (params (NewItem :type Struct%20Monster%20Structure%20%28by%20ref%29) (NewItem2 :type Struct%20Monster%20Structure%20%28by%20ref%29) (NewItem3 :type Struct%20Monster%20Structure%20%28by%20ref%29) (NewItem4 :type Struct%20Monster%20Structure%20%28by%20ref%29) (NewItem5 :type Struct%20Monster%20Structure%20%28by%20ref%29) (NewItem6 :type Struct%20Monster%20Structure%20%28by%20ref%29))
  (bind _monsterarray (Variables|Default|GetMonsterArray))
  (Utilities|Array|Clear (Variables|Default|GetMonsterArray))
  (Utilities|Array|Add _monsterarray NewItem)
  (Utilities|Array|Add _monsterarray NewItem2)
  (Utilities|Array|Add _monsterarray NewItem3)
  (Utilities|Array|Add _monsterarray NewItem4)
  (Utilities|Array|Add _monsterarray NewItem5)
  (Utilities|Array|Add _monsterarray NewItem6))

(fn SetAllBattled
  (params (Battled :type Boolean))
  (bind _monsterrosterstruct (Variables|Default|GetMonsterRosterStruct))
  (Utilities|FlowControl|Sequence
    (:then_0
      (CallFunction|SetBattled (.monster_1 _monsterrosterstruct) Battled))
    (:then_1
      (CallFunction|SetBattled (.monster_2 _monsterrosterstruct) Battled))
    (:then_2
      (CallFunction|SetBattled (.monster_3 _monsterrosterstruct) Battled))
    (:then_3
      (CallFunction|SetBattled (.monster_4 _monsterrosterstruct) Battled))
    (:then_4
      (CallFunction|SetBattled (.monster_5 _monsterrosterstruct) Battled))
    (:then_5
      (CallFunction|SetBattled (.monster_6 _monsterrosterstruct) Battled))))

(fn SetBattled
  (params (Monster :type Struct%20Monster%20Structure%20%28by%20ref%29) (Battled :type Boolean))
  (|SetBy-RefVar (.Battled (Utilities|Struct|BreakStruct_Monster Monster)) Battled))

(fn HealParty
  (bind _monsterrosterstruct (Variables|Default|GetMonsterRosterStruct))
  (bind _stats (Utilities|Struct|BreakStruct_Monster (.monster_6 _monsterrosterstruct)))
  (bind _stats_2 (Utilities|Struct|BreakStruct_Monster (.monster_5 _monsterrosterstruct)))
  (bind _stats_3 (Utilities|Struct|BreakStruct_Monster (.monster_1 _monsterrosterstruct)))
  (bind _stats_4 (Utilities|Struct|BreakStruct_Monster (.monster_2 _monsterrosterstruct)))
  (bind _stats_5 (Utilities|Struct|BreakStruct_Monster (.monster_3 _monsterrosterstruct)))
  (bind _stats_6 (Utilities|Struct|BreakStruct_Monster (.monster_4 _monsterrosterstruct)))
  (bind (_health _totalhealth) (Utilities|Struct|BreakStruct_Stats _stats_6))
  (bind (_health_2 _totalhealth_2) (Utilities|Struct|BreakStruct_Stats _stats_2))
  (bind (_health_3 _totalhealth_3) (Utilities|Struct|BreakStruct_Stats _stats))
  (bind (_health_4 _totalhealth_4) (Utilities|Struct|BreakStruct_Stats _stats_3))
  (bind (_health_5 _totalhealth_5) (Utilities|Struct|BreakStruct_Stats _stats_4))
  (bind (_health_6 _totalhealth_6) (Utilities|Struct|BreakStruct_Stats _stats_5))
  (Utilities|FlowControl|Sequence
    (:then_0
      (|SetBy-RefVar _health_4 _totalhealth_4))
    (:then_1
      (|SetBy-RefVar _health_5 _totalhealth_5))
    (:then_2
      (|SetBy-RefVar _health_6 _totalhealth_6))
    (:then_3
      (|SetBy-RefVar _health _totalhealth))
    (:then_4
      (|SetBy-RefVar _health_2 _totalhealth_2))
    (:then_5
      (|SetBy-RefVar _health_3 _totalhealth_3)
      (CallFunction|SetOrder))))