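; BP_Monster is a monster Blueprint that carries its data in MonsterStruct and links to the player's monster roster.
; On BeginPlay it casts the player pawn to BP_Character, caches it and its MonsterRoster, then calls SetID.
; SetID assigns a random float UniqueID when the current one is below the valid range, with no collision check.
; A stat debug print is left unconnected.
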(event EventBeginPlay
  (bind _asbp_character (Utilities|Casting|CastToBP_Character (Game|GetPlayerCharacter 0)))
  (bind _output_get (Variables|Default|SetCharacter _asbp_character))
  (Variables|Default|SetMonster%20Roster (Variables|/Game/Blueprints/Avatar/BP_Character.BP_Character_C|GetMonsterRoster _output_get))
  (CallFunction|SetID))

(event Collision|EventActorBeginOverlap
  (params (OtherActor :type Actor%20Object%20Reference)))

(event EventTick
  (params (DeltaSeconds :type Float%20%28single-precision%29)))

(fn ConstructionScript)

(fn SetID
  (bind _monster_struct (Variables|Default|GetMonster%20Struct))
  (bind _monsterdetails (Utilities|Struct|BreakStruct_Monster _monster_struct))
  (bind _uniqueid (Utilities|Struct|BreakStruct_MonsterDetails _monsterdetails))
  (if (<= _uniqueid 9999.0)
    (|SetBy-RefVar _uniqueid (Math|Random|RandomFloatinRange 1e+04 1e+05))))