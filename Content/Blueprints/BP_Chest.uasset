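; Interactive chest actor that spawns an item when the player presses E nearby.
; Overlapping Box1 with BP_Character shows a text prompt and enables input while unopened; leaving hides it and disables input.
; Pressing E spawns the SpawnItem1 class at Box2's location at half scale, hides the prompt and sets Opened.
; E itself never checks Opened or disables input, so repeated presses before leaving spawn more items.
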(event OnComponentBeginOverlap(Box1)
  (params (OverlappedComponent :type Primitive%20Component%20Object%20Reference) (OtherActor :type Actor%20Object%20Reference) (OtherComp :type Primitive%20Component%20Object%20Reference) (OtherBodyIndex :type Integer) (bFromSweep :type Boolean) (SweepResult :type Hit%20Result%20Structure%20%28by%20ref%29))
  (Utilities|Casting|CastToBP_Character OtherActor)
  (if (not (Variables|Default|GetOpened?))
    (Development|SetHiddeninGame (Variables|Default|GetTextRender) false false)
    (Input|EnableInput (Game|GetPlayerController 0))))

(event OnComponentEndOverlap(Box1)
  (params (OverlappedComponent :type Primitive%20Component%20Object%20Reference) (OtherActor :type Actor%20Object%20Reference) (OtherComp :type Primitive%20Component%20Object%20Reference) (OtherBodyIndex :type Integer))
  (Utilities|Casting|CastToBP_Character OtherActor)
  (Development|SetHiddeninGame (Variables|Default|GetTextRender) true false)
  (Input|DisableInput (Game|GetPlayerController 0)))

(event Custom|Spawn
  (Game|SpawnActorfromClass (Variables|Default|GetSpawnItem1) (Math|Transform|MakeTransform (Transformation|GetWorldLocation (Variables|Default|GetBox2)) "0, 0, 0" "0.500000,0.500000,0.500000") "Undefined" 0 0))

(event EventBeginPlay)

(event Collision|EventActorBeginOverlap
  (params (OtherActor :type Actor%20Object%20Reference)))

(event EventTick
  (params (DeltaSeconds :type Float%20%28single-precision%29)))

(event Input|KeyboardEvents|E
  (params (Key :type Key%20Structure))
  (:Pressed
    (CallFunction|Spawn)
    (Development|SetHiddeninGame (Variables|Default|GetTextRender) true false)
    (Variables|Default|SetOpened? true)))

(fn ConstructionScript)