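; Winged Sandals inventory item that toggles the sandals state on the player character when used.
; On BeginPlay it adds itself straight to the inventory of player 0's BP_Character, with no pickup step.
; UseItem prints a debug message and flips the character's WingedSandals flag, ignoring its item and stat parameters.
; The effect of that flag is handled outside this asset.
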(event Collision|EventActorBeginOverlap
  (params (OtherActor :type Actor%20Object%20Reference))
  (|CallParentFunction OtherActor) ; This node is disabled and will not be called.\nDrag off pins to build functionality.
)

(event EventTick
  (params (DeltaSeconds :type Float%20%28single-precision%29))
  (|CallParentFunction DeltaSeconds) ; This node is disabled and will not be called.\nDrag off pins to build functionality.
)

(event EventBeginPlay
  (bind _asbp_character (Utilities|Casting|CastToBP_Character (Game|GetPlayerCharacter 0)))
  (Default|AddItemtoInventory (Variables|/Game/Blueprints/Avatar/BP_Character.BP_Character_C|GetBP_Inventory _asbp_character) self))

(fn ConstructionScript
  (|CallParentFunction))

(fn UseItem
  (params (Name :type String) (OnPlayer :type Boolean) (ItemType :type Enum_ItemTypes%20Enum :default "NewEnumerator5") (StatAffected :type Enum_Effect%20Enum :default "NewEnumerator0") (ImpactFactor :type Float%20%28single-precision%29))
  (Development|PrintString "Sandals being used")
  (bind _asbp_character (Utilities|Casting|CastToBP_Character (Game|GetPlayerCharacter 0)))
  (if (Variables|/Game/Blueprints/Avatar/BP_Character.BP_Character_C|GetWingedSandals _asbp_character)
    (Variables|/Game/Blueprints/Avatar/BP_Character.BP_Character_C|SetWingedSandals _asbp_character false)
    (else
      (Variables|/Game/Blueprints/Avatar/BP_Character.BP_Character_C|SetWingedSandals _asbp_character true))))