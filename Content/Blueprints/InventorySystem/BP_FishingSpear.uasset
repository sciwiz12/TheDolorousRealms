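; BP_FishingSpear is an inventory item that lets the player fish at a fishing spot.
; Its UseItem override calls the parent, then sets HasSpear on the player character's FishingSpot, before that reference is validity-checked.
; If the spot is valid, it plays the pause menu's SwitcherOpacity animation in reverse and calls FishingInteract on the spot.
; The box overlap and tick events add no logic of their own.
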(event OnComponentBeginOverlap(box)
  (params (OverlappedComponent :type Primitive%20Component%20Object%20Reference) (OtherActor :type Actor%20Object%20Reference) (OtherComp :type Primitive%20Component%20Object%20Reference) (OtherBodyIndex :type Integer) (bFromSweep :type Boolean) (SweepResult :type Hit%20Result%20Structure%20%28by%20ref%29)))

(event Collision|EventActorBeginOverlap
  (params (OtherActor :type Actor%20Object%20Reference))
  (|CallParentFunction OtherActor) ; This node is disabled and will not be called.\nDrag off pins to build functionality.
)

(event EventTick
  (params (DeltaSeconds :type Float%20%28single-precision%29))
  (|CallParentFunction DeltaSeconds))

(fn ConstructionScript
  (|CallParentFunction))

(fn UseItem
  (params (Name :type String) (OnPlayer :type Boolean) (ItemType :type Enum_ItemTypes%20Enum :default "NewEnumerator5") (StatAffected :type Enum_Effect%20Enum :default "NewEnumerator0") (ImpactFactor :type Float%20%28single-precision%29))
  (|CallParentFunction "" false "NewEnumerator5" "NewEnumerator0" 0.0)
  (bind _asbp_character (Utilities|Casting|CastToBP_Character (Game|GetPlayerCharacter 0)))
  (Variables|/Game/Blueprints/Wild_Area_Types/Wild_Areas/BP_FishingArea.BP_FishingArea_C|SetHasSpear (Variables|/Game/Blueprints/Avatar/BP_Character.BP_Character_C|GetFishingSpot _asbp_character) true)
  (Variables|Default|SetFishing%20Spot (Variables|/Game/Blueprints/Avatar/BP_Character.BP_Character_C|GetFishingSpot _asbp_character))
  (Utilities|IsValid (Variables|Default|GetFishing%20Spot)
    (:Is%20Valid
      (bind _foundwidgets (Widget|GetAllWidgetsOfClass "/Game/Blueprints/GUIs/GUI_PauseMenu.GUI_PauseMenu_C" false))
      (UserInterface|Animation|PlayAnimation (Utilities|Array|Get(acopy) _foundwidgets) (Variables|/Game/Blueprints/GUIs/GUI_PauseMenu.GUI_PauseMenu_C|GetSwitcherOpacity (Utilities|Array|Get(acopy) _foundwidgets)) 0.0 1 "Reverse" 1.0 false)
      (Default|FishingInteract (Variables|Default|GetFishing%20Spot)))))