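; Inventory item for a move scroll that teaches its Move to a monster picked from the roster.
; UseItem runs the parent logic and starts a short timer; ActivateRoster switches the pause menu to the roster, passing itself as the item.
; OnSelectedMonster fills the first empty of four move slots, or flags NoBlank if none is free.
; ReplaceMove overwrites a given slot, rebuilding and returning the monster struct.
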(event EventBeginPlay
  (|CallParentFunction) ; This node is disabled and will not be called.\nDrag off pins to build functionality.
)

(event Collision|EventActorBeginOverlap
  (params (OtherActor :type Actor%20Object%20Reference))
  (|CallParentFunction OtherActor) ; This node is disabled and will not be called.\nDrag off pins to build functionality.
)

(event EventTick
  (params (DeltaSeconds :type Float%20%28single-precision%29))
  (|CallParentFunction DeltaSeconds) ; This node is disabled and will not be called.\nDrag off pins to build functionality.
)

(fn ConstructionScript
  (|CallParentFunction))

(fn UseItem
  (params (Name :type String) (OnPlayer :type Boolean) (ItemType :type Enum_ItemTypes%20Enum :default "NewEnumerator5") (StatAffected :type Enum_Effect%20Enum :default "NewEnumerator0") (ImpactFactor :type Float%20%28single-precision%29))
  (|CallParentFunction Name OnPlayer ItemType StatAffected ImpactFactor)
  (Utilities|Time|SetTimerbyEvent (EventDispatchers|CreateEvent :!event ActivateRoster) 0.5))

(fn OnSelectedMonster
  (params (Monster :type Struct%20Monster%20Structure))
  (Utilities|FlowControl|Sequence
    (:then_0
      (Variables|Default|SetMonster Monster)
      (CallFunction|AssigntoBlank))
    (:then_1
      (if (not (Variables|Default|GetMoveAssigned))
        (Variables|Default|SetNoBlank true)))
    (:then_2
      (return (Variables|Default|GetMonster)))))

(fn CheckMoveAssigned
  (params (InputPin :type Struct%20Move%20Structure))
  (if (Utilities|Enum|Equal(Enum) (.MoveName (Utilities|Struct|BreakStruct_Move InputPin)) "")
    (Variables|Default|SetMoveAssigned true)
    (switch int (Variables|Default|GetIndex)
      (:0
        (Variables|Default|SetMonster (Utilities|Struct|MakeStruct_Monster (.monsterdetails (Variables|Default|GetMonster)) (.levelandxp (Variables|Default|GetMonster)) (.stats (Variables|Default|GetMonster)) (.basestats (Variables|Default|GetMonster)) (.statusactive (Variables|Default|GetMonster)) (.status (Variables|Default|GetMonster)) (Utilities|Struct|MakeStruct_MovesList (Variables|Default|GetMove) (.Move2 (Utilities|Struct|BreakStruct_MovesList (.moveslist (Variables|Default|GetMonster)))) (.Move3 (Utilities|Struct|BreakStruct_MovesList (.moveslist (Variables|Default|GetMonster)))) (.Move4 (Utilities|Struct|BreakStruct_MovesList (.moveslist (Variables|Default|GetMonster))))) (.battled (Variables|Default|GetMonster)))))
      (:1
        (Variables|Default|SetMonster (Utilities|Struct|MakeStruct_Monster (.monsterdetails (Variables|Default|GetMonster)) (.levelandxp (Variables|Default|GetMonster)) (.stats (Variables|Default|GetMonster)) (.basestats (Variables|Default|GetMonster)) (.statusactive (Variables|Default|GetMonster)) (.status (Variables|Default|GetMonster)) (Utilities|Struct|MakeStruct_MovesList (.Move1 (Utilities|Struct|BreakStruct_MovesList (.moveslist (Variables|Default|GetMonster)))) (Variables|Default|GetMove) (.Move3 (Utilities|Struct|BreakStruct_MovesList (.moveslist (Variables|Default|GetMonster)))) (.Move4 (Utilities|Struct|BreakStruct_MovesList (.moveslist (Variables|Default|GetMonster))))) (.battled (Variables|Default|GetMonster)))))
      (:2
        (Variables|Default|SetMonster (Utilities|Struct|MakeStruct_Monster (.monsterdetails (Variables|Default|GetMonster)) (.levelandxp (Variables|Default|GetMonster)) (.stats (Variables|Default|GetMonster)) (.basestats (Variables|Default|GetMonster)) (.statusactive (Variables|Default|GetMonster)) (.status (Variables|Default|GetMonster)) (Utilities|Struct|MakeStruct_MovesList (.Move1 (Utilities|Struct|BreakStruct_MovesList (.moveslist (Variables|Default|GetMonster)))) (.Move2 (Utilities|Struct|BreakStruct_MovesList (.moveslist (Variables|Default|GetMonster)))) (Variables|Default|GetMove) (.Move4 (Utilities|Struct|BreakStruct_MovesList (.moveslist (Variables|Default|GetMonster))))) (.battled (Variables|Default|GetMonster)))))
      (:3
        (Variables|Default|SetMonster (Utilities|Struct|MakeStruct_Monster (.monsterdetails (Variables|Default|GetMonster)) (.levelandxp (Variables|Default|GetMonster)) (.stats (Variables|Default|GetMonster)) (.basestats (Variables|Default|GetMonster)) (.statusactive (Variables|Default|GetMonster)) (.status (Variables|Default|GetMonster)) (Utilities|Struct|MakeStruct_MovesList (.Move1 (Utilities|Struct|BreakStruct_MovesList (.moveslist (Variables|Default|GetMonster)))) (.Move2 (Utilities|Struct|BreakStruct_MovesList (.moveslist (Variables|Default|GetMonster)))) (.Move3 (Utilities|Struct|BreakStruct_MovesList (.moveslist (Variables|Default|GetMonster)))) (Variables|Default|GetMove)) (.battled (Variables|Default|GetMonster))))))
    (else
      (bind _result (Math|Integer|IncrementInt (Variables|Default|GetIndex))
        (:%20%20
          (Variables|Default|SetIndex _result))))))

(fn ActivateRoster
  (bind _foundwidgets (Widget|GetAllWidgetsOfClass "/Game/Blueprints/GUIs/GUI_MonsterRosterMenu.GUI_MonsterRosterMenu_C" false))
  (Utilities|IsValid (Utilities|Array|Get(acopy) _foundwidgets)
    (:Is%20Valid
      (bind _foundwidgets_2 (Widget|GetAllWidgetsOfClass "/Game/Blueprints/GUIs/GUI_PauseMenu.GUI_PauseMenu_C" false))
      (Variables|/Game/Blueprints/GUIs/GUI_MonsterRosterMenu.GUI_MonsterRosterMenu_C|SetFromItems (Utilities|Array|Get(acopy) _foundwidgets) true)
      (Variables|/Game/Blueprints/GUIs/GUI_MonsterRosterMenu.GUI_MonsterRosterMenu_C|SetUse (Utilities|Array|Get(acopy) _foundwidgets) true)
      (Variables|/Game/Blueprints/GUIs/GUI_MonsterRosterMenu.GUI_MonsterRosterMenu_C|SetItem (Utilities|Array|Get(acopy) _foundwidgets) self)
      (Class|WidgetSwitcher|SetActiveWidget (Variables|/Game/Blueprints/GUIs/GUI_PauseMenu.GUI_PauseMenu_C|GetWidgetSwitcher_0 (Utilities|Array|Get(acopy) _foundwidgets_2)) (Utilities|Array|Get(acopy) _foundwidgets)))
    (:Is%20Not%20Valid
      (Development|PrintString "No Roster Found"))))

(fn AssigntoBlank
  (bind _monster (Variables|Default|GetMonster))
  (bind _moveslist (Utilities|Struct|BreakStruct_Monster _monster))
  (bind (_move1 _move2 _move3 _move4) (Utilities|Struct|BreakStruct_MovesList _moveslist))
  (CallFunction|CheckMoveAssigned _move1)
  (if (not (Variables|Default|GetMoveAssigned))
    (CallFunction|CheckMoveAssigned _move2)
    (if (not (Variables|Default|GetMoveAssigned))
      (CallFunction|CheckMoveAssigned _move3)
      (if (not (Variables|Default|GetMoveAssigned))
        (CallFunction|CheckMoveAssigned _move4)))))

(fn ReplaceMove
  (params (MoveToReplace :type Integer))
  (switch int MoveToReplace
    (:0
      (Variables|Default|SetMonster (Utilities|Struct|MakeStruct_Monster (.monsterdetails (Variables|Default|GetMonster)) (.levelandxp (Variables|Default|GetMonster)) (.stats (Variables|Default|GetMonster)) (.basestats (Variables|Default|GetMonster)) (.statusactive (Variables|Default|GetMonster)) (.status (Variables|Default|GetMonster)) (Utilities|Struct|MakeStruct_MovesList (Variables|Default|GetMove) (.Move2 (Utilities|Struct|BreakStruct_MovesList (.moveslist (Variables|Default|GetMonster)))) (.Move3 (Utilities|Struct|BreakStruct_MovesList (.moveslist (Variables|Default|GetMonster)))) (.Move4 (Utilities|Struct|BreakStruct_MovesList (.moveslist (Variables|Default|GetMonster))))) (.battled (Variables|Default|GetMonster)))))
    (:1
      (Variables|Default|SetMonster (Utilities|Struct|MakeStruct_Monster (.monsterdetails (Variables|Default|GetMonster)) (.levelandxp (Variables|Default|GetMonster)) (.stats (Variables|Default|GetMonster)) (.basestats (Variables|Default|GetMonster)) (.statusactive (Variables|Default|GetMonster)) (.status (Variables|Default|GetMonster)) (Utilities|Struct|MakeStruct_MovesList (.Move1 (Utilities|Struct|BreakStruct_MovesList (.moveslist (Variables|Default|GetMonster)))) (Variables|Default|GetMove) (.Move3 (Utilities|Struct|BreakStruct_MovesList (.moveslist (Variables|Default|GetMonster)))) (.Move4 (Utilities|Struct|BreakStruct_MovesList (.moveslist (Variables|Default|GetMonster))))) (.battled (Variables|Default|GetMonster)))))
    (:2
      (Variables|Default|SetMonster (Utilities|Struct|MakeStruct_Monster (.monsterdetails (Variables|Default|GetMonster)) (.levelandxp (Variables|Default|GetMonster)) (.stats (Variables|Default|GetMonster)) (.basestats (Variables|Default|GetMonster)) (.statusactive (Variables|Default|GetMonster)) (.status (Variables|Default|GetMonster)) (Utilities|Struct|MakeStruct_MovesList (.Move1 (Utilities|Struct|BreakStruct_MovesList (.moveslist (Variables|Default|GetMonster)))) (.Move2 (Utilities|Struct|BreakStruct_MovesList (.moveslist (Variables|Default|GetMonster)))) (Variables|Default|GetMove) (.Move4 (Utilities|Struct|BreakStruct_MovesList (.moveslist (Variables|Default|GetMonster))))) (.battled (Variables|Default|GetMonster)))))
    (:3
      (Variables|Default|SetMonster (Utilities|Struct|MakeStruct_Monster (.monsterdetails (Variables|Default|GetMonster)) (.levelandxp (Variables|Default|GetMonster)) (.stats (Variables|Default|GetMonster)) (.basestats (Variables|Default|GetMonster)) (.statusactive (Variables|Default|GetMonster)) (.status (Variables|Default|GetMonster)) (Utilities|Struct|MakeStruct_MovesList (.Move1 (Utilities|Struct|BreakStruct_MovesList (.moveslist (Variables|Default|GetMonster)))) (.Move2 (Utilities|Struct|BreakStruct_MovesList (.moveslist (Variables|Default|GetMonster)))) (.Move3 (Utilities|Struct|BreakStruct_MovesList (.moveslist (Variables|Default|GetMonster)))) (Variables|Default|GetMove)) (.battled (Variables|Default|GetMonster))))))
  (return (Variables|Default|GetMonster)))