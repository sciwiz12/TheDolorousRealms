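; BP_Item_MoveScroll_Climb is a move scroll item that unlocks climbing for the player character.
; On actor overlap it runs the parent logic, casts the other actor to BP_Character and stores it as Player.
; It then sets CanClimb to true on that character, or prints a message if the reference is invalid.
; BeginPlay and construction only call the parent, and Tick is disabled.
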(event EventBeginPlay
  (|CallParentFunction))

(event Collision|EventActorBeginOverlap
  (params (OtherActor :type Actor%20Object%20Reference))
  (|CallParentFunction OtherActor)
  (bind _asbp_character (Utilities|Casting|CastToBP_Character OtherActor))
  (Variables|Default|SetPlayer _asbp_character)
  (Utilities|IsValid (Variables|Default|GetPlayer)
    (:Is%20Valid
      (Variables|/Game/Blueprints/Avatar/BP_Character.BP_Character_C|SetCanClimb (Variables|Default|GetPlayer) true))
    (:Is%20Not%20Valid
      (Development|PrintString "Not valid"))))

(event EventTick
  (params (DeltaSeconds :type Float%20%28single-precision%29))
  (|CallParentFunction DeltaSeconds) ; This node is disabled and will not be called.\nDrag off pins to build functionality.
)

(fn ConstructionScript
  (|CallParentFunction))