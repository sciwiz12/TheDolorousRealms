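; Illusion scroll actor that reverses the player character's movement when an actor overlaps it.
; ReverseMovement flips BP_Character's DirectionFactor to negative and alters the post-process volume's contrast as a visual cue.
; CorrectMovement restores direction and neutral contrast, but nothing in this graph calls it.
; GotoLoseScreen is a placeholder that only prints a reminder string.
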(event EventBeginPlay
  (|CallParentFunction))

(event Collision|EventActorBeginOverlap
  (params (OtherActor :type Actor%20Object%20Reference))
  (|CallParentFunction OtherActor)
  (CallFunction|ReverseMovement))

(fn ConstructionScript
  (|CallParentFunction))

(fn ReverseMovement
  (bind _asbp_character (Utilities|Casting|CastToBP_Character (Game|GetPlayerCharacter 0)))
  (Variables|/Game/Blueprints/Avatar/BP_Character.BP_Character_C|SetDirectionFactor _asbp_character -1.0)
  (|SetBy-RefVar (Utilities|Struct|BreakPostProcessSettings (Variables|/Script/Engine.PostProcessVolume|GetSettings (Variables|Default|GetPostProcessingVolume))) (Math|Vector4|MakeVector4 1.0 0.0 1.0 2.0)))

(fn GotoLoseScreen
  (Development|PrintString "Add whatever you're gonna do here to take them to a lose screen. Add a GUI to the viewport or whatever."))

(fn CorrectMovement
  (bind _asbp_character (Utilities|Casting|CastToBP_Character (Game|GetPlayerCharacter 0)))
  (Variables|/Game/Blueprints/Avatar/BP_Character.BP_Character_C|SetDirectionFactor _asbp_character 1.0)
  (|SetBy-RefVar (Utilities|Struct|BreakPostProcessSettings (Variables|/Script/Engine.PostProcessVolume|GetSettings (Variables|Default|GetPostProcessingVolume))) (Math|Vector4|MakeVector4 1.0 1.0 1.0 1.0)))