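; BP_Illusion_Freeze is an illusion actor that immobilizes the player when any actor overlaps it.
; On overlap it sets the player character's movement mode to None and spawns a flame sprite actor at the character's location, keeping a reference to it.
; Unfreeze restores walking and destroys that sprite, but nothing in this Blueprint calls it.
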(event EventBeginPlay
  (|CallParentFunction) ; This node is disabled and will not be called.\nDrag off pins to build functionality.
)

(event Collision|EventActorBeginOverlap
  (params (OtherActor :type Actor%20Object%20Reference))
  (|CallParentFunction OtherActor)
  (CallFunction|FreezePlayer))

(event EventTick
  (params (DeltaSeconds :type Float%20%28single-precision%29))
  (|CallParentFunction DeltaSeconds) ; This node is disabled and will not be called.\nDrag off pins to build functionality.
)

(fn ConstructionScript
  (|CallParentFunction))

(fn FreezePlayer
  (Pawn|Components|CharacterMovement|SetMovementMode (Variables|/Script/Engine.Character|GetCharacterMovement (Game|GetPlayerCharacter 0)) "MOVE_None" 0)
  (CallFunction|SpawnFlipBook))

(fn Unfreeze
  (Pawn|Components|CharacterMovement|SetMovementMode (Variables|/Script/Engine.Character|GetCharacterMovement (Game|GetPlayerCharacter 0)) "MOVE_Walking" 0)
  (CallFunction|DestroyFire))

(fn SpawnFlipBook
  (bind _asbp_character (Utilities|Casting|CastToBP_Character (Game|GetPlayerCharacter 0)))
  (bind _returnvalue (Game|SpawnActorfromClass (Variables|Default|GetFlameSprite) (Math|Transform|MakeTransform (Transformation|GetActorLocation _asbp_character) "0, 0, 0" "1,1,1") "Undefined" 0 0))
  (Variables|Default|SetFlameSpriteActor _returnvalue))

(fn DestroyFire
  (Utilities|IsValid (Variables|Default|GetFlameSpriteActor)
    (:Is%20Valid
      (Actor|DestroyActor (Variables|Default|GetFlameSpriteActor)))))