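; Pickup item actor that a BP_Character can collect into its inventory when standing inside the item's box trigger.
; Overlap registers the item on the character, shows a text prompt and opens a gate that allows Interact; leaving hides and closes it.
; Interact increments the count of a same-named inventory entry or adds the item, then destroys the actor.
; UseItem is an empty stub and OnSelectedMonster returns the monster passed to it.
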(event OnComponentBeginOverlap(Box)
  (params (OverlappedComponent :type Primitive%20Component%20Object%20Reference) (OtherActor :type Actor%20Object%20Reference) (OtherComp :type Primitive%20Component%20Object%20Reference) (OtherBodyIndex :type Integer) (bFromSweep :type Boolean) (SweepResult :type Hit%20Result%20Structure%20%28by%20ref%29))
  (bind _self self)
  (bind _asbp_character (Utilities|Casting|CastToBP_Character OtherActor))
  (bind _output_get (Variables|Default|SetAs%20BP%20Character _asbp_character))
  (Variables|/Game/Blueprints/Avatar/BP_Character.BP_Character_C|SetItem _output_get self)
  (Development|SetHiddeninGame (Variables|Default|GetTextRender) false false)
  (Utilities|FlowControl|Gate true) ; enters at Open
)

(event OnComponentEndOverlap(Box)
  (params (OverlappedComponent :type Primitive%20Component%20Object%20Reference) (OtherActor :type Actor%20Object%20Reference) (OtherComp :type Primitive%20Component%20Object%20Reference) (OtherBodyIndex :type Integer))
  (bind _self self)
  (bind _as_bp_character (Variables|Default|GetAs%20BP%20Character))
  (bind _bp_inventory (Variables|/Game/Blueprints/Avatar/BP_Character.BP_Character_C|GetBP_Inventory _as_bp_character))
  (bind _structinventory (Variables|/Game/Blueprints/InventorySystem/BP_Inventory.BP_Inventory_C|GetStructInventory _bp_inventory))
  (Utilities|Casting|CastToBP_Character OtherActor)
  (Development|SetHiddeninGame (Variables|Default|GetTextRender) true false)
  (Utilities|FlowControl|Gate true) ; enters at Close
)

(event Custom|Interact
  (bind _self self)
  (bind _as_bp_character (Variables|Default|GetAs%20BP%20Character))
  (bind _bp_inventory (Variables|/Game/Blueprints/Avatar/BP_Character.BP_Character_C|GetBP_Inventory _as_bp_character))
  (bind _structinventory (Variables|/Game/Blueprints/InventorySystem/BP_Inventory.BP_Inventory_C|GetStructInventory _bp_inventory))
  (Utilities|FlowControl|Gate true
    (:Exit
      (for (_ _array_index) _structinventory
        (if (Utilities|Enum|Equal(Enum) (.Name (Utilities|Struct|BreakStruct_Item (Utilities|Array|Get(acopy) _structinventory _array_index))) (.name (Variables|Default|GetItemStruct _self)))
          (Variables|Default|SetInventoryNameMatch (Utilities|Enum|Equal(Enum) (.Name (Utilities|Struct|BreakStruct_Item (Utilities|Array|Get(acopy) _structinventory _array_index))) (.name (Variables|Default|GetItemStruct _self))))
          (Variables|Default|SetIndexofDuplicate _array_index)))
      (if (Variables|Default|GetInventoryNameMatch)
        (Default|IncrementItemCount _bp_inventory (Variables|Default|GetIndexofDuplicate))
        (Actor|DestroyActor)
        (else
          (Default|AddItemtoInventory _bp_inventory _self)
          (Actor|DestroyActor))))))

(event EventBeginPlay)

(event Collision|EventActorBeginOverlap
  (params (OtherActor :type Actor%20Object%20Reference)))

(event EventTick
  (params (DeltaSeconds :type Float%20%28single-precision%29)))

(fn ConstructionScript)

(fn UseItem
  (params (Name :type String) (OnPlayer :type Boolean) (ItemType :type Enum_ItemTypes%20Enum :default "NewEnumerator5") (StatAffected :type Enum_Effect%20Enum :default "NewEnumerator0") (ImpactFactor :type Float%20%28single-precision%29)))

(fn OnSelectedMonster
  (params (Monster :type Struct%20Monster%20Structure))
  (return Monster))