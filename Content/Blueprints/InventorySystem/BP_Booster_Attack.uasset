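; BP_Booster_Attack is an inventory item that boosts the attack damage of the player's monster.
; Its UseItem override finds the GUI_BattleMenu_Test1 widget and reads PlayerMonster from the first instance found.
; If that monster is valid, it adds ImpactFactor to the damage of Move1 only, then calls the parent UseItem.
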(event EventBeginPlay
  (|CallParentFunction) ; This node is disabled and will not be called.\nDrag off pins to build functionality.
)

(event Collision|EventActorBeginOverlap
  (params (OtherActor :type Actor%20Object%20Reference))
  (|CallParentFunction OtherActor) ; This node is disabled and will not be called.\nDrag off pins to build functionality.
)

(event EventTick
  (params (DeltaSeconds :type Float%20%28single-precision%29))
  (|CallParentFunction DeltaSeconds) ; This node is disabled and will not be called.\nDrag off pins to build functionality.
)

(fn ConstructionScript
  (|CallParentFunction))

(fn UseItem
  (params (Name :type String) (OnPlayer :type Boolean) (ItemType :type Enum_ItemTypes%20Enum :default "NewEnumerator5") (StatAffected :type Enum_Effect%20Enum :default "NewEnumerator0") (ImpactFactor :type Float%20%28single-precision%29))
  (bind _foundwidgets (Widget|GetAllWidgetsOfClass "/Game/Blueprints/GUIs/GUI_BattleMenu_Test1.GUI_BattleMenu_Test1_C" false))
  (Utilities|IsValid (Variables|/Game/Blueprints/GUIs/GUI_BattleMenu_Test1.GUI_BattleMenu_Test1_C|GetPlayerMonster (Utilities|Array|Get(acopy) _foundwidgets))
    (:Is%20Valid
      (bind _output_get (LocalVariables|SetPlayerMonster (Variables|/Game/Blueprints/GUIs/GUI_BattleMenu_Test1.GUI_BattleMenu_Test1_C|GetPlayerMonster (Utilities|Array|Get(acopy) _foundwidgets))))
      (bind _output_get_2 (LocalVariables|SetImpact ImpactFactor))
      (|SetBy-RefVar (.Damage (Utilities|Struct|BreakStruct_Move (.Move1 (Utilities|Struct|BreakStruct_MovesList (.MovesList (Utilities|Struct|BreakStruct_Monster (Variables|/Game/Blueprints/MonsterAssets/BP_Monster.BP_Monster_C|GetMonster%20Struct (LocalVariables|GetPlayerMonster)))))))) (+ _output_get_2 (.Damage (Utilities|Struct|BreakStruct_Move (.Move1 (Utilities|Struct|BreakStruct_MovesList (.MovesList (Utilities|Struct|BreakStruct_Monster (Variables|/Game/Blueprints/MonsterAssets/BP_Monster.BP_Monster_C|GetMonster%20Struct _output_get)))))))))
      (|CallParentFunction "" false "NewEnumerator5" "NewEnumerator0" 0.0))))