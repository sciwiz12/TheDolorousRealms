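; BP_SoulStone_OK is an inventory item that attempts to capture a monster during battle.
; UseItem rolls a random integer against a threshold and acts only when the roll meets or exceeds it.
; On success, a sequence gets the monster to catch, gets the roster array, fills an empty slot and closes the battle menu.
; A failed roll has no handling, and the other event graph nodes are disabled stubs.
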(event EventBeginPlay
  (|CallParentFunction) ; This node is disabled and will not be called.\nDrag off pins to build functionality.
)

(event Collision|EventActorBeginOverlap
  (params (OtherActor :type Actor%20Object%20Reference))
  (|CallParentFunction OtherActor) ; This node is disabled and will not be called.\nDrag off pins to build functionality.
)

(event EventTick
  (params (DeltaSeconds :type Float%20%28single-precision%29))
  (|CallParentFunction DeltaSeconds) ; This node is disabled and will not be called.\nDrag off pins to build functionality.
)

(fn ConstructionScript
  (|CallParentFunction))

(fn UseItem
  (params (Name :type String) (OnPlayer :type Boolean) (ItemType :type Enum_ItemTypes%20Enum :default "NewEnumerator5") (StatAffected :type Enum_Effect%20Enum :default "NewEnumerator0") (ImpactFactor :type Float%20%28single-precision%29))
  (if (>= (Math|Random|RandomIntegerinRange 0 100) (Variables|Default|GetThreashold))
    (Utilities|FlowControl|Sequence
      (:then_0
        (CallFunction|GetMontoCatch))
      (:then_1
        (CallFunction|GetRosterSetArray))
      (:then_2
        (CallFunction|FindEmptyandSet))
      (:then_3
        (Default|CloseDown (Variables|Default|GetBattleMenu))))))