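; BP_StatusRemover is an inventory item that clears a monster's status condition.
; In battle, UseItem resets the player monster's status, reverses the status visibility animation on the battle menu, then calls the parent logic.
; Otherwise it switches the pause menu to the monster roster, passing itself as the item in use.
; OnSelectedMonster applies the same reset to the given monster and returns it.
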(event EventBeginPlay
  (|CallParentFunction) ; This node is disabled and will not be called.\nDrag off pins to build functionality.
)

(event Collision|EventActorBeginOverlap
  (params (OtherActor :type Actor%20Object%20Reference))
  (|CallParentFunction OtherActor) ; This node is disabled and will not be called.\nDrag off pins to build functionality.
)

(event EventTick
  (params (DeltaSeconds :type Float%20%28single-precision%29))
  (|CallParentFunction DeltaSeconds) ; This node is disabled and will not be called.\nDrag off pins to build functionality.
)

(fn ConstructionScript
  (|CallParentFunction))

(fn UseItem
  (params (Name :type String) (OnPlayer :type Boolean) (ItemType :type Enum_ItemTypes%20Enum :default "NewEnumerator5") (StatAffected :type Enum_Effect%20Enum :default "NewEnumerator0") (ImpactFactor :type Float%20%28single-precision%29))
  (bind _foundwidgets (Widget|GetAllWidgetsOfClass "/Game/Blueprints/GUIs/GUI_BattleMenu_Test1.GUI_BattleMenu_Test1_C" false))
  (Utilities|IsValid (Utilities|Array|Get(acopy) _foundwidgets)
    (:Is%20Valid
      (Utilities|IsValid (Variables|/Game/Blueprints/GUIs/GUI_BattleMenu_Test1.GUI_BattleMenu_Test1_C|GetPlayerMonster (Utilities|Array|Get(acopy) _foundwidgets))
        (:Is%20Valid
          (|SetBy-RefVar (.StatusActive (Utilities|Struct|BreakStruct_Monster (Variables|/Game/Blueprints/MonsterAssets/BP_Monster.BP_Monster_C|GetMonster%20Struct (Variables|/Game/Blueprints/GUIs/GUI_BattleMenu_Test1.GUI_BattleMenu_Test1_C|GetPlayerMonster (Utilities|Array|Get(acopy) _foundwidgets))))) false)
          (|SetBy-RefVar (.Status (Utilities|Struct|BreakStruct_Monster (Variables|/Game/Blueprints/MonsterAssets/BP_Monster.BP_Monster_C|GetMonster%20Struct (Variables|/Game/Blueprints/GUIs/GUI_BattleMenu_Test1.GUI_BattleMenu_Test1_C|GetPlayerMonster (Utilities|Array|Get(acopy) _foundwidgets))))) "NewEnumerator6")
          (UserInterface|Animation|PlayAnimation (Utilities|Array|Get(acopy) _foundwidgets) (Variables|/Game/Blueprints/GUIs/GUI_BattleMenu_Test1.GUI_BattleMenu_Test1_C|GetMyStatusVisibility (Utilities|Array|Get(acopy) _foundwidgets)) 0.0 1 "Reverse" 1.0 false)
          (|CallParentFunction "" false "NewEnumerator5" "NewEnumerator0" 0.0))
        (:Is%20Not%20Valid
          (bind _foundwidgets_2 (Widget|GetAllWidgetsOfClass "/Game/Blueprints/GUIs/GUI_MonsterRosterMenu.GUI_MonsterRosterMenu_C" false :!label _label))
          (Utilities|IsValid (Utilities|Array|Get(acopy) _foundwidgets_2)
            (:Is%20Valid
              (bind _foundwidgets_3 (Widget|GetAllWidgetsOfClass "/Game/Blueprints/GUIs/GUI_PauseMenu.GUI_PauseMenu_C" false))
              (Variables|/Game/Blueprints/GUIs/GUI_MonsterRosterMenu.GUI_MonsterRosterMenu_C|SetFromItems (Utilities|Array|Get(acopy) _foundwidgets_2) true)
              (Variables|/Game/Blueprints/GUIs/GUI_MonsterRosterMenu.GUI_MonsterRosterMenu_C|SetUse (Utilities|Array|Get(acopy) _foundwidgets_2) true)
              (Variables|/Game/Blueprints/GUIs/GUI_MonsterRosterMenu.GUI_MonsterRosterMenu_C|SetItem (Utilities|Array|Get(acopy) _foundwidgets_2) self)
              (Class|WidgetSwitcher|SetActiveWidget (Variables|/Game/Blueprints/GUIs/GUI_PauseMenu.GUI_PauseMenu_C|GetWidgetSwitcher_0 (Utilities|Array|Get(acopy) _foundwidgets_3)) (Utilities|Array|Get(acopy) _foundwidgets_2)))))))
    (:Is%20Not%20Valid
      (goto _label))))

(fn OnSelectedMonster
  (params (Monster :type Struct%20Monster%20Structure))
  (bind (_monsterdetails _levelandxp _stats _basestats _statusactive _status) (Utilities|Struct|BreakStruct_Monster Monster))
  (|SetBy-RefVar _statusactive false)
  (|SetBy-RefVar _status "NewEnumerator6")
  (return Monster))