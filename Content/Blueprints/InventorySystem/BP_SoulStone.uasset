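; BP_SoulStone is an inventory item that captures the monster being fought in battle, with no success roll.
; On use, it copies the spawned monster's struct from the battle menu widget and rebuilds the player's roster array.
; It writes the monster into the first of six roster slots with an empty name, or sends it to BP_MonsterStorage when full.
; It then closes the battle menu.
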(event EventBeginPlay
  (|CallParentFunction) ; This node is disabled and will not be called.\nDrag off pins to build functionality.
)

(event Collision|EventActorBeginOverlap
  (params (OtherActor :type Actor%20Object%20Reference))
  (|CallParentFunction OtherActor) ; This node is disabled and will not be called.\nDrag off pins to build functionality.
)

(event EventTick
  (params (DeltaSeconds :type Float%20%28single-precision%29))
  (|CallParentFunction DeltaSeconds) ; This node is disabled and will not be called.\nDrag off pins to build functionality.
)

(fn ConstructionScript
  (|CallParentFunction))

(fn UseItem
  (params (Name :type String) (OnPlayer :type Boolean) (ItemType :type Enum_ItemTypes%20Enum :default "NewEnumerator5") (StatAffected :type Enum_Effect%20Enum :default "NewEnumerator0") (ImpactFactor :type Float%20%28single-precision%29))
  (|CallParentFunction Name OnPlayer ItemType StatAffected ImpactFactor)
  (Utilities|FlowControl|Sequence
    (:then_0
      (CallFunction|GetMontoCatch))
    (:then_1
      (CallFunction|GetRosterSetArray))
    (:then_2
      (CallFunction|FindEmptyandSet))
    (:then_3
      (Default|CloseDown (Variables|Default|GetBattleMenu)))))

(fn SetRosterSlot
  (params (Selection :type Integer))
  (bind _monster_roster (Variables|Default|GetMonster%20Roster))
  (bind _monsterrosterstruct (Variables|/Game/Blueprints/MonsterAssets/BP_Component_MonsterRoster.BP_Component_MonsterRoster_C|GetMonsterRosterStruct _monster_roster))
  (switch int Selection
    (:0
      (|SetBy-RefVar (.monster_1 _monsterrosterstruct) (Variables|Default|GetMonster%20Struct)))
    (:1
      (|SetBy-RefVar (.monster_2 _monsterrosterstruct) (Variables|Default|GetMonster%20Struct)))
    (:2
      (|SetBy-RefVar (.monster_3 _monsterrosterstruct) (Variables|Default|GetMonster%20Struct)))
    (:3
      (|SetBy-RefVar (.monster_4 _monsterrosterstruct) (Variables|Default|GetMonster%20Struct)))
    (:4
      (|SetBy-RefVar (.monster_5 _monsterrosterstruct) (Variables|Default|GetMonster%20Struct)))
    (:5
      (|SetBy-RefVar (.monster_6 _monsterrosterstruct) (Variables|Default|GetMonster%20Struct)))))

(fn GetMontoCatch
  (bind _foundwidgets (Widget|GetAllWidgetsOfClass "/Game/Blueprints/GUIs/GUI_BattleMenu_Test1.GUI_BattleMenu_Test1_C" true))
  (Variables|Default|SetBattleMenu (Utilities|Array|Get(acopy) _foundwidgets))
  (Variables|Default|SetMonster%20Struct (Variables|/Game/Blueprints/MonsterAssets/BP_Monster.BP_Monster_C|GetMonster%20Struct (Variables|/Game/Blueprints/GUIs/GUI_BattleMenu_Test1.GUI_BattleMenu_Test1_C|GetSpawnedMonster (Utilities|Array|Get(acopy) _foundwidgets)))))

(fn GetRosterSetArray
  (bind _asbp_character (Utilities|Casting|CastToBP_Character (Game|GetPlayerCharacter 0)))
  (Variables|Default|SetMonster%20Roster (Variables|/Game/Blueprints/Avatar/BP_Character.BP_Character_C|GetMonsterRoster _asbp_character))
  (Default|AddtoArray (Variables|Default|GetMonster%20Roster) (.monster_1 (Variables|/Game/Blueprints/MonsterAssets/BP_Component_MonsterRoster.BP_Component_MonsterRoster_C|GetMonsterRosterStruct (Variables|Default|GetMonster%20Roster))) (.monster_2 (Variables|/Game/Blueprints/MonsterAssets/BP_Component_MonsterRoster.BP_Component_MonsterRoster_C|GetMonsterRosterStruct (Variables|Default|GetMonster%20Roster))) (.monster_3 (Variables|/Game/Blueprints/MonsterAssets/BP_Component_MonsterRoster.BP_Component_MonsterRoster_C|GetMonsterRosterStruct (Variables|Default|GetMonster%20Roster))) (.monster_4 (Variables|/Game/Blueprints/MonsterAssets/BP_Component_MonsterRoster.BP_Component_MonsterRoster_C|GetMonsterRosterStruct (Variables|Default|GetMonster%20Roster))) (.monster_5 (Variables|/Game/Blueprints/MonsterAssets/BP_Component_MonsterRoster.BP_Component_MonsterRoster_C|GetMonsterRosterStruct (Variables|Default|GetMonster%20Roster))) (.monster_6 (Variables|/Game/Blueprints/MonsterAssets/BP_Component_MonsterRoster.BP_Component_MonsterRoster_C|GetMonsterRosterStruct (Variables|Default|GetMonster%20Roster)))))

(fn FindEmptyandSet
  (Variables|Default|SetMonsterParty 0)
  (bind (_array_element _array_index) (Utilities|Array|ForEachLoopwithBreak (Variables|/Game/Blueprints/MonsterAssets/BP_Component_MonsterRoster.BP_Component_MonsterRoster_C|GetMonsterArray (Variables|Default|GetMonster%20Roster)) :!label _label)
    (:LoopBody
      (if (Utilities|Enum|Equal(Enum) (.Name (Utilities|Struct|BreakStruct_MonsterDetails (.MonsterDetails (Utilities|Struct|BreakStruct_Monster _array_element)))) "")
        (CallFunction|SetRosterSlot _array_index)
        (goto _label Break)
        (else
          (bind _result (Math|Integer|IncrementInt (Variables|Default|GetMonsterParty))
            (:%20%20
              (Variables|Default|SetMonsterParty _result))))))
    (:Completed
      (if (>= (Variables|Default|GetMonsterParty) 6)
        (bind _returnvalue (Actor|GetActorOfClass "/Game/Blueprints/InventorySystem/BP_MonsterStorage.BP_MonsterStorage_C"))
        (Utilities|IsValid _returnvalue
          (:Is%20Valid
            (bind _output_get (Variables|Default|SetStorageSystem _returnvalue))
            (Default|AddtoStorage _output_get (Variables|Default|GetMonster%20Struct))))))))