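; BP_MonsterStorage is a world actor where the player accesses stored monsters, kept in a Monsters array filled by AddToStorage.
; On BeginPlay it registers with GI_Main and calls LoadStorageSystem.
; Box overlap shows a text prompt, tracks range and gives BP_Character a reference to the storage.
; PlayerAccess plays the flipbook, then after a delay shows or creates GUI_Monster_Storage and freezes player movement, enabling the cursor only for an existing widget.
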(event OnComponentBeginOverlap(box)
  (params (OverlappedComponent :type Primitive%20Component%20Object%20Reference) (OtherActor :type Actor%20Object%20Reference) (OtherComp :type Primitive%20Component%20Object%20Reference) (OtherBodyIndex :type Integer) (bFromSweep :type Boolean) (SweepResult :type Hit%20Result%20Structure%20%28by%20ref%29))
  (bind _asbp_character (Utilities|Casting|CastToBP_Character OtherActor))
  (Rendering|SetVisibility (Variables|Default|GetTextRender) true false)
  (Variables|/Game/Blueprints/Avatar/BP_Character.BP_Character_C|SetStorageSystem _asbp_character self)
  (Variables|Default|SetInRange true))

(event OnComponentEndOverlap(box)
  (params (OverlappedComponent :type Primitive%20Component%20Object%20Reference) (OtherActor :type Actor%20Object%20Reference) (OtherComp :type Primitive%20Component%20Object%20Reference) (OtherBodyIndex :type Integer))
  (Utilities|Casting|CastToBP_Character OtherActor)
  (Rendering|SetVisibility (Variables|Default|GetTextRender) false false)
  (Variables|Default|SetInRange false)
  (Components|Timeline|SetPlayRate (Variables|Default|GetPaperFlipbook) 0.0))

(event Custom|PlayerAccess
  (bind _returnvalue (Game|GetPlayerCharacter 0))
  (bind _charactermovement (Variables|/Script/Engine.Character|GetCharacterMovement _returnvalue))
  (if (Variables|Default|GetInRange)
    (Components|Timeline|SetPlayRate (Variables|Default|GetPaperFlipbook) 1.0)
    (Utilities|FlowControl|Delay 3.0)
    (bind _foundwidgets (Widget|GetAllWidgetsOfClass "/Game/Blueprints/GUIs/GUI_Monster_Storage.GUI_Monster_Storage_C" false))
    (Utilities|IsValid (Utilities|Array|Get(acopy) _foundwidgets)
      (:Is%20Valid
        (Widget|SetVisibility (Utilities|Array|Get(acopy) _foundwidgets) "Visible")
        (Pawn|Components|CharacterMovement|SetMovementMode _charactermovement "MOVE_None" 0)
        (Variables|/Script/Engine.PlayerController|SetbShowMouseCursor (Game|GetPlayerController 0) true))
      (:Is%20Not%20Valid
        (bind _returnvalue_2 (UserInterface|CreateWidget "/Game/Blueprints/GUIs/GUI_Monster_Storage.GUI_Monster_Storage_C"))
        (UserInterface|Viewport|AddtoViewport _returnvalue_2 0)
        (Pawn|Components|CharacterMovement|SetMovementMode _charactermovement "MOVE_None" 0)))))

(event Collision|EventActorBeginOverlap
  (params (OtherActor :type Actor%20Object%20Reference)))

(event EventTick
  (params (DeltaSeconds :type Float%20%28single-precision%29)))

(event EventBeginPlay
  (bind _asgi_main (Utilities|Casting|CastToGI_Main (Game|GetGameInstance)))
  (Variables|/Game/Blueprints/GI_Main.GI_Main_C|SetStoragesystem _asgi_main self)
  (Default|LoadStorageSystem _asgi_main))

(fn ConstructionScript)

(fn AddtoStorage
  (params (Monster :type Struct%20Monster%20Structure))
  (Utilities|Array|Add (Variables|Default|GetMonsters) Monster))