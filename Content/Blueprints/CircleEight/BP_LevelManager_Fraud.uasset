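; Level manager for the Fraud level (Circle Eight) that sets up the player character when play begins.
; BeginLevel raises the character's camera and copies the saved monster roster from GI_Main into the character's MonsterRoster.
; Tick adjusts the camera's relative height by an axis value and prints a debug "Hello".
; The EncounterBeasts and EncounterVirgil events are empty stubs.
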(event Custom|BeginLevel
  (bind _asbp_character (Utilities|Casting|CastToBP_Character (Game|GetPlayerCharacter 0)))
  (bind _output_get (Variables|Default|SetCharacter _asbp_character))
  (Transformation|SetRelativeLocation (Variables|/Game/Blueprints/Avatar/BP_Character.BP_Character_C|GetCamera _output_get) "15.832092, 0,1000.000000" false false)
  (bind _asgi_main (Utilities|Casting|CastToGI_Main (Game|GetGameInstance)))
  (bind _asbp_character_2 (Utilities|Casting|CastToBP_Character (Game|GetPlayerCharacter 0)))
  (Variables|/Game/Blueprints/MonsterAssets/BP_Component_MonsterRoster.BP_Component_MonsterRoster_C|SetMonsterRosterStruct (Variables|/Game/Blueprints/Avatar/BP_Character.BP_Character_C|GetMonsterRoster _asbp_character_2) (Variables|/Game/Blueprints/GI_Main.GI_Main_C|Getmonster%20struct%20roster _asgi_main)))

(event Custom|EncounterBeasts)

(event Custom|EncounterVirgil)

(event EventBeginPlay
  (CallFunction|BeginLevel))

(event Collision|EventActorBeginOverlap
  (params (OtherActor :type Actor%20Object%20Reference)))

(event EventTick
  (params (DeltaSeconds :type Float%20%28single-precision%29))
  (bind _axisvalue (Variables|Default|GetAxisValue))
  (Transformation|SetRelativeLocation (Variables|/Game/Blueprints/Avatar/BP_Character.BP_Character_C|GetCamera (Variables|Default|GetCharacter)) (Math|Vector|MakeVector 15.832092 0.0 (+ (Variables|Default|GetNew%20Location%20Z) _axisvalue)) false false)
  (Development|PrintString "Hello" true true "(R=0.000000,G=0.660000,B=1.000000,A=1.000000)" _axisvalue))

(fn ConstructionScript)