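; BP_Climb is a moving tile that travels to an end point when its Climb event fires and the character can climb.
; A character entering the trigger box gets this actor registered as the Climb reference on its move executer component.
; Climb plays a timeline that lerps the tile between positions cached at BeginPlay, at a configurable play rate.
; A character leaving the box reverses the timeline.
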(event OnComponentBeginOverlap(Box)
  (params (OverlappedComponent :type Primitive%20Component%20Object%20Reference) (OtherActor :type Actor%20Object%20Reference) (OtherComp :type Primitive%20Component%20Object%20Reference) (OtherBodyIndex :type Integer) (bFromSweep :type Boolean) (SweepResult :type Hit%20Result%20Structure%20%28by%20ref%29))
  (bind _asbp_character (Utilities|Casting|CastToBP_Character OtherActor))
  (Variables|/Game/Blueprints/Moves/BP_Component_MoveExecuter.BP_Component_MoveExecuter_C|SetClimb (Variables|/Game/Blueprints/Avatar/BP_Character.BP_Character_C|GetBP_Component_MoveExecuter _asbp_character) self))

(event OnComponentEndOverlap(Box)
  (params (OverlappedComponent :type Primitive%20Component%20Object%20Reference) (OtherActor :type Actor%20Object%20Reference) (OtherComp :type Primitive%20Component%20Object%20Reference) (OtherBodyIndex :type Integer))
  (Utilities|Casting|CastToBP_Character OtherActor)
  (bind _newtrack_0 (Timeline|platformMoving Reverse)
    (:Update
      (Transformation|SetWorldLocation (Variables|Default|GetMovingTile) (Math|Vector|Lerp(Vector) (Variables|Default|GetStartLocation) (Variables|Default|GetEndLocation) _newtrack_0) false false))))

(event Custom|Climb
  (if (Variables|/Game/Blueprints/Avatar/BP_Character.BP_Character_C|GetCanClimb (stale OnComponentBeginOverlap(Box) _asbp_character))
    (Development|PrintString "Hello")
    (bind _newtrack_0 (Timeline|platformMoving Play)
      (:Update
        (Transformation|SetWorldLocation (Variables|Default|GetMovingTile) (Math|Vector|Lerp(Vector) (Variables|Default|GetStartLocation) (Variables|Default|GetEndLocation) _newtrack_0) false false)))))

(event EventBeginPlay
  (Variables|Default|SetStartLocation (Transformation|GetWorldLocation (Variables|Default|GetMovingTile)))
  (Variables|Default|SetEndLocation (Transformation|GetWorldLocation (Variables|Default|Getend%20point)))
  (Components|Timeline|SetPlayRate (Variables|Default|GetplatformMoving) (Variables|Default|GetPlayRate)))

(fn ConstructionScript)