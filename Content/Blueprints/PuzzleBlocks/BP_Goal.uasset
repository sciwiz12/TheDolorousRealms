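; BP_Goal is a puzzle-block goal that shows whether a BP_Pushblock is resting in its trigger box.
; On BeginPlay it gives the Ere component a dynamic material instance glowing red.
; Box overlaps turn it green when a pushblock's Cube component enters and a slightly more orange red when it leaves.
; The feedback is purely visual, with no occupancy count or completion signal.
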(event OnComponentBeginOverlap(Box)
  (params (OverlappedComponent :type Primitive%20Component%20Object%20Reference) (OtherActor :type Actor%20Object%20Reference) (OtherComp :type Primitive%20Component%20Object%20Reference) (OtherBodyIndex :type Integer) (bFromSweep :type Boolean) (SweepResult :type Hit%20Result%20Structure%20%28by%20ref%29))
  (bind _asbp_pushblock (Utilities|Casting|CastToBP_Pushblock OtherActor))
  (if (== OtherComp (Variables|/Game/Blueprints/PuzzleBlocks/BP_Pushblock.BP_Pushblock_C|GetCube _asbp_pushblock))
    (Rendering|Material|SetVectorParameterValue (stale EventBeginPlay _returnvalue) "Colour" "(R=0.027681,G=1.000000,B=0.000000,A=1.000000)" :!class /Script/Engine.MaterialInstanceDynamic)))

(event OnComponentEndOverlap(Box)
  (params (OverlappedComponent :type Primitive%20Component%20Object%20Reference) (OtherActor :type Actor%20Object%20Reference) (OtherComp :type Primitive%20Component%20Object%20Reference) (OtherBodyIndex :type Integer))
  (bind _asbp_pushblock (Utilities|Casting|CastToBP_Pushblock OtherActor))
  (if (== OtherComp (Variables|/Game/Blueprints/PuzzleBlocks/BP_Pushblock.BP_Pushblock_C|GetCube _asbp_pushblock))
    (Rendering|Material|SetVectorParameterValue (stale EventBeginPlay _returnvalue) "Colour" "(R=1.000000,G=0.068705,B=0.000000,A=1.000000)" :!class /Script/Engine.MaterialInstanceDynamic)))

(event EventBeginPlay
  (bind _ere (Variables|Default|Getere))
  (bind _returnvalue (Rendering|Material|CreateDynamicMaterialInstance _ere 0 "/Game/ArtAssets/Materials/Mat_PuzzleBlock.Mat_PuzzleBlock" "None" :!class /Script/Engine.PrimitiveComponent))
  (Rendering|Material|SetMaterial _ere 0 _returnvalue)
  (Rendering|Material|SetScalarParameterValue _returnvalue "Intensity" 2e+01 :!class /Script/Engine.MaterialInstanceDynamic)
  (Rendering|Material|SetVectorParameterValue _returnvalue "Colour" "(R=1.000000,G=0.000000,B=0.028356,A=1.000000)" :!class /Script/Engine.MaterialInstanceDynamic))

(fn ConstructionScript)