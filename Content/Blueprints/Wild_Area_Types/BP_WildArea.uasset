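; Wild encounter zone that can start random monster battles when the player character or boat overlaps its respective trigger box.
; A GrassInterval counter on the overlapping pawn limits rolls to periodic entries, each tested against Threshold.
; A successful roll halts player movement and picks a monster from MonsterTable by cumulative spawn weight.
; Duplicate Battle macros store that class in GI_Main and open the battle menu if none exists.
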(event OnComponentEndOverlap(Box)
  (params (OverlappedComponent :type Primitive%20Component%20Object%20Reference) (OtherActor :type Actor%20Object%20Reference) (OtherComp :type Primitive%20Component%20Object%20Reference) (OtherBodyIndex :type Integer))
  (Variables|Default|SetinWildArea false))

(event OnComponentBeginOverlap(Box1)
  (params (OverlappedComponent :type Primitive%20Component%20Object%20Reference) (OtherActor :type Actor%20Object%20Reference) (OtherComp :type Primitive%20Component%20Object%20Reference) (OtherBodyIndex :type Integer) (bFromSweep :type Boolean) (SweepResult :type Hit%20Result%20Structure%20%28by%20ref%29))
  (bind _asbp_new_boat (Utilities|Casting|CastToBP_NewBoat OtherActor))
  (bind _output_get (Variables|Default|SetAs%20BP%20Boat _asbp_new_boat))
  (if (<= (Variables|/Game/Blueprints/BP_NewBoat.BP_NewBoat_C|GetGrassInterval _output_get) 0)
    (bind _result (Math|Integer|IncrementInt (Variables|/Game/Blueprints/BP_NewBoat.BP_NewBoat_C|GetGrassInterval (Variables|Default|GetAs%20BP%20Boat)))
      (:%20%20
        (Variables|/Game/Blueprints/BP_NewBoat.BP_NewBoat_C|SetGrassInterval (Variables|Default|GetAs%20BP%20Boat) _result)
        (Variables|Default|SetinWildArea true)
        (if (Variables|Default|GetinWildArea)
          (Variables|Default|SetRandom%20Number (Math|Random|RandomIntegerinRange 0 100))
          (if (<= (Variables|Default|GetRandom%20Number) (Variables|Default|GetThreshold))
            (Pawn|Components|CharacterMovement|SetMovementMode (Variables|/Script/Engine.Character|GetCharacterMovement (Game|GetPlayerCharacter 0)) "MOVE_None" 0)
            (|Battle_2)))))
    (elif (>= (Variables|/Game/Blueprints/BP_NewBoat.BP_NewBoat_C|GetGrassInterval _output_get) 5)
      (Variables|/Game/Blueprints/BP_NewBoat.BP_NewBoat_C|SetGrassInterval (Variables|Default|GetAs%20BP%20Boat) 0)
      (else
        (bind _result_2 (Math|Integer|IncrementInt (Variables|/Game/Blueprints/BP_NewBoat.BP_NewBoat_C|GetGrassInterval (Variables|Default|GetAs%20BP%20Boat)))
          (:%20%20
            (Variables|/Game/Blueprints/BP_NewBoat.BP_NewBoat_C|SetGrassInterval (Variables|Default|GetAs%20BP%20Boat) _result_2)))))))

(event OnComponentEndOverlap(Box1)
  (params (OverlappedComponent :type Primitive%20Component%20Object%20Reference) (OtherActor :type Actor%20Object%20Reference) (OtherComp :type Primitive%20Component%20Object%20Reference) (OtherBodyIndex :type Integer))
  (Variables|Default|SetinWildArea false))

(event OnComponentBeginOverlap(Box)
  (params (OverlappedComponent :type Primitive%20Component%20Object%20Reference) (OtherActor :type Actor%20Object%20Reference) (OtherComp :type Primitive%20Component%20Object%20Reference) (OtherBodyIndex :type Integer) (bFromSweep :type Boolean) (SweepResult :type Hit%20Result%20Structure%20%28by%20ref%29))
  (bind _asbp_character (Utilities|Casting|CastToBP_Character OtherActor))
  (bind _output_get (Variables|Default|SetAs%20BP%20Character _asbp_character))
  (if (<= (Variables|/Game/Blueprints/Avatar/BP_Character.BP_Character_C|GetGrassInterval _output_get) 0)
    (bind _result (Math|Integer|IncrementInt (Variables|/Game/Blueprints/Avatar/BP_Character.BP_Character_C|GetGrassInterval (Variables|Default|GetAs%20BP%20Character)))
      (:%20%20
        (Variables|/Game/Blueprints/Avatar/BP_Character.BP_Character_C|SetGrassInterval (Variables|Default|GetAs%20BP%20Character) _result)
        (Variables|Default|SetinWildArea true)
        (if (Variables|Default|GetinWildArea)
          (Variables|Default|SetRandom%20Number (Math|Random|RandomIntegerinRange 0 100))
          (if (<= (Variables|Default|GetRandom%20Number) (Variables|Default|GetThreshold))
            (Pawn|Components|CharacterMovement|SetMovementMode (Variables|/Script/Engine.Character|GetCharacterMovement (Game|GetPlayerCharacter 0)) "MOVE_None" 0)
            (|Battle)))))
    (elif (>= (Variables|/Game/Blueprints/Avatar/BP_Character.BP_Character_C|GetGrassInterval _output_get) 5)
      (Variables|/Game/Blueprints/Avatar/BP_Character.BP_Character_C|SetGrassInterval (Variables|Default|GetAs%20BP%20Character) 0)
      (else
        (bind _result_2 (Math|Integer|IncrementInt (Variables|/Game/Blueprints/Avatar/BP_Character.BP_Character_C|GetGrassInterval (Variables|Default|GetAs%20BP%20Character)))
          (:%20%20
            (Variables|/Game/Blueprints/Avatar/BP_Character.BP_Character_C|SetGrassInterval (Variables|Default|GetAs%20BP%20Character) _result_2)))))))

(fn ConstructionScript)

(fn MonsterLookUP
  (Variables|Default|SetRandom%20Value (Math|Random|RandomIntegerinRange 1 (Variables|Default|GetRVMax)))
  (CallFunction|SetRefbyProbability)
  (return (Variables|Default|GetMonsterClassReference)))

(fn AddtoMonsterTable
  (params (Monster%20Struct :type Struct%20Monster%20Structure%20%28by%20ref%29))
  (bind _returnvalue (Utilities|Array|Add (Variables|Default|GetMonsterTable) Monster%20Struct))
  (Variables|Default|SetRVMax (+ (.ChancetoSpawninWild (Utilities|Struct|BreakStruct_MonsterDetails (.MonsterDetails (Utilities|Struct|BreakStruct_Monster (Utilities|Array|Get(acopy) (Variables|Default|GetMonsterTable) _returnvalue))))) (Variables|Default|GetRVMax))))

(fn SetRefbyProbability
  (for _array_element (Variables|Default|GetMonsterTable)
    (if (> (Variables|Default|GetRandom%20Value) (Variables|Default|GetCurrTotalPossibility))
      (bind _output_get (Variables|Default|SetCurrTotalPossibility (+ (.ChancetoSpawninWild (Utilities|Struct|BreakStruct_MonsterDetails (.MonsterDetails (Utilities|Struct|BreakStruct_Monster _array_element)))) (Variables|Default|GetCurrTotalPossibility))))
      (if (<= (Variables|Default|GetRandom%20Value) _output_get)
        (Variables|Default|SetMonsterClassReference (.ClassReference (Utilities|Struct|BreakStruct_MonsterDetails (.MonsterDetails (Utilities|Struct|BreakStruct_Monster _array_element))))))))
  (Variables|Default|SetCurrTotalPossibility 0))