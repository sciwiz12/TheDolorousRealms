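; BP_Trainer is a trainer actor that starts a one-time battle when the player presses Interact inside its trigger box.
; Overlap shows a text prompt and opens an input gate until the battle flag is set.
; Interacting freezes player movement, spawns BP_C_Strength at Box1 and calls Battle.
; Battle rolls a monster from a cumulative spawn-weight table, stores its class in GI_Main and opens the battle menu widget.
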(event OnComponentEndOverlap(Box)
  (params (OverlappedComponent :type Primitive%20Component%20Object%20Reference) (OtherActor :type Actor%20Object%20Reference) (OtherComp :type Primitive%20Component%20Object%20Reference) (OtherBodyIndex :type Integer))
  (Input|DisableInput (Game|GetPlayerController 0))
  (Utilities|Casting|CastToBP_Character OtherActor)
  (Development|SetHiddeninGame (Variables|Default|GetTextRender) true false)
  (Utilities|FlowControl|Gate true) ; enters at Close
)

(event OnComponentBeginOverlap(Box)
  (params (OverlappedComponent :type Primitive%20Component%20Object%20Reference) (OtherActor :type Actor%20Object%20Reference) (OtherComp :type Primitive%20Component%20Object%20Reference) (OtherBodyIndex :type Integer) (bFromSweep :type Boolean) (SweepResult :type Hit%20Result%20Structure%20%28by%20ref%29))
  (Utilities|Casting|CastToBP_Character OtherActor)
  (if (not (Variables|Default|GetBatte?))
    (Input|EnableInput (Game|GetPlayerController 0))
    (Development|SetHiddeninGame (Variables|Default|GetTextRender) false false)
    (Utilities|FlowControl|Gate true) ; enters at Open
  ))

(event Input|ActionEvents|InputActionInteract
  (params (Key :type Key%20Structure :default "None"))
  (:Pressed
    (Utilities|FlowControl|Gate true
      (:Exit
        (Pawn|Components|CharacterMovement|SetMovementMode (Variables|/Script/Engine.Character|GetCharacterMovement (Game|GetPlayerCharacter 0)) "MOVE_None" 0)
        (Game|SpawnActorfromClass "/Game/Blueprints/InventorySystem/MoveScrolls/BP_C_Strength.BP_C_Strength_C" (Math|Transform|MakeTransform (Transformation|GetWorldLocation (Variables|Default|GetBox1)) "0, 0, 0" "1,1,1") "Undefined" 0 0)
        (Variables|Default|SetBatte? true)
        (|Battle)))))

(fn ConstructionScript)

(fn MonsterLookUP
  (Variables|Default|SetRandom%20Value (Math|Random|RandomIntegerinRange 1 (Variables|Default|GetRVMax)))
  (CallFunction|SetRefbyProbability)
  (return (Variables|Default|GetMonsterClassReference)))

(fn AddtoMonsterTable
  (params (Monster%20Struct :type Struct%20Monster%20Structure%20%28by%20ref%29))
  (bind _returnvalue (Utilities|Array|Add (Variables|Default|GetMonsterTable) Monster%20Struct))
  (Variables|Default|SetRVMax (+ (.ChancetoSpawninWild (Utilities|Struct|BreakStruct_MonsterDetails (.MonsterDetails (Utilities|Struct|BreakStruct_Monster (Utilities|Array|Get(acopy) (Variables|Default|GetMonsterTable) _returnvalue))))) (Variables|Default|GetRVMax))))

(fn SetRefbyProbability
  (for _array_element (Variables|Default|GetMonsterTable)
    (if (> (Variables|Default|GetRandom%20Value) (Variables|Default|GetCurrTotalPossibility))
      (bind _output_get (Variables|Default|SetCurrTotalPossibility (+ (.ChancetoSpawninWild (Utilities|Struct|BreakStruct_MonsterDetails (.MonsterDetails (Utilities|Struct|BreakStruct_Monster _array_element)))) (Variables|Default|GetCurrTotalPossibility))))
      (if (<= (Variables|Default|GetRandom%20Value) _output_get)
        (Variables|Default|SetMonsterClassReference (.ClassReference (Utilities|Struct|BreakStruct_MonsterDetails (.MonsterDetails (Utilities|Struct|BreakStruct_Monster _array_element))))))))
  (Variables|Default|SetCurrTotalPossibility 0))