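; Rock variant of a wild area that defines which monsters belong to it.
; On BeginPlay it fills the monster table with a bat, three goblin types and two mushroom sizes, passing each monster's class defaults to AddToMonsterTable.
; The construction script only runs the parent's, and this Blueprint adds no other logic.
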(event EventBeginPlay
  (CallFunction|AddtoMonsterTable (Utilities|GetClassDefaults (Variables|Default|GetMr_Bat)))
  (CallFunction|AddtoMonsterTable (Utilities|GetClassDefaults (Variables|Default|GetGoblinMage)))
  (CallFunction|AddtoMonsterTable (Utilities|GetClassDefaults (Variables|Default|GetGoblinMelee)))
  (CallFunction|AddtoMonsterTable (Utilities|GetClassDefaults (Variables|Default|GetGoblinRange)))
  (CallFunction|AddtoMonsterTable (Utilities|GetClassDefaults (Variables|Default|GetSmallMushroom)))
  (CallFunction|AddtoMonsterTable (Utilities|GetClassDefaults (Variables|Default|GetBigMushroom))))

(fn ConstructionScript
  (|CallParentFunction))