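; BP_C_MagicArea is a wild area type that supplies the magic-themed monsters for that area.
; On BeginPlay it passes the class defaults of five MagicMonster classes to AddToMonsterTable, one call each, to fill the area's monster table.
; The construction script only calls the parent's version.
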(event EventBeginPlay
  (CallFunction|AddtoMonsterTable (Utilities|GetClassDefaults (Variables|Default|GetMagicMonster1)))
  (CallFunction|AddtoMonsterTable (Utilities|GetClassDefaults (Variables|Default|GetMagicMonster2)))
  (CallFunction|AddtoMonsterTable (Utilities|GetClassDefaults (Variables|Default|GetMagic%20Monster3)))
  (CallFunction|AddtoMonsterTable (Utilities|GetClassDefaults (Variables|Default|GetMagic%20MOnster%204)))
  (CallFunction|AddtoMonsterTable (Utilities|GetClassDefaults (Variables|Default|GetMagic%20monster%205))))

(fn ConstructionScript
  (|CallParentFunction))