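; BP_C_NormalArea is a wild area type that defines which monsters belong to the normal area.
; On BeginPlay it reads class defaults for Normal, Orge, Hawk, Slither and Bear and passes each to AddToMonsterTable to fill its monster table.
; The construction script only calls the parent, and the file holds no other logic, such as how the table gets used.
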(event EventBeginPlay
  (CallFunction|AddtoMonsterTable (Utilities|GetClassDefaults (Variables|Default|GetNormal)))
  (CallFunction|AddtoMonsterTable (Utilities|GetClassDefaults (Variables|Default|GetOrge)))
  (CallFunction|AddtoMonsterTable (Utilities|GetClassDefaults (Variables|Default|GetHawk)))
  (CallFunction|AddtoMonsterTable (Utilities|GetClassDefaults (Variables|Default|GetSlither)))
  (CallFunction|AddtoMonsterTable (Utilities|GetClassDefaults (Variables|Default|GetBear))))

(fn ConstructionScript
  (|CallParentFunction))