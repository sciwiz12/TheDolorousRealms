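; BP_C_DarkArea is a wild area Blueprint for the dark area, defining which monsters belong to it.
; On BeginPlay it passes the class defaults of Snake, GraveLeopard, BloodLion and BoneWolf to AddToMonsterTable, one call per monster.
; It holds no other logic of its own, and its construction script only calls the parent's.
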(event EventBeginPlay
  (CallFunction|AddtoMonsterTable (Utilities|GetClassDefaults (Variables|Default|GetSnake)))
  (CallFunction|AddtoMonsterTable (Utilities|GetClassDefaults (Variables|Default|GetGrave%20Leopard)))
  (CallFunction|AddtoMonsterTable (Utilities|GetClassDefaults (Variables|Default|GetBlood%20Lion)))
  (CallFunction|AddtoMonsterTable (Utilities|GetClassDefaults (Variables|Default|GetBone%20Wolf))))

(fn ConstructionScript
  (|CallParentFunction))