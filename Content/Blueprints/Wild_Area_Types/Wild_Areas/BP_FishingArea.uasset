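; Fishing spot that registers itself on the overlapping player character and starts wild water-monster battles.
; FishingInteract shows a spear sprite if HasSpear, which Tick rotates then thrusts using frame counters before setting a short timer.
; StartBattle hides and resets the spear, disables player movement and opens the battle menu.
; The monster is a weighted random pick from a BeginPlay-built table, stored in GI_Main.
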(event OnComponentBeginOverlap(Box)
  (params (OverlappedComponent :type Primitive%20Component%20Object%20Reference) (OtherActor :type Actor%20Object%20Reference) (OtherComp :type Primitive%20Component%20Object%20Reference) (OtherBodyIndex :type Integer) (bFromSweep :type Boolean) (SweepResult :type Hit%20Result%20Structure%20%28by%20ref%29))
  (bind _asbp_character (Utilities|Casting|CastToBP_Character OtherActor))
  (bind _output_get (Variables|Default|SetAs%20BP%20Character _asbp_character))
  (Variables|/Game/Blueprints/Avatar/BP_Character.BP_Character_C|SetFishingSpot _output_get self)
  (Variables|Default|SetinWildArea true))

(event OnComponentEndOverlap(Box)
  (params (OverlappedComponent :type Primitive%20Component%20Object%20Reference) (OtherActor :type Actor%20Object%20Reference) (OtherComp :type Primitive%20Component%20Object%20Reference) (OtherBodyIndex :type Integer))
  (Variables|Default|SetinWildArea false))

(event Custom|FishingInteract
  (if (Variables|Default|GetinWildArea)
    (CallFunction|FishingSpearAnimation)))

(event Custom|Start%20Battle
  (bind _papersprite (Variables|Default|GetPaperSprite))
  (CallFunction|InvisAnim)
  (Transformation|SetWorldRotation _papersprite (Variables|Default|GetOriginal%20Rotation) false false)
  (Transformation|SetRelativeLocation _papersprite (Variables|Default|GetOriginal%20Location) false false)
  (Pawn|Components|CharacterMovement|SetMovementMode (Variables|/Script/Engine.Character|GetCharacterMovement (Game|GetPlayerCharacter 0)) "MOVE_None" 0)
  (|Battle_2_2))

(event EventBeginPlay
  (bind _papersprite (Variables|Default|GetPaperSprite))
  (CallFunction|AddtoMonsterTable (Utilities|GetClassDefaults (Variables|Default|GetWaterMonster1)))
  (CallFunction|AddtoMonsterTable (Utilities|GetClassDefaults (Variables|Default|GetWaterMonster2)))
  (CallFunction|AddtoMonsterTable (Utilities|GetClassDefaults (Variables|Default|GetWaterMonster3)))
  (CallFunction|AddtoMonsterTable (Utilities|GetClassDefaults (Variables|Default|GetWaterMonster4)))
  (CallFunction|AddtoMonsterTable (Utilities|GetClassDefaults (Variables|Default|GetWaterMonster5)))
  (Variables|Default|SetOriginal%20Rotation (Transformation|GetWorldRotation _papersprite))
  (Variables|Default|SetOriginal%20Location (Variables|/Script/Engine.SceneComponent|GetRelativeLocation _papersprite)))

(event Collision|EventActorBeginOverlap
  (params (OtherActor :type Actor%20Object%20Reference)))

(event EventTick
  (params (DeltaSeconds :type Float%20%28single-precision%29))
  (bind _papersprite (Variables|Default|GetPaperSprite))
  (bind _papersprite_2 (Variables|Default|GetPaperSprite))
  (bind _locspeed (Variables|Default|GetLocSpeed))
  (bind _relativerotation (Variables|/Script/Engine.SceneComponent|GetRelativeRotation _papersprite))
  (bind _relativelocation (Variables|/Script/Engine.SceneComponent|GetRelativeLocation _papersprite_2))
  (Utilities|FlowControl|Sequence
    (:then_0
      (if (Variables|Default|GetAnimateRot)
        (Transformation|SetRelativeRotation _papersprite (Math|Rotator|MakeRotator (.roll _relativerotation) (.pitch _relativerotation) (+ (.yaw _relativerotation) (Variables|Default|GetRotSpeed))) false false)
        (bind _result (Math|Integer|IncrementInt (Variables|Default|GetCount))
          (:%20%20
            (Variables|Default|SetCount _result)
            (if (>= (Variables|Default|GetCount) (Variables|Default|GetRotationThreshold))
              (Variables|Default|SetAnimateRot false)
              (Variables|Default|SetAnimateLoc true)
              (Variables|Default|SetCount 0))))))
    (:then_1
      (if (Variables|Default|GetAnimateLoc)
        (Transformation|SetRelativeLocation _papersprite_2 (Math|Vector|MakeVector (- (.x _relativelocation) _locspeed) (+ (.y _relativelocation) _locspeed) (.z _relativelocation)) false false)
        (bind _result_2 (Math|Integer|IncrementInt (Variables|Default|GetCount))
          (:%20%20
            (Variables|Default|SetCount _result_2)
            (if (>= (Variables|Default|GetCount) (Variables|Default|GetLocationThreshold))
              (Variables|Default|SetAnimateLoc false)
              (Variables|Default|SetCount 0)
              (Utilities|Time|SetTimerbyEvent (EventDispatchers|CreateEvent :!event Custom|Start%20Battle) 1.0))))))))

(fn ConstructionScript)

(fn FishingSpearAnimation
  (bind _papersprite (Variables|Default|GetPaperSprite))
  (bind _spritecolor (Variables|/Script/Paper2D.PaperSpriteComponent|GetSpriteColor _papersprite))
  (if (Variables|Default|GetHasSpear)
    (Sprite|SetSpriteColor _papersprite (Utilities|Struct|MakeLinearColor (.r _spritecolor) (.g _spritecolor) (.b _spritecolor) 1.0))
    (Variables|Default|SetAnimateRot true)))

(fn MonsterLookUP
  (Variables|Default|SetRandom%20Value (Math|Random|RandomIntegerinRange 1 (Variables|Default|GetRVMax)))
  (CallFunction|SetRefbyProbability)
  (return (Variables|Default|GetMonsterClassReference)))

(fn AddtoMonsterTable
  (params (Monster%20Struct :type Struct%20Monster%20Structure%20%28by%20ref%29))
  (bind _returnvalue (Utilities|Array|Add (Variables|Default|GetMonsterTable) Monster%20Struct))
  (Variables|Default|SetRVMax (+ (.ChancetoSpawninWild (Utilities|Struct|BreakStruct_MonsterDetails (.MonsterDetails (Utilities|Struct|BreakStruct_Monster (Utilities|Array|Get(acopy) (Variables|Default|GetMonsterTable) _returnvalue))))) (Variables|Default|GetRVMax))))

(fn SetRefbyProbability
  (for _array_element (Variables|Default|GetMonsterTable)
    (if (> (Variables|Default|GetRandom%20Value) (Variables|Default|GetCurrTotalPossibility))
      (bind _output_get (Variables|Default|SetCurrTotalPossibility (+ (.ChancetoSpawninWild (Utilities|Struct|BreakStruct_MonsterDetails (.MonsterDetails (Utilities|Struct|BreakStruct_Monster _array_element)))) (Variables|Default|GetCurrTotalPossibility))))
      (if (<= (Variables|Default|GetRandom%20Value) _output_get)
        (Variables|Default|SetMonsterClassReference (.ClassReference (Utilities|Struct|BreakStruct_MonsterDetails (.MonsterDetails (Utilities|Struct|BreakStruct_Monster _array_element))))))))
  (Variables|Default|SetCurrTotalPossibility 0))

(fn InvisAnim
  (bind _papersprite (Variables|Default|GetPaperSprite))
  (bind _spritecolor (Variables|/Script/Paper2D.PaperSpriteComponent|GetSpriteColor _papersprite))
  (Sprite|SetSpriteColor _papersprite (Utilities|Struct|MakeLinearColor (.r _spritecolor) (.g _spritecolor) (.b _spritecolor) 0.0)))