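; Poison-type wild area that registers the monsters belonging to it.
; On BeginPlay it reads the class defaults of five poison monster classes and passes each to AddToMonsterTable.
; The construction script only calls the parent's, and the graph holds no other logic of its own.
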(event EventBeginPlay
  (CallFunction|AddtoMonsterTable (Utilities|GetClassDefaults (Variables|Default|GetPoisonMonster1)))
  (CallFunction|AddtoMonsterTable (Utilities|GetClassDefaults (Variables|Default|GetPoisonMOnster2)))
  (CallFunction|AddtoMonsterTable (Utilities|GetClassDefaults (Variables|Default|GetPoisonMOnster3)))
  (CallFunction|AddtoMonsterTable (Utilities|GetClassDefaults (Variables|Default|GetPoisonMOnster4)))
  (CallFunction|AddtoMonsterTable (Utilities|GetClassDefaults (Variables|Default|GetPoisonMOnster5))))

(fn ConstructionScript
  (|CallParentFunction))