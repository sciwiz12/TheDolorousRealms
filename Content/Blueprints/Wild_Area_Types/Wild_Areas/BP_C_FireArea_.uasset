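; Fire-themed wild area Blueprint that defines which monsters belong to this area.
; On BeginPlay it passes the class defaults of five monsters, from Slamander to Testomon, to AddToMonsterTable to fill the area's monster table.
; The construction script only calls its parent, and the file itself contains no other logic.
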(event EventBeginPlay
  (CallFunction|AddtoMonsterTable (Utilities|GetClassDefaults (Variables|Default|GetSlamander)))
  (CallFunction|AddtoMonsterTable (Utilities|GetClassDefaults (Variables|Default|GetFlamemon)))
  (CallFunction|AddtoMonsterTable (Utilities|GetClassDefaults (Variables|Default|GetFireImp)))
  (CallFunction|AddtoMonsterTable (Utilities|GetClassDefaults (Variables|Default|GetHound)))
  (CallFunction|AddtoMonsterTable (Utilities|GetClassDefaults (Variables|Default|Gettestomon))))

(fn ConstructionScript
  (|CallParentFunction))