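; BP_C_IceArea is the ice-themed wild area Blueprint that sets which monsters belong to that area.
; On BeginPlay it passes the class defaults of Spikes and FrostGolem to AddToMonsterTable.
; Matching entries for IceFairy, Yeti and Ice are present but disconnected, so they never reach the table.
; The construction script only calls the parent's.
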(event EventBeginPlay
  (CallFunction|AddtoMonsterTable (Utilities|GetClassDefaults (Variables|Default|GetSpikes)))
  (CallFunction|AddtoMonsterTable (Utilities|GetClassDefaults (Variables|Default|GetFrost%20Golem))))

(fn ConstructionScript
  (|CallParentFunction))