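; BP_C_WaterArea is a water-type wild area that supplies the monsters for its monster table.
; On BeginPlay it reads the class defaults of five water monster classes and passes each to AddToMonsterTable.
; Its construction script only calls the parent version.
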(event EventBeginPlay
  (CallFunction|AddtoMonsterTable (Utilities|GetClassDefaults (Variables|Default|GetWaterMonster1)))
  (CallFunction|AddtoMonsterTable (Utilities|GetClassDefaults (Variables|Default|GetWaterMonster2)))
  (CallFunction|AddtoMonsterTable (Utilities|GetClassDefaults (Variables|Default|GetWaterMonster3)))
  (CallFunction|AddtoMonsterTable (Utilities|GetClassDefaults (Variables|Default|GetWaterMonster4)))
  (CallFunction|AddtoMonsterTable (Utilities|GetClassDefaults (Variables|Default|GetWaterMonster5))))

(fn ConstructionScript
  (|CallParentFunction))