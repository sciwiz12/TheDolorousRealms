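; BP_NPC_GateGuardian is an NPC tied to a gate that tracks whether its monster roster has been defeated.
; Box overlap by BP_Character passes the Gate and this guardian to that character's MoveExecuter component.
; CheckifDeafeated orders the roster, counts monsters below one health and sets IsDefeated once the count reaches six.
; MonstersDefeated is not reset here, so repeated checks accumulate.
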(event OnComponentBeginOverlap(Box)
  (params (OverlappedComponent :type Primitive%20Component%20Object%20Reference) (OtherActor :type Actor%20Object%20Reference) (OtherComp :type Primitive%20Component%20Object%20Reference) (OtherBodyIndex :type Integer) (bFromSweep :type Boolean) (SweepResult :type Hit%20Result%20Structure%20%28by%20ref%29))
  (bind _asbp_character (Utilities|Casting|CastToBP_Character OtherActor))
  (Variables|/Game/Blueprints/Moves/BP_Component_MoveExecuter.BP_Component_MoveExecuter_C|SetGate (Variables|/Game/Blueprints/Avatar/BP_Character.BP_Character_C|GetBP_Component_MoveExecuter _asbp_character) (Variables|Default|GetGate))
  (Variables|/Game/Blueprints/Moves/BP_Component_MoveExecuter.BP_Component_MoveExecuter_C|SetGate%20Guardian (Variables|/Game/Blueprints/Avatar/BP_Character.BP_Character_C|GetBP_Component_MoveExecuter _asbp_character) self))

(event Custom|CheckifDeafeated
  (bind _bp_component_monsterroster (Variables|Default|GetBP_Component_MonsterRoster))
  (Default|SetOrder _bp_component_monsterroster)
  (for _array_element (Variables|/Game/Blueprints/MonsterAssets/BP_Component_MonsterRoster.BP_Component_MonsterRoster_C|GetMonsterArray _bp_component_monsterroster)
    (if (< (.Health (Utilities|Struct|BreakStruct_Stats (.Stats (Utilities|Struct|BreakStruct_Monster _array_element)))) 1.0)
      (bind _result (Math|Integer|IncrementInt (Variables|Default|GetMonstersDefeated))
        (:%20%20
          (Variables|Default|SetMonstersDefeated _result)))))
  (if (>= (Variables|Default|GetMonstersDefeated) 6)
    (Variables|Default|SetIsDefeated true)))

(event EventBeginPlay)

(event Collision|EventActorBeginOverlap
  (params (OtherActor :type Actor%20Object%20Reference)))

(event EventTick
  (params (DeltaSeconds :type Float%20%28single-precision%29)))

(fn ConstructionScript
  (|CallParentFunction))