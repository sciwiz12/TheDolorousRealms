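; BP_NPC is a configurable NPC that shows dialog when the player overlaps its box, optionally freezing movement to force interaction.
; A resettable DoOnce steps through NPCText rows, then flags select a tutorial movie, trainer battle, party heal or item shop.
; BeginPlay builds its six-monster roster, which Battle heals before opening the battle menu.
; Battles can repeat, drop items or be illusory, and ending overlap can spawn a strength item.
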(event OnComponentBeginOverlap(Box)
  (params (OverlappedComponent :type Primitive%20Component%20Object%20Reference) (OtherActor :type Actor%20Object%20Reference) (OtherComp :type Primitive%20Component%20Object%20Reference) (OtherBodyIndex :type Integer) (bFromSweep :type Boolean) (SweepResult :type Hit%20Result%20Structure%20%28by%20ref%29))
  (Utilities|Casting|CastToBP_Character OtherActor)
  (Development|SetHiddeninGame (Variables|Default|GetTextRender) false false)
  (bind _returnvalue (UserInterface|CreateWidget "/Game/Blueprints/GUIs/GUI_Dialog_NPC.GUI_Dialog_NPC_C"))
  (bind _output_get (Variables|Default|SetDialogUI _returnvalue))
  (UserInterface|Viewport|AddtoViewport _output_get 0)
  (if (Variables|Default|GetForcesBattle)
    (Pawn|Components|CharacterMovement|SetMovementMode (Variables|/Script/Engine.Character|GetCharacterMovement (Game|GetPlayerCharacter 0)) "MOVE_None" 0)
    (CallFunction|ForceInteraction)))

(event OnComponentEndOverlap(Box)
  (params (OverlappedComponent :type Primitive%20Component%20Object%20Reference) (OtherActor :type Actor%20Object%20Reference) (OtherComp :type Primitive%20Component%20Object%20Reference) (OtherBodyIndex :type Integer))
  (Utilities|Casting|CastToBP_Character OtherActor)
  (Development|SetHiddeninGame (Variables|Default|GetTextRender) true false)
  (Widget|RemovefromParent (Variables|Default|GetDialogUI))
  (if (Variables|Default|GetSpawn%20Item)
    (Game|SpawnActorfromClass "/Game/Blueprints/InventorySystem/MoveScrolls/BP_C_Strength.BP_C_Strength_C" (Math|Transform|MakeTransform "-27327.0,14524.0,-19290.000000" "0, 0, 0" "1,1,1") "Undefined" 0 0)))

(event Custom|Reset%20dialog
  (bind _returnvalue (Game|GetPlayerCharacter 0))
  (bind _returnvalue_2 (Game|GetPlayerCharacter 0))
  (bind _dialogui (Variables|Default|GetDialogUI))
  (bind _charactermovement (Variables|/Script/Engine.Character|GetCharacterMovement _returnvalue_2))
  (bind _charactermovement_2 (Variables|/Script/Engine.Character|GetCharacterMovement _returnvalue))
  (Utilities|FlowControl|DoOnce false) ; enters at Reset
)

(event Custom|ForceInteraction
  (bind _returnvalue (Game|GetPlayerCharacter 0))
  (bind _returnvalue_2 (Game|GetPlayerCharacter 0))
  (bind _dialogui (Variables|Default|GetDialogUI))
  (bind _charactermovement (Variables|/Script/Engine.Character|GetCharacterMovement _returnvalue_2))
  (bind _charactermovement_2 (Variables|/Script/Engine.Character|GetCharacterMovement _returnvalue))
  (Utilities|FlowControl|DoOnce false
    (:Completed
      (Variables|/Game/Blueprints/GUIs/GUI_Dialog_NPC.GUI_Dialog_NPC_C|Settest _dialogui (Variables|Default|GetNPCText))
      (Widget|SetVisibility (Variables|/Game/Blueprints/GUIs/GUI_Dialog_NPC.GUI_Dialog_NPC_C|GetImage_0 _dialogui) "Visible")
      (if (> (+ (Variables|/Game/Blueprints/GUIs/GUI_Dialog_NPC.GUI_Dialog_NPC_C|Gettext%20row _dialogui) 1) (- (Utilities|Array|Length (Variables|Default|GetNPCText)) 1))
        (Widget|RemovefromParent (Variables|Default|GetDialogUI))
        (if (Variables|Default|GetTutorial)
          (bind _returnvalue_3 (UserInterface|CreateWidget "/Game/Blueprints/GUIs/GUI_Movies.GUI_Movies_C" (Game|GetPlayerController 0)))
          (Variables|/Game/Blueprints/GUIs/GUI_Movies.GUI_Movies_C|SetMediaPlayer _returnvalue_3 (Variables|Default|GetMediaPlayer))
          (Variables|/Game/Blueprints/GUIs/GUI_Movies.GUI_Movies_C|SetMedia%20Source _returnvalue_3 (Variables|Default|GetMedia%20Source))
          (Variables|/Game/Blueprints/GUIs/GUI_Movies.GUI_Movies_C|SetMaterial _returnvalue_3 (Variables|Default|GetMaterial))
          (UserInterface|Viewport|AddtoViewport _returnvalue_3 0)
          (elif (Variables|Default|GetWillBattle)
            (if (Variables|Default|GetMultBattles)
              (CallFunction|ResetDialog))
            (CallFunction|Battle)
            (if (Variables|Default|GetDropsItem)
              (Game|SpawnActorfromClass (Variables|Default|GetItemToSpawn) (Math|Transform|MakeTransform (Transformation|GetActorLocation self) "0, 0, 0" "1,1,1") "AdjustIfPossibleButAlwaysSpawn" 0 0)
              (switch Utilities|FlowControl|Switch|SwitchonEMovementMode (Variables|/Script/Engine.CharacterMovementComponent|GetMovementMode _charactermovement)
                (:MOVE_None
                  (Pawn|Components|CharacterMovement|SetMovementMode _charactermovement "MOVE_Walking" 0)))
              (else
                (switch Utilities|FlowControl|Switch|SwitchonEnum_IllusionType (Variables|Default|GetIllusionType)
                  (:NewEnumerator2
                    (Variables|/Game/Blueprints/GUIs/GUI_BattleMenu_Test1.GUI_BattleMenu_Test1_C|SetIllusory (Variables|Default|GetBattleGui) true)
                    (Actor|DestroyActor)
                    (switch Utilities|FlowControl|Switch|SwitchonEMovementMode (Variables|/Script/Engine.CharacterMovementComponent|GetMovementMode _charactermovement_2)
                      (:MOVE_None
                        (Pawn|Components|CharacterMovement|SetMovementMode _charactermovement_2 "MOVE_Walking" 0)))))))
            (elif (Variables|Default|GetIsHealer)
              (bind _asbp_character (Utilities|Casting|CastToBP_Character (Game|GetPlayerCharacter 0)))
              (Default|HealParty (Variables|/Game/Blueprints/Avatar/BP_Character.BP_Character_C|GetMonsterRoster _asbp_character))
              (CallFunction|ResetDialog)
              (elif (Variables|Default|GetIs%20ShopKeep)
                (Pawn|Components|CharacterMovement|SetMovementMode (Variables|/Script/Engine.Character|GetCharacterMovement (Game|GetPlayerCharacter 0)) "MOVE_None" 0)
                (bind _foundwidgets (Widget|GetAllWidgetsOfClass "/Game/Blueprints/GUIs/GUI_ItemShop.GUI_ItemShop_C" true))
                (Utilities|IsValid (Utilities|Array|Get(acopy) _foundwidgets)
                  (:Is%20Valid
                    (Variables|/Game/Blueprints/GUIs/GUI_ItemShop.GUI_ItemShop_C|SetShopInventory (Utilities|Array|Get(acopy) _foundwidgets) (Variables|Default|GetInventory))
                    (CallFunction|ResetDialog))
                  (:Is%20Not%20Valid
                    (bind _returnvalue_4 (UserInterface|CreateWidget "/Game/Blueprints/GUIs/GUI_ItemShop.GUI_ItemShop_C"))
                    (Variables|/Game/Blueprints/GUIs/GUI_ItemShop.GUI_ItemShop_C|SetShopInventory _returnvalue_4 (Variables|Default|GetInventory))
                    (UserInterface|Viewport|AddtoViewport _returnvalue_4 0)
                    (CallFunction|ResetDialog)))))))
        (else
          (Variables|/Game/Blueprints/GUIs/GUI_Dialog_NPC.GUI_Dialog_NPC_C|Settext%20row (Variables|Default|GetDialogUI) (+ (Variables|/Game/Blueprints/GUIs/GUI_Dialog_NPC.GUI_Dialog_NPC_C|Gettext%20row _dialogui) 1))
          (CallFunction|ResetDialog))))))

(event EventBeginPlay
  (bind _bp_component_monsterroster (Variables|Default|GetBP_Component_MonsterRoster))
  (bind _monsterrosterstruct (Variables|/Game/Blueprints/MonsterAssets/BP_Component_MonsterRoster.BP_Component_MonsterRoster_C|GetMonsterRosterStruct _bp_component_monsterroster))
  (Default|AddtoArray (Variables|Default|GetBP_Component_MonsterRoster) (.monster_1 _monsterrosterstruct) (.monster_2 _monsterrosterstruct) (.monster_3 _monsterrosterstruct) (.monster_4 _monsterrosterstruct) (.monster_5 _monsterrosterstruct) (.monster_6 _monsterrosterstruct))
  (Default|SetOrder (Variables|Default|GetBP_Component_MonsterRoster))
  (Default|AssignPartyIDs (Variables|Default|GetBP_Component_MonsterRoster)))

(event EventEventDialogOccurs
  (bind _returnvalue (Game|GetPlayerCharacter 0))
  (bind _returnvalue_2 (Game|GetPlayerCharacter 0))
  (bind _dialogui (Variables|Default|GetDialogUI))
  (bind _charactermovement (Variables|/Script/Engine.Character|GetCharacterMovement _returnvalue_2))
  (bind _charactermovement_2 (Variables|/Script/Engine.Character|GetCharacterMovement _returnvalue))
  (Utilities|FlowControl|DoOnce false
    (:Completed
      (Variables|/Game/Blueprints/GUIs/GUI_Dialog_NPC.GUI_Dialog_NPC_C|Settest _dialogui (Variables|Default|GetNPCText))
      (Widget|SetVisibility (Variables|/Game/Blueprints/GUIs/GUI_Dialog_NPC.GUI_Dialog_NPC_C|GetImage_0 _dialogui) "Visible")
      (if (> (+ (Variables|/Game/Blueprints/GUIs/GUI_Dialog_NPC.GUI_Dialog_NPC_C|Gettext%20row _dialogui) 1) (- (Utilities|Array|Length (Variables|Default|GetNPCText)) 1))
        (Widget|RemovefromParent (Variables|Default|GetDialogUI))
        (if (Variables|Default|GetTutorial)
          (bind _returnvalue_3 (UserInterface|CreateWidget "/Game/Blueprints/GUIs/GUI_Movies.GUI_Movies_C" (Game|GetPlayerController 0)))
          (Variables|/Game/Blueprints/GUIs/GUI_Movies.GUI_Movies_C|SetMediaPlayer _returnvalue_3 (Variables|Default|GetMediaPlayer))
          (Variables|/Game/Blueprints/GUIs/GUI_Movies.GUI_Movies_C|SetMedia%20Source _returnvalue_3 (Variables|Default|GetMedia%20Source))
          (Variables|/Game/Blueprints/GUIs/GUI_Movies.GUI_Movies_C|SetMaterial _returnvalue_3 (Variables|Default|GetMaterial))
          (UserInterface|Viewport|AddtoViewport _returnvalue_3 0)
          (elif (Variables|Default|GetWillBattle)
            (if (Variables|Default|GetMultBattles)
              (CallFunction|ResetDialog))
            (CallFunction|Battle)
            (if (Variables|Default|GetDropsItem)
              (Game|SpawnActorfromClass (Variables|Default|GetItemToSpawn) (Math|Transform|MakeTransform (Transformation|GetActorLocation self) "0, 0, 0" "1,1,1") "AdjustIfPossibleButAlwaysSpawn" 0 0)
              (switch Utilities|FlowControl|Switch|SwitchonEMovementMode (Variables|/Script/Engine.CharacterMovementComponent|GetMovementMode _charactermovement)
                (:MOVE_None
                  (Pawn|Components|CharacterMovement|SetMovementMode _charactermovement "MOVE_Walking" 0)))
              (else
                (switch Utilities|FlowControl|Switch|SwitchonEnum_IllusionType (Variables|Default|GetIllusionType)
                  (:NewEnumerator2
                    (Variables|/Game/Blueprints/GUIs/GUI_BattleMenu_Test1.GUI_BattleMenu_Test1_C|SetIllusory (Variables|Default|GetBattleGui) true)
                    (Actor|DestroyActor)
                    (switch Utilities|FlowControl|Switch|SwitchonEMovementMode (Variables|/Script/Engine.CharacterMovementComponent|GetMovementMode _charactermovement_2)
                      (:MOVE_None
                        (Pawn|Components|CharacterMovement|SetMovementMode _charactermovement_2 "MOVE_Walking" 0)))))))
            (elif (Variables|Default|GetIsHealer)
              (bind _asbp_character (Utilities|Casting|CastToBP_Character (Game|GetPlayerCharacter 0)))
              (Default|HealParty (Variables|/Game/Blueprints/Avatar/BP_Character.BP_Character_C|GetMonsterRoster _asbp_character))
              (CallFunction|ResetDialog)
              (elif (Variables|Default|GetIs%20ShopKeep)
                (Pawn|Components|CharacterMovement|SetMovementMode (Variables|/Script/Engine.Character|GetCharacterMovement (Game|GetPlayerCharacter 0)) "MOVE_None" 0)
                (bind _foundwidgets (Widget|GetAllWidgetsOfClass "/Game/Blueprints/GUIs/GUI_ItemShop.GUI_ItemShop_C" true))
                (Utilities|IsValid (Utilities|Array|Get(acopy) _foundwidgets)
                  (:Is%20Valid
                    (Variables|/Game/Blueprints/GUIs/GUI_ItemShop.GUI_ItemShop_C|SetShopInventory (Utilities|Array|Get(acopy) _foundwidgets) (Variables|Default|GetInventory))
                    (CallFunction|ResetDialog))
                  (:Is%20Not%20Valid
                    (bind _returnvalue_4 (UserInterface|CreateWidget "/Game/Blueprints/GUIs/GUI_ItemShop.GUI_ItemShop_C"))
                    (Variables|/Game/Blueprints/GUIs/GUI_ItemShop.GUI_ItemShop_C|SetShopInventory _returnvalue_4 (Variables|Default|GetInventory))
                    (UserInterface|Viewport|AddtoViewport _returnvalue_4 0)
                    (CallFunction|ResetDialog)))))))
        (else
          (Variables|/Game/Blueprints/GUIs/GUI_Dialog_NPC.GUI_Dialog_NPC_C|Settext%20row (Variables|Default|GetDialogUI) (+ (Variables|/Game/Blueprints/GUIs/GUI_Dialog_NPC.GUI_Dialog_NPC_C|Gettext%20row _dialogui) 1))
          (CallFunction|ResetDialog))))))

(fn ConstructionScript)

(fn Battle
  (Default|HealParty (Variables|Default|GetBP_Component_MonsterRoster))
  (bind _foundwidgets (Widget|GetAllWidgetsOfClass "/Game/Blueprints/GUIs/GUI_BattleMenu_Test1.GUI_BattleMenu_Test1_C" true))
  (Utilities|IsValid (Utilities|Array|Get(acopy) _foundwidgets)
    (:Is%20Not%20Valid
      (bind _returnvalue (UserInterface|CreateWidget "/Game/Blueprints/GUIs/GUI_BattleMenu_Test1.GUI_BattleMenu_Test1_C" (Game|GetPlayerController 0)))
      (Variables|Default|SetBattleGui _returnvalue)
      (Variables|/Game/Blueprints/GUIs/GUI_BattleMenu_Test1.GUI_BattleMenu_Test1_C|SetDefeatText (Variables|Default|GetBattleGui) (Variables|Default|GetDefeat%20Text))
      (Variables|/Game/Blueprints/GUIs/GUI_BattleMenu_Test1.GUI_BattleMenu_Test1_C|SetMoneyToAdd (Variables|Default|GetBattleGui) (Variables|Default|GetMoney%20to%20Add))
      (Variables|/Game/Blueprints/GUIs/GUI_BattleMenu_Test1.GUI_BattleMenu_Test1_C|SetIs%20End%20Boss (Variables|Default|GetBattleGui) (Variables|Default|GetIs%20end%20boss))
      (Variables|/Game/Blueprints/GUIs/GUI_BattleMenu_Test1.GUI_BattleMenu_Test1_C|SetIsTrainerBattle (Variables|Default|GetBattleGui) true)
      (Variables|/Game/Blueprints/GUIs/GUI_BattleMenu_Test1.GUI_BattleMenu_Test1_C|SetLevel (Variables|Default|GetBattleGui) (Variables|Default|GetLevel))
      (Variables|/Game/Blueprints/GUIs/GUI_BattleMenu_Test1.GUI_BattleMenu_Test1_C|SetEnemyTrainer (Variables|Default|GetBattleGui) self)
      (UserInterface|Viewport|AddtoViewport (Variables|Default|GetBattleGui) 0)
      (Variables|/Script/Engine.PlayerController|SetbShowMouseCursor (Game|GetPlayerController 0) true)
      (if (not (Variables|Default|GetMultBattles))
        (Variables|Default|SetWillBattle false)))))