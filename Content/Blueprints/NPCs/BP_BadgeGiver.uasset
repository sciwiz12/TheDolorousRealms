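; BP_BadgeGiver is an NPC that talks to the player and grants the Blue Badge.
; Overlapping its Box with BP_Character reveals a TextRender and creates a GUI_Dialog_NPC widget; leaving hides and removes them.
; EventDialogOccurs advances dialog rows through a DoOnce, reset after each advance, choosing NPCText1 or NPCText2 by HasBlueBadge.
; Finishing NPCText1 closes the widget and sets HasBlueBadge on the character.
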(event OnComponentBeginOverlap(Box)
  (params (OverlappedComponent :type Primitive%20Component%20Object%20Reference) (OtherActor :type Actor%20Object%20Reference) (OtherComp :type Primitive%20Component%20Object%20Reference) (OtherBodyIndex :type Integer) (bFromSweep :type Boolean) (SweepResult :type Hit%20Result%20Structure%20%28by%20ref%29))
  (bind _asbp_character (Utilities|Casting|CastToBP_Character OtherActor))
  (Development|SetHiddeninGame (Variables|Default|GetTextRender) false false)
  (bind _returnvalue (UserInterface|CreateWidget "/Game/Blueprints/GUIs/GUI_Dialog_NPC.GUI_Dialog_NPC_C"))
  (bind _output_get (Variables|Default|SetDialogUI _returnvalue))
  (UserInterface|Viewport|AddtoViewport _output_get 0))

(event OnComponentEndOverlap(Box)
  (params (OverlappedComponent :type Primitive%20Component%20Object%20Reference) (OtherActor :type Actor%20Object%20Reference) (OtherComp :type Primitive%20Component%20Object%20Reference) (OtherBodyIndex :type Integer))
  (Utilities|Casting|CastToBP_Character OtherActor)
  (Development|SetHiddeninGame (Variables|Default|GetTextRender) true false)
  (Widget|RemovefromParent (Variables|Default|GetDialogUI)))

(event Custom|Reset%20dialog
  (bind _dialogui (Variables|Default|GetDialogUI))
  (bind _dialogui_2 (Variables|Default|GetDialogUI))
  (Utilities|FlowControl|DoOnce false) ; enters at Reset
)

(event EventEventDialogOccurs
  (bind _dialogui (Variables|Default|GetDialogUI))
  (bind _dialogui_2 (Variables|Default|GetDialogUI))
  (Utilities|FlowControl|DoOnce false
    (:Completed
      (if (Variables|/Game/Blueprints/Avatar/BP_Character.BP_Character_C|GetHasBlueBadge (stale OnComponentBeginOverlap(Box) _asbp_character))
        (Variables|/Game/Blueprints/GUIs/GUI_Dialog_NPC.GUI_Dialog_NPC_C|Settest _dialogui_2 (Variables|Default|GetNPCText_2))
        (Widget|SetVisibility (Variables|/Game/Blueprints/GUIs/GUI_Dialog_NPC.GUI_Dialog_NPC_C|GetImage_0 _dialogui_2) "Visible")
        (if (> (+ (Variables|/Game/Blueprints/GUIs/GUI_Dialog_NPC.GUI_Dialog_NPC_C|Gettext%20row _dialogui_2) 1) (- (Utilities|Array|Length (Variables|Default|GetNPCText_2)) 1))
          (Widget|RemovefromParent (Variables|Default|GetDialogUI))
          (else
            (Variables|/Game/Blueprints/GUIs/GUI_Dialog_NPC.GUI_Dialog_NPC_C|Settext%20row (Variables|Default|GetDialogUI) (+ (Variables|/Game/Blueprints/GUIs/GUI_Dialog_NPC.GUI_Dialog_NPC_C|Gettext%20row _dialogui_2) 1))
            (CallFunction|ResetDialog)))
        (else
          (Variables|/Game/Blueprints/GUIs/GUI_Dialog_NPC.GUI_Dialog_NPC_C|Settest _dialogui (Variables|Default|GetNPCText_1))
          (Widget|SetVisibility (Variables|/Game/Blueprints/GUIs/GUI_Dialog_NPC.GUI_Dialog_NPC_C|GetImage_0 _dialogui) "Visible")
          (if (> (+ (Variables|/Game/Blueprints/GUIs/GUI_Dialog_NPC.GUI_Dialog_NPC_C|Gettext%20row _dialogui) 1) (- (Utilities|Array|Length (Variables|Default|GetNPCText_1)) 1))
            (Widget|RemovefromParent (Variables|Default|GetDialogUI))
            (Variables|/Game/Blueprints/Avatar/BP_Character.BP_Character_C|SetHasBlueBadge (stale OnComponentBeginOverlap(Box) _asbp_character) true)
            (else
              (Variables|/Game/Blueprints/GUIs/GUI_Dialog_NPC.GUI_Dialog_NPC_C|Settext%20row (Variables|Default|GetDialogUI) (+ (Variables|/Game/Blueprints/GUIs/GUI_Dialog_NPC.GUI_Dialog_NPC_C|Gettext%20row _dialogui) 1))
              (CallFunction|ResetDialog))))))))

(fn ConstructionScript)