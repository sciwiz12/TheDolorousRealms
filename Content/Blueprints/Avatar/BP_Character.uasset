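; Player character Blueprint that handles movement, interaction and in-game UI, and starts a new game through GI_Main on BeginPlay.
; Input drives control-yaw-relative movement, sandals-gated sprint, interaction with items, dialog actors and storage, and mouse-wheel forwarding to the CircleOne level manager.
; Climbing and boulder pushing are flag-gated calls to a move executer component.
; The Pokegear pauses the game, while the unfinished pause menu toggle only disables movement.
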(event OnComponentBeginOverlap(Box)
  (params (OverlappedComponent :type Primitive%20Component%20Object%20Reference) (OtherActor :type Actor%20Object%20Reference) (OtherComp :type Primitive%20Component%20Object%20Reference) (OtherBodyIndex :type Integer) (bFromSweep :type Boolean) (SweepResult :type Hit%20Result%20Structure%20%28by%20ref%29))
  ;[1 1 1] Shield Trigger
)

(event EventBeginPlay
  (Utilities|FlowControl|Sequence
    (:then_0
      (Pawn|Possess (Pawn|GetController) self)
      (Variables|/Script/Engine.CharacterMovementComponent|SetMaxWalkSpeed (Variables|Character|GetCharacterMovement) 3e+02))
    (:then_1
      (Pawn|SetControlRotation (Game|GetPlayerController 0) (Transformation|GetActorRotation))
      (bind _asgi_main (Utilities|Casting|CastToGI_Main (Game|GetGameInstance)))
      (Variables|Default|SetAs%20GI%20Main _asgi_main))
    (:then_2
      (bind _asgi_main_2 (Utilities|Casting|CastToGI_Main (Game|GetGameInstance)))
      (Default|NewGame _asgi_main_2))
    (:then_3
      (bind _returnvalue (UserInterface|CreateWidget "/Game/Blueprints/GUIs/GUI_Currency.GUI_Currency_C" (Game|GetPlayerController 0)))
      (UserInterface|Viewport|AddtoViewport _returnvalue 0))
    (:then_4
      (CallFunction|PauseMenu true))))

(event Collision|EventActorBeginOverlap
  (params (OtherActor :type Actor%20Object%20Reference)))

(event Input|ActionEvents|InputActionSprint
  (params (Key :type Key%20Structure :default "None"))
  (bind _charactermovement (Variables|Character|GetCharacterMovement))
  (:Pressed
    (if (Variables|Default|GetWingedSandals)
      (Variables|/Script/Engine.CharacterMovementComponent|SetMaxWalkSpeed _charactermovement 5e+02)))
  (:Released
    (Variables|/Script/Engine.CharacterMovementComponent|SetMaxWalkSpeed _charactermovement 3e+02)))

(event Input|AxisEvents|InputAxisMoveUp
  (params (AxisValue :type Float%20%28single-precision%29))
  (Pawn|Input|AddMovementInput (Math|Vector|GetForwardVector (Math|Rotator|MakeRotator 0.0 0.0 (.Yaw (Math|Rotator|BreakRotator (Pawn|GetControlRotation :!class /Script/Engine.Pawn))))) (* AxisValue (Variables|Default|GetDirectionFactor)) false))

(event Input|AxisEvents|InputAxisMoveRight
  (params (AxisValue :type Float%20%28single-precision%29))
  (Pawn|Input|AddMovementInput (Math|Vector|GetRightVector (Math|Rotator|MakeRotator 0.0 0.0 (.Yaw (Math|Rotator|BreakRotator (Pawn|GetControlRotation :!class /Script/Engine.Pawn))))) (* AxisValue (Variables|Default|GetDirectionFactor)) false))

(event Input|MouseEvents|MouseWheelAxis
  (params (AxisValue :type Float%20%28single-precision%29))
  (bind _outactors (Actor|GetAllActorsOfClass "/Game/Blueprints/CircleOne/BP_LevelManager_CircleOne.BP_LevelManager_CircleOne_C"))
  (bind _asbp_level_manager_circle_one (Utilities|Casting|CastToBP_LevelManager_CircleOne (Utilities|Array|Get(acopy) _outactors)))
  (Variables|/Game/Blueprints/CircleOne/BP_LevelManager_CircleOne.BP_LevelManager_CircleOne_C|SetAxisValue _asbp_level_manager_circle_one AxisValue))

(event Input|KeyboardEvents|W
  (params (Key :type Key%20Structure :default "None"))
  (:Pressed
    (Variables|Default|SetIsWPressed true))
  (:Released
    (Variables|Default|SetIsWPressed false)))

(event Input|KeyboardEvents|S
  (params (Key :type Key%20Structure :default "None"))
  (:Pressed
    (Variables|Default|SetIsSPressed true))
  (:Released
    (Variables|Default|SetIsSPressed false)))

(event Input|KeyboardEvents|C
  (params (Key :type Key%20Structure :default "None"))
  (:Pressed
    (if (Variables|Default|GetCanClimb)
      (Default|Climb (Variables|/Game/Blueprints/Moves/BP_Component_MoveExecuter.BP_Component_MoveExecuter_C|GetClimb (Variables|Default|GetBP_Component_MoveExecuter))))))

(event Input|KeyboardEvents|U
  (params (Key :type Key%20Structure :default "None")))

(event Input|KeyboardEvents|SpaceBar
  (params (Key :type Key%20Structure :default "None"))
  ;[1 1 1] Push Space bar to push boulder after it has been activacted
  (:Pressed
    (if (Variables|Default|GetMoveBoulder)
      (Audio|PlaySoundatLocation "/Game/AudioAssets/stone-push-sound.stone-push-sound" "0, 0, 0" "0, 0, 0" 1.0 1.0 0.0 0 0 0)
      (Default|Moveboulder (Variables|Default|GetBP_Component_MoveExecuter)))))

(event Input|KeyboardEvents|Q
  (params (Key :type Key%20Structure :default "None"))
  ;[1 1 1] simulate Death
)

(event Input|KeyboardEvents|P
  (params (Key :type Key%20Structure :default "None"))
  (bind _charactermovement (Variables|Character|GetCharacterMovement))
  (:Pressed
    (Utilities|FlowControl|FlipFlop
      (:A
        (Pawn|Components|CharacterMovement|SetMovementMode _charactermovement "MOVE_None" 0)
        (Variables|Default|SetTogglePauseBool true))
      (:B
        (Pawn|Components|CharacterMovement|SetMovementMode _charactermovement "MOVE_Walking" 0)
        (Variables|Default|SetTogglePauseBool false)))
    (CallFunction|PauseMenu (Variables|Default|GetTogglePauseBool))))

(event Input|KeyboardEvents|A
  (params (Key :type Key%20Structure :default "None"))
  (:Pressed
    (Variables|Default|SetIsAPressed true))
  (:Released
    (Variables|Default|SetIsAPressed false)))

(event Input|KeyboardEvents|D
  (params (Key :type Key%20Structure :default "None"))
  (:Pressed
    (Variables|Default|SetIsDPressed true))
  (:Released
    (Variables|Default|SetIsDPressed false)))

(event Input|KeyboardEvents|P
  (params (Key :type Key%20Structure :default "None"))
  ;[1 1 1] ignoring pause functionality (still in progress)
)

(event Input|KeyboardEvents|Escape
  (params (Key :type Key%20Structure :default "None"))
  (bind _charactermovement (Variables|Character|GetCharacterMovement))
  (:Pressed
    (Utilities|FlowControl|FlipFlop
      (:A
        (Pawn|Components|CharacterMovement|SetMovementMode _charactermovement "MOVE_None" 0)
        (Variables|Default|SetTogglePauseBool true))
      (:B
        (Pawn|Components|CharacterMovement|SetMovementMode _charactermovement "MOVE_Walking" 0)
        (Variables|Default|SetTogglePauseBool false)))
    (CallFunction|PauseMenu (Variables|Default|GetTogglePauseBool))))

(event Input|KeyboardEvents|E
  (params (Key :type Key%20Structure :default "None"))
  (bind _storagesystem (Variables|Default|GetStorageSystem))
  (:Pressed
    (Utilities|FlowControl|Sequence
      (:then_0
        (Utilities|IsValid (Variables|Default|GetItem)
          (:Is%20Valid
            (Default|PlaySoundFX (Variables|Default|GetAs%20GI%20Main) "/Game/AudioAssets/SoundEffects/Select.Select")
            (Default|Interact (Variables|Default|GetItem)))
          (:Is%20Not%20Valid
            _))
        (bind _array_element (Utilities|Array|ForEachLoopwithBreak (Collision|GetOverlappingActors 0 :!class /Script/Engine.Actor) :!label _label)
          (:LoopBody
            (if (Utilities|DoesObjectImplementInterface _array_element "/Game/Blueprints/TestFolderForWildEncounters/Characters/BP_Interface_Dialog.BP_Interface_Dialog_C")
              (Default|PlaySoundFX (Variables|Default|GetAs%20GI%20Main) "/Game/AudioAssets/SoundEffects/Select.Select")
              (Class|BPInterfaceDialog|EventDialogOccurs(Message) _array_element)
              (goto _label Break)))))
      (:then_1
        (Utilities|IsValid _storagesystem
          (:Is%20Valid
            (Default|PlaySoundFX (Variables|Default|GetAs%20GI%20Main) "/Game/AudioAssets/SoundEffects/Select.Select")
            (Default|PlayerAccess _storagesystem)))))))

(event Input|KeyboardEvents|I
  (params (Key :type Key%20Structure :default "None"))
  (bind _returnvalue (Game|GetPlayerController 0))
  (:Pressed
    (Utilities|FlowControl|FlipFlop
      (:A
        (bind _returnvalue_2 (UserInterface|CreateWidget "/Game/Blueprints/GUIs/GUI_Pokegear.GUI_Pokegear_C"))
        (UserInterface|Viewport|AddtoViewport _returnvalue_2 0)
        (Game|SetGamePaused true)
        (Variables|/Script/Engine.PlayerController|SetbShowMouseCursor _returnvalue true))
      (:B
        (Widget|RemovefromParent _returnvalue_2)
        (Game|SetGamePaused false)
        (Variables|/Script/Engine.PlayerController|SetbShowMouseCursor _returnvalue false)))))

(event Input|KeyboardEvents|Q
  (params (Key :type Key%20Structure :default "None"))
  ;[1 1 1] Fire Protect Key
)

(event Input|KeyboardEvents|Tab
  (params (Key :type Key%20Structure :default "None"))
  (bind _charactermovement (Variables|Character|GetCharacterMovement))
  (:Pressed
    (Utilities|FlowControl|FlipFlop
      (:A
        (Pawn|Components|CharacterMovement|SetMovementMode _charactermovement "MOVE_None" 0)
        (Variables|Default|SetTogglePauseBool true))
      (:B
        (Pawn|Components|CharacterMovement|SetMovementMode _charactermovement "MOVE_Walking" 0)
        (Variables|Default|SetTogglePauseBool false)))
    (CallFunction|PauseMenu (Variables|Default|GetTogglePauseBool))))

(fn ConstructionScript)

(fn PauseMenu
  (params (Condition :type Boolean))
  (Variables|/Script/Engine.PlayerController|SetbShowMouseCursor (Game|GetPlayerController 0) Condition)
  (if Condition
    (bind _foundwidgets (Widget|GetAllWidgetsOfClass "/Game/Blueprints/GUIs/GUI_PauseMenu.GUI_PauseMenu_C" false))
    (Utilities|IsValid (Utilities|Array|Get(acopy) _foundwidgets)
      (:Is%20Valid
        (Widget|SetVisibility (Utilities|Array|Get(acopy) _foundwidgets) "Visible")
        (UserInterface|Viewport|AddtoViewport (Utilities|Array|Get(acopy) _foundwidgets) 0))
      (:Is%20Not%20Valid
        (bind _returnvalue (UserInterface|CreateWidget "/Game/Blueprints/GUIs/GUI_PauseMenu.GUI_PauseMenu_C"))
        (Variables|Default|SetPauseMenuWidget _returnvalue)))
    (else
      (Widget|RemovefromParent (Variables|Default|GetPauseMenuWidget)))))