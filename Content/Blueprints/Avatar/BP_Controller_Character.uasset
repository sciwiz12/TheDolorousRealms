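; Player controller that switches control between the on-foot character and the boat.
; Key 1 near the boat plays a creak sound, waits briefly, hides the character and possesses the first BP_NewBoat found.
; Key 2 near the exit does the reverse, possessing BP_Character, then moving the player character to a hardcoded location and unhiding it.
; The proximity flags gating both keys are not set in this graph.
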(event Input|KeyboardEvents|1
  (params (Key :type Key%20Structure))
  ;[1 1 1] possessing boat
  (:Pressed
    (if (Variables|Default|GetIsNearBoat)
      (Audio|PlaySound2D "/Game/AudioAssets/SFX/wooden-floor-creak-81237.wooden-floor-creak-81237" 1.0 1.0 0.0 0 0)
      (Utilities|FlowControl|Delay 2.0)
      (Rendering|SetActorHiddenInGame (Game|GetPlayerCharacter 0) true)
      (bind _outactors (Actor|GetAllActorsOfClass "/Game/Blueprints/BP_NewBoat.BP_NewBoat_C"))
      (Pawn|Possess (Utilities|Array|Get(acopy) _outactors)))))

(event Input|KeyboardEvents|2
  (params (Key :type Key%20Structure))
  (bind _returnvalue (Game|GetPlayerCharacter 0))
  (:Pressed
    ;[1 1 1] possessing player
    (if (Variables|Default|GetIsNearExit)
      (Audio|PlaySound2D "/Game/AudioAssets/SFX/wooden-floor-creak-81237.wooden-floor-creak-81237" 1.0 1.0 0.0 0 0)
      (Utilities|FlowControl|Delay 2.0)
      (bind _outactors (Actor|GetAllActorsOfClass "/Game/Blueprints/Avatar/BP_Character.BP_Character_C"))
      (Pawn|Possess (Utilities|Array|Get(acopy) _outactors))
      (Transformation|SetActorLocation _returnvalue "9155.000000,-1575.000000,350.000000" false false)
      (Rendering|SetActorHiddenInGame _returnvalue false))))

(fn ConstructionScript)