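; Main game instance for a monster-collecting game, handling single-slot save/load and global audio.
; Save and load copy player transform, inventory, monster roster, storage and level between BP_Character, Storagesystem and BP_SaveGame, with BeingLoaded flagging level loads.
; NewGame reuses an existing save or creates one with three starter monsters; RestartLevel deletes it.
; Audio functions manage 2D music and effects, including timed fades; countdown timer experiments are unused.
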(event Custom|SaveGame
  (bind _storagesystem (Variables|Default|GetStoragesystem))
  (bind _returnvalue (SaveGame|LoadGamefromSlot (Variables|Default|GetSave1)))
  (bind _asbp_save_game (Utilities|Casting|CastToBP_SaveGame _returnvalue))
  (bind _asbp_character (Utilities|Casting|CastToBP_Character (Game|GetPlayerCharacter 0))
    (:then
      (Variables|/Game/Blueprints/SaveLoad/BP_SaveGame.BP_SaveGame_C|SetPlayerTransform _asbp_save_game (Transformation|GetActorTransform _asbp_character))
      (Variables|/Game/Blueprints/SaveLoad/BP_SaveGame.BP_SaveGame_C|SetMonsterRoster _asbp_save_game (Variables|/Game/Blueprints/MonsterAssets/BP_Component_MonsterRoster.BP_Component_MonsterRoster_C|GetMonsterRosterStruct (Variables|/Game/Blueprints/Avatar/BP_Character.BP_Character_C|GetMonsterRoster _asbp_character)))
      (Default|SetOrder (Variables|/Game/Blueprints/Avatar/BP_Character.BP_Character_C|GetMonsterRoster _asbp_character))
      (Variables|/Game/Blueprints/SaveLoad/BP_SaveGame.BP_SaveGame_C|SetInventory _asbp_save_game (Variables|/Game/Blueprints/InventorySystem/BP_Inventory.BP_Inventory_C|GetStructInventory (Variables|/Game/Blueprints/Avatar/BP_Character.BP_Character_C|GetBP_Inventory _asbp_character))))
    (:CastFailed
      _))
  (bind _returnvalue_2 (Game|GetCurrentLevelName true))
  (Variables|/Game/Blueprints/SaveLoad/BP_SaveGame.BP_SaveGame_C|SetLevelName _asbp_save_game _returnvalue_2)
  (Utilities|IsValid _storagesystem
    (:Is%20Valid
      (Variables|/Game/Blueprints/SaveLoad/BP_SaveGame.BP_SaveGame_C|SetMonsterStruct _asbp_save_game (Variables|/Game/Blueprints/InventorySystem/BP_MonsterStorage.BP_MonsterStorage_C|GetMonsters _storagesystem)))
    (:Is%20Not%20Valid
      _))
  (Variables|Default|SetAs%20BP%20Save%20Game _asbp_save_game)
  (SaveGame|SaveGametoSlot _asbp_save_game (Variables|Default|GetSave1)))

(event Custom|New%20Game
  (bind _returnvalue (SaveGame|DoesSaveGameExist "Save1"))
  (if _returnvalue
    (bind _returnvalue_2 (SaveGame|LoadGamefromSlot (Variables|Default|GetSave1)))
    (bind _asbp_save_game (Utilities|Casting|CastToBP_SaveGame _returnvalue_2))
    (Variables|Default|SetAs%20BP%20Save%20Game _asbp_save_game)
    (if (Variables|Default|GetBeingLoaded)
      (bind _asbp_character (Utilities|Casting|CastToBP_Character (Game|GetPlayerCharacter 0)))
      (Transformation|SetActorTransform _asbp_character (Variables|/Game/Blueprints/SaveLoad/BP_SaveGame.BP_SaveGame_C|GetPlayerTransform (Variables|Default|GetAs%20BP%20Save%20Game)))
      (Variables|/Game/Blueprints/InventorySystem/BP_Inventory.BP_Inventory_C|SetStructInventory (Variables|/Game/Blueprints/Avatar/BP_Character.BP_Character_C|GetBP_Inventory _asbp_character) (Variables|/Game/Blueprints/SaveLoad/BP_SaveGame.BP_SaveGame_C|GetInventory (Variables|Default|GetAs%20BP%20Save%20Game)))
      (Variables|/Game/Blueprints/MonsterAssets/BP_Component_MonsterRoster.BP_Component_MonsterRoster_C|SetMonsterRosterStruct (Variables|/Game/Blueprints/Avatar/BP_Character.BP_Character_C|GetMonsterRoster _asbp_character) (Variables|/Game/Blueprints/SaveLoad/BP_SaveGame.BP_SaveGame_C|GetMonsterRoster (Variables|Default|GetAs%20BP%20Save%20Game))))
    (else
      (bind _returnvalue_3 (SaveGame|CreateSaveGameObject "/Game/Blueprints/SaveLoad/BP_SaveGame.BP_SaveGame_C"))
      (bind _output_get (Variables|Default|SetAs%20BP%20Save%20Game _returnvalue_3))
      (SaveGame|SaveGametoSlot _output_get (Variables|Default|GetSave1))
      (bind _asbp_character_2 (Utilities|Casting|CastToBP_Character (Game|GetPlayerCharacter 0)))
      (Variables|/Game/Blueprints/MonsterAssets/BP_Component_MonsterRoster.BP_Component_MonsterRoster_C|SetMonsterRosterStruct (Variables|/Game/Blueprints/Avatar/BP_Character.BP_Character_C|GetMonsterRoster _asbp_character_2) (Utilities|Struct|MakeStruct_MonsterRoster (Utilities|GetClassDefaults "/Game/Blueprints/MonsterAssets/JohnsMons/BP_BoneWolf.BP_BoneWolf_C") (Utilities|GetClassDefaults "/Game/Blueprints/MonsterAssets/JohnsMons/BP_GraveLeopard.BP_GraveLeopard_C") (Utilities|GetClassDefaults "/Game/Blueprints/MonsterAssets/JohnsMons/BP_BloodLion.BP_BloodLion_C") "(MonsterDetails_86_8DFBD9AA40500468EF80C382E2ACE38A=(ClassReference_12_E6BE22314C9C72CD9B5B2F83081DB27C=None,Name_13_FEB187FD4BB1FB8CA266FD8171986D71=\"\",Images_28_42911BE84027A19A60792FAE57940E93=,ElementalType_25_8AB48DF244F979A5D2AB7681ADFBA3D6=NewEnumerator0,ElementalSubType_26_600CA940488451F5F148EAA32D63AB06=NewEnumerator13,ChancetoSpawninWild_17_FB8FFA95400E250874AAC68E5245643E=0,PlaceInRoster_20_867F68F24A03C033C8EDB2BE2A8CF63F=NewEnumerator6,UniqueID_23_AA1DBB014530C31EE4B75CAA96EA3449=0.000000),LevelandXP_84_2B697C3E441D3CE3737E3DB406FA0037=(Level_2_71C401644B4329F342CA7E9D07950E11=0,XP_11_4D82DD03434EA725922B27A67A67A17D=0.000000,XPtoLevelUp_12_2926FF624018A540CFB56187B4B4ED1E=0.000000,Evolutions_13_9EEB8EBC4129A4E4E1C3D387CE48E513=(LevelThreshold_2_1308E8BC47DC5E67B43988967EE8793A=0,EvolutionReference_5_4E7B602E489D41DA37A51486640C5EB6=None)),Stats_81_73365ACA41B2F0C7BCE62EB1A727DF44=(Health_16_3004B651431E090062CE88B245E8048A=0.000000,TotalHealth_17_1522A5DF44A7A6C691DACA940AEA78EA=0.000000,Speed_18_C0D3D89F42577E81E8444B872C843673=0,Attack_19_0F2465BE41595B388FA6589D78620B29=0,SpecialAttack_20_F69EC9AE4942C28AA0A4FB91ED667CA8=0,Defense_21_946B9B9F472864574D53F1AFAE141488=0,SpecialDefense_22_C1FE2629487D6EEBE95DBD89EA041329=0,Evasion_23_A8ADDE4A44525E1CA28853911FCF7AB1=0),BaseStats_92_38D80BB44D0CEE69EF89A4B7EEAF8960=(Health_16_3004B651431E090062CE88B245E8048A=0.000000,TotalHealth_17_1522A5DF44A7A6C691DACA940AEA78EA=0.000000,Speed_18_C0D3D89F42577E81E8444B872C843673=0,Attack_19_0F2465BE41595B388FA6589D78620B29=0,SpecialAttack_20_F69EC9AE4942C28AA0A4FB91ED667CA8=0,Defense_21_946B9B9F472864574D53F1AFAE141488=0,SpecialDefense_22_C1FE2629487D6EEBE95DBD89EA041329=0,Evasion_23_A8ADDE4A44525E1CA28853911FCF7AB1=0,Factor_26_BDCB68704CDDECEC4BB9B4A3AEC8DA82=0.000000),StatusActive_47_4FFC0D354C689DDB36DC4CB05E930FB0=False,Status_51_6B1A05204FF4CCB2CC298089C573E986=NewEnumerator6,MovesList_79_096DA19A460DC9C09CD986B80FB87516=(Move1_2_C3908C7040914DA478CD9CB0202C689C=(MoveName_2_43F0BF544EAAF8A690427CB947E7131F=\"\",MoveType_22_07E95F2C41F3C9341B7904971492E67C=NewEnumerator0,ElementType_23_2FAF1B2B499571551749F6B39F4BC37D=NewEnumerator0,SubType_30_AE9CCCF34C44A8E40556BC935A44D0E8=NewEnumerator13,PhysicalSpecialStatus_8_5DC943EA407D54B86BB243AB74D2061F=NewEnumerator0,Damage_11_DDB65D3849CE29C5B91384868780960B=0.000000,StatusEffect_26_96750FA3440CC08E8E62D4B3652D80CF=(StatusEffectName_6_FA334B9A46A1625B9465C486DECB7109=\"\",StatusEffectType_18_502EF54F491DF29148F612953C32058B=NewEnumerator6,ChancetoActivate_29_0596FFD440B899CCBD8DD2B916E60F25=0.000000,StatusEffectDialogueText_7_EF66845C403B2941A9B0E48788D56C2D=\"\",StatusEffectSymbol_10_B772178E429378675266F495F7CB57D9=None,DamageOverType_21_2B1F28EA4CCA2CC5EF204AA0E2DBF95A=False,DOTDamage_27_E554A32045248BB7030520B5705802B6=0.000000,PreventsFromAttacking_23_5A5E14E44C3D17A7A3FE449E887CAB12=False),StatAffected_34_F783641C4EA304A29ABDDA945C1399E4=NewEnumerator0),Move2_6_1FDBAE674CB4AF337F4E52A5BEB44525=(MoveName_2_43F0BF544EAAF8A690427CB947E7131F=\"\",MoveType_22_07E95F2C41F3C9341B7904971492E67C=NewEnumerator0,ElementType_23_2FAF1B2B499571551749F6B39F4BC37D=NewEnumerator0,SubType_30_AE9CCCF34C44A8E40556BC935A44D0E8=NewEnumerator13,PhysicalSpecialStatus_8_5DC943EA407D54B86BB243AB74D2061F=NewEnumerator0,Damage_11_DDB65D3849CE29C5B91384868780960B=0.000000,StatusEffect_26_96750FA3440CC08E8E62D4B3652D80CF=(StatusEffectName_6_FA334B9A46A1625B9465C486DECB7109=\"\",StatusEffectType_18_502EF54F491DF29148F612953C32058B=NewEnumerator6,ChancetoActivate_29_0596FFD440B899CCBD8DD2B916E60F25=0.000000,StatusEffectDialogueText_7_EF66845C403B2941A9B0E48788D56C2D=\"\",StatusEffectSymbol_10_B772178E429378675266F495F7CB57D9=None,DamageOverType_21_2B1F28EA4CCA2CC5EF204AA0E2DBF95A=False,DOTDamage_27_E554A32045248BB7030520B5705802B6=0.000000,PreventsFromAttacking_23_5A5E14E44C3D17A7A3FE449E887CAB12=False),StatAffected_34_F783641C4EA304A29ABDDA945C1399E4=NewEnumerator0),Move3_7_BE0263184D8FD95A11746497F3836EE5=(MoveName_2_43F0BF544EAAF8A690427CB947E7131F=\"\",MoveType_22_07E95F2C41F3C9341B7904971492E67C=NewEnumerator0,ElementType_23_2FAF1B2B499571551749F6B39F4BC37D=NewEnumerator0,SubType_30_AE9CCCF34C44A8E40556BC935A44D0E8=NewEnumerator13,PhysicalSpecialStatus_8_5DC943EA407D54B86BB243AB74D2061F=NewEnumerator0,Damage_11_DDB65D3849CE29C5B91384868780960B=0.000000,StatusEffect_26_96750FA3440CC08E8E62D4B3652D80CF=(StatusEffectName_6_FA334B9A46A1625B9465C486DECB7109=\"\",StatusEffectType_18_502EF54F491DF29148F612953C32058B=NewEnumerator6,ChancetoActivate_29_0596FFD440B899CCBD8DD2B916E60F25=0.000000,StatusEffectDialogueText_7_EF66845C403B2941A9B0E48788D56C2D=\"\",StatusEffectSymbol_10_B772178E429378675266F495F7CB57D9=None,DamageOverType_21_2B1F28EA4CCA2CC5EF204AA0E2DBF95A=False,DOTDamage_27_E554A32045248BB7030520B5705802B6=0.000000,PreventsFromAttacking_23_5A5E14E44C3D17A7A3FE449E887CAB12=False),StatAffected_34_F783641C4EA304A29ABDDA945C1399E4=NewEnumerator0),Move4_8_3C9EA81B4DD2C43837432D9247CA531D=(MoveName_2_43F0BF544EAAF8A690427CB947E7131F=\"\",MoveType_22_07E95F2C41F3C9341B7904971492E67C=NewEnumerator0,ElementType_23_2FAF1B2B499571551749F6B39F4BC37D=NewEnumerator0,SubType_30_AE9CCCF34C44A8E40556BC935A44D0E8=NewEnumerator13,PhysicalSpecialStatus_8_5DC943EA407D54B86BB243AB74D2061F=NewEnumerator0,Damage_11_DDB65D3849CE29C5B91384868780960B=0.000000,StatusEffect_26_96750FA3440CC08E8E62D4B3652D80CF=(StatusEffectName_6_FA334B9A46A1625B9465C486DECB7109=\"\",StatusEffectType_18_502EF54F491DF29148F612953C32058B=NewEnumerator6,ChancetoActivate_29_0596FFD440B899CCBD8DD2B916E60F25=0.000000,StatusEffectDialogueText_7_EF66845C403B2941A9B0E48788D56C2D=\"\",StatusEffectSymbol_10_B772178E429378675266F495F7CB57D9=None,DamageOverType_21_2B1F28EA4CCA2CC5EF204AA0E2DBF95A=False,DOTDamage_27_E554A32045248BB7030520B5705802B6=0.000000,PreventsFromAttacking_23_5A5E14E44C3D17A7A3FE449E887CAB12=False),StatAffected_34_F783641C4EA304A29ABDDA945C1399E4=NewEnumerator0)),Battled_89_F480929841A407ED2344FA97712C4968=False)" "(MonsterDetails_86_8DFBD9AA40500468EF80C382E2ACE38A=(ClassReference_12_E6BE22314C9C72CD9B5B2F83081DB27C=None,Name_13_FEB187FD4BB1FB8CA266FD8171986D71=\"\",Images_28_42911BE84027A19A60792FAE57940E93=,ElementalType_25_8AB48DF244F979A5D2AB7681ADFBA3D6=NewEnumerator0,ElementalSubType_26_600CA940488451F5F148EAA32D63AB06=NewEnumerator13,ChancetoSpawninWild_17_FB8FFA95400E250874AAC68E5245643E=0,PlaceInRoster_20_867F68F24A03C033C8EDB2BE2A8CF63F=NewEnumerator6,UniqueID_23_AA1DBB014530C31EE4B75CAA96EA3449=0.000000),LevelandXP_84_2B697C3E441D3CE3737E3DB406FA0037=(Level_2_71C401644B4329F342CA7E9D07950E11=0,XP_11_4D82DD03434EA725922B27A67A67A17D=0.000000,XPtoLevelUp_12_2926FF624018A540CFB56187B4B4ED1E=0.000000,Evolutions_13_9EEB8EBC4129A4E4E1C3D387CE48E513=(LevelThreshold_2_1308E8BC47DC5E67B43988967EE8793A=0,EvolutionReference_5_4E7B602E489D41DA37A51486640C5EB6=None)),Stats_81_73365ACA41B2F0C7BCE62EB1A727DF44=(Health_16_3004B651431E090062CE88B245E8048A=0.000000,TotalHealth_17_1522A5DF44A7A6C691DACA940AEA78EA=0.000000,Speed_18_C0D3D89F42577E81E8444B872C843673=0,Attack_19_0F2465BE41595B388FA6589D78620B29=0,SpecialAttack_20_F69EC9AE4942C28AA0A4FB91ED667CA8=0,Defense_21_946B9B9F472864574D53F1AFAE141488=0,SpecialDefense_22_C1FE2629487D6EEBE95DBD89EA041329=0,Evasion_23_A8ADDE4A44525E1CA28853911FCF7AB1=0),BaseStats_92_38D80BB44D0CEE69EF89A4B7EEAF8960=(Health_16_3004B651431E090062CE88B245E8048A=0.000000,TotalHealth_17_1522A5DF44A7A6C691DACA940AEA78EA=0.000000,Speed_18_C0D3D89F42577E81E8444B872C843673=0,Attack_19_0F2465BE41595B388FA6589D78620B29=0,SpecialAttack_20_F69EC9AE4942C28AA0A4FB91ED667CA8=0,Defense_21_946B9B9F472864574D53F1AFAE141488=0,SpecialDefense_22_C1FE2629487D6EEBE95DBD89EA041329=0,Evasion_23_A8ADDE4A44525E1CA28853911FCF7AB1=0,Factor_26_BDCB68704CDDECEC4BB9B4A3AEC8DA82=0.000000),StatusActive_47_4FFC0D354C689DDB36DC4CB05E930FB0=False,Status_51_6B1A05204FF4CCB2CC298089C573E986=NewEnumerator6,MovesList_79_096DA19A460DC9C09CD986B80FB87516=(Move1_2_C3908C7040914DA478CD9CB0202C689C=(MoveName_2_43F0BF544EAAF8A690427CB947E7131F=\"\",MoveType_22_07E95F2C41F3C9341B7904971492E67C=NewEnumerator0,ElementType_23_2FAF1B2B499571551749F6B39F4BC37D=NewEnumerator0,SubType_30_AE9CCCF34C44A8E40556BC935A44D0E8=NewEnumerator13,PhysicalSpecialStatus_8_5DC943EA407D54B86BB243AB74D2061F=NewEnumerator0,Damage_11_DDB65D3849CE29C5B91384868780960B=0.000000,StatusEffect_26_96750FA3440CC08E8E62D4B3652D80CF=(StatusEffectName_6_FA334B9A46A1625B9465C486DECB7109=\"\",StatusEffectType_18_502EF54F491DF29148F612953C32058B=NewEnumerator6,ChancetoActivate_29_0596FFD440B899CCBD8DD2B916E60F25=0.000000,StatusEffectDialogueText_7_EF66845C403B2941A9B0E48788D56C2D=\"\",StatusEffectSymbol_10_B772178E429378675266F495F7CB57D9=None,DamageOverType_21_2B1F28EA4CCA2CC5EF204AA0E2DBF95A=False,DOTDamage_27_E554A32045248BB7030520B5705802B6=0.000000,PreventsFromAttacking_23_5A5E14E44C3D17A7A3FE449E887CAB12=False),StatAffected_34_F783641C4EA304A29ABDDA945C1399E4=NewEnumerator0),Move2_6_1FDBAE674CB4AF337F4E52A5BEB44525=(MoveName_2_43F0BF544EAAF8A690427CB947E7131F=\"\",MoveType_22_07E95F2C41F3C9341B7904971492E67C=NewEnumerator0,ElementType_23_2FAF1B2B499571551749F6B39F4BC37D=NewEnumerator0,SubType_30_AE9CCCF34C44A8E40556BC935A44D0E8=NewEnumerator13,PhysicalSpecialStatus_8_5DC943EA407D54B86BB243AB74D2061F=NewEnumerator0,Damage_11_DDB65D3849CE29C5B91384868780960B=0.000000,StatusEffect_26_96750FA3440CC08E8E62D4B3652D80CF=(StatusEffectName_6_FA334B9A46A1625B9465C486DECB7109=\"\",StatusEffectType_18_502EF54F491DF29148F612953C32058B=NewEnumerator6,ChancetoActivate_29_0596FFD440B899CCBD8DD2B916E60F25=0.000000,StatusEffectDialogueText_7_EF66845C403B2941A9B0E48788D56C2D=\"\",StatusEffectSymbol_10_B772178E429378675266F495F7CB57D9=None,DamageOverType_21_2B1F28EA4CCA2CC5EF204AA0E2DBF95A=False,DOTDamage_27_E554A32045248BB7030520B5705802B6=0.000000,PreventsFromAttacking_23_5A5E14E44C3D17A7A3FE449E887CAB12=False),StatAffected_34_F783641C4EA304A29ABDDA945C1399E4=NewEnumerator0),Move3_7_BE0263184D8FD95A11746497F3836EE5=(MoveName_2_43F0BF544EAAF8A690427CB947E7131F=\"\",MoveType_22_07E95F2C41F3C9341B7904971492E67C=NewEnumerator0,ElementType_23_2FAF1B2B499571551749F6B39F4BC37D=NewEnumerator0,SubType_30_AE9CCCF34C44A8E40556BC935A44D0E8=NewEnumerator13,PhysicalSpecialStatus_8_5DC943EA407D54B86BB243AB74D2061F=NewEnumerator0,Damage_11_DDB65D3849CE29C5B91384868780960B=0.000000,StatusEffect_26_96750FA3440CC08E8E62D4B3652D80CF=(StatusEffectName_6_FA334B9A46A1625B9465C486DECB7109=\"\",StatusEffectType_18_502EF54F491DF29148F612953C32058B=NewEnumerator6,ChancetoActivate_29_0596FFD440B899CCBD8DD2B916E60F25=0.000000,StatusEffectDialogueText_7_EF66845C403B2941A9B0E48788D56C2D=\"\",StatusEffectSymbol_10_B772178E429378675266F495F7CB57D9=None,DamageOverType_21_2B1F28EA4CCA2CC5EF204AA0E2DBF95A=False,DOTDamage_27_E554A32045248BB7030520B5705802B6=0.000000,PreventsFromAttacking_23_5A5E14E44C3D17A7A3FE449E887CAB12=False),StatAffected_34_F783641C4EA304A29ABDDA945C1399E4=NewEnumerator0),Move4_8_3C9EA81B4DD2C43837432D9247CA531D=(MoveName_2_43F0BF544EAAF8A690427CB947E7131F=\"\",MoveType_22_07E95F2C41F3C9341B7904971492E67C=NewEnumerator0,ElementType_23_2FAF1B2B499571551749F6B39F4BC37D=NewEnumerator0,SubType_30_AE9CCCF34C44A8E40556BC935A44D0E8=NewEnumerator13,PhysicalSpecialStatus_8_5DC943EA407D54B86BB243AB74D2061F=NewEnumerator0,Damage_11_DDB65D3849CE29C5B91384868780960B=0.000000,StatusEffect_26_96750FA3440CC08E8E62D4B3652D80CF=(StatusEffectName_6_FA334B9A46A1625B9465C486DECB7109=\"\",StatusEffectType_18_502EF54F491DF29148F612953C32058B=NewEnumerator6,ChancetoActivate_29_0596FFD440B899CCBD8DD2B916E60F25=0.000000,StatusEffectDialogueText_7_EF66845C403B2941A9B0E48788D56C2D=\"\",StatusEffectSymbol_10_B772178E429378675266F495F7CB57D9=None,DamageOverType_21_2B1F28EA4CCA2CC5EF204AA0E2DBF95A=False,DOTDamage_27_E554A32045248BB7030520B5705802B6=0.000000,PreventsFromAttacking_23_5A5E14E44C3D17A7A3FE449E887CAB12=False),StatAffected_34_F783641C4EA304A29ABDDA945C1399E4=NewEnumerator0)),Battled_89_F480929841A407ED2344FA97712C4968=False)" "(MonsterDetails_86_8DFBD9AA40500468EF80C382E2ACE38A=(ClassReference_12_E6BE22314C9C72CD9B5B2F83081DB27C=None,Name_13_FEB187FD4BB1FB8CA266FD8171986D71=\"\",Images_28_42911BE84027A19A60792FAE57940E93=,ElementalType_25_8AB48DF244F979A5D2AB7681ADFBA3D6=NewEnumerator0,ElementalSubType_26_600CA940488451F5F148EAA32D63AB06=NewEnumerator13,ChancetoSpawninWild_17_FB8FFA95400E250874AAC68E5245643E=0,PlaceInRoster_20_867F68F24A03C033C8EDB2BE2A8CF63F=NewEnumerator6,UniqueID_23_AA1DBB014530C31EE4B75CAA96EA3449=0.000000),LevelandXP_84_2B697C3E441D3CE3737E3DB406FA0037=(Level_2_71C401644B4329F342CA7E9D07950E11=0,XP_11_4D82DD03434EA725922B27A67A67A17D=0.000000,XPtoLevelUp_12_2926FF624018A540CFB56187B4B4ED1E=0.000000,Evolutions_13_9EEB8EBC4129A4E4E1C3D387CE48E513=(LevelThreshold_2_1308E8BC47DC5E67B43988967EE8793A=0,EvolutionReference_5_4E7B602E489D41DA37A51486640C5EB6=None)),Stats_81_73365ACA41B2F0C7BCE62EB1A727DF44=(Health_16_3004B651431E090062CE88B245E8048A=0.000000,TotalHealth_17_1522A5DF44A7A6C691DACA940AEA78EA=0.000000,Speed_18_C0D3D89F42577E81E8444B872C843673=0,Attack_19_0F2465BE41595B388FA6589D78620B29=0,SpecialAttack_20_F69EC9AE4942C28AA0A4FB91ED667CA8=0,Defense_21_946B9B9F472864574D53F1AFAE141488=0,SpecialDefense_22_C1FE2629487D6EEBE95DBD89EA041329=0,Evasion_23_A8ADDE4A44525E1CA28853911FCF7AB1=0),BaseStats_92_38D80BB44D0CEE69EF89A4B7EEAF8960=(Health_16_3004B651431E090062CE88B245E8048A=0.000000,TotalHealth_17_1522A5DF44A7A6C691DACA940AEA78EA=0.000000,Speed_18_C0D3D89F42577E81E8444B872C843673=0,Attack_19_0F2465BE41595B388FA6589D78620B29=0,SpecialAttack_20_F69EC9AE4942C28AA0A4FB91ED667CA8=0,Defense_21_946B9B9F472864574D53F1AFAE141488=0,SpecialDefense_22_C1FE2629487D6EEBE95DBD89EA041329=0,Evasion_23_A8ADDE4A44525E1CA28853911FCF7AB1=0,Factor_26_BDCB68704CDDECEC4BB9B4A3AEC8DA82=0.000000),StatusActive_47_4FFC0D354C689DDB36DC4CB05E930FB0=False,Status_51_6B1A05204FF4CCB2CC298089C573E986=NewEnumerator6,MovesList_79_096DA19A460DC9C09CD986B80FB87516=(Move1_2_C3908C7040914DA478CD9CB0202C689C=(MoveName_2_43F0BF544EAAF8A690427CB947E7131F=\"\",MoveType_22_07E95F2C41F3C9341B7904971492E67C=NewEnumerator0,ElementType_23_2FAF1B2B499571551749F6B39F4BC37D=NewEnumerator0,SubType_30_AE9CCCF34C44A8E40556BC935A44D0E8=NewEnumerator13,PhysicalSpecialStatus_8_5DC943EA407D54B86BB243AB74D2061F=NewEnumerator0,Damage_11_DDB65D3849CE29C5B91384868780960B=0.000000,StatusEffect_26_96750FA3440CC08E8E62D4B3652D80CF=(StatusEffectName_6_FA334B9A46A1625B9465C486DECB7109=\"\",StatusEffectType_18_502EF54F491DF29148F612953C32058B=NewEnumerator6,ChancetoActivate_29_0596FFD440B899CCBD8DD2B916E60F25=0.000000,StatusEffectDialogueText_7_EF66845C403B2941A9B0E48788D56C2D=\"\",StatusEffectSymbol_10_B772178E429378675266F495F7CB57D9=None,DamageOverType_21_2B1F28EA4CCA2CC5EF204AA0E2DBF95A=False,DOTDamage_27_E554A32045248BB7030520B5705802B6=0.000000,PreventsFromAttacking_23_5A5E14E44C3D17A7A3FE449E887CAB12=False),StatAffected_34_F783641C4EA304A29ABDDA945C1399E4=NewEnumerator0),Move2_6_1FDBAE674CB4AF337F4E52A5BEB44525=(MoveName_2_43F0BF544EAAF8A690427CB947E7131F=\"\",MoveType_22_07E95F2C41F3C9341B7904971492E67C=NewEnumerator0,ElementType_23_2FAF1B2B499571551749F6B39F4BC37D=NewEnumerator0,SubType_30_AE9CCCF34C44A8E40556BC935A44D0E8=NewEnumerator13,PhysicalSpecialStatus_8_5DC943EA407D54B86BB243AB74D2061F=NewEnumerator0,Damage_11_DDB65D3849CE29C5B91384868780960B=0.000000,StatusEffect_26_96750FA3440CC08E8E62D4B3652D80CF=(StatusEffectName_6_FA334B9A46A1625B9465C486DECB7109=\"\",StatusEffectType_18_502EF54F491DF29148F612953C32058B=NewEnumerator6,ChancetoActivate_29_0596FFD440B899CCBD8DD2B916E60F25=0.000000,StatusEffectDialogueText_7_EF66845C403B2941A9B0E48788D56C2D=\"\",StatusEffectSymbol_10_B772178E429378675266F495F7CB57D9=None,DamageOverType_21_2B1F28EA4CCA2CC5EF204AA0E2DBF95A=False,DOTDamage_27_E554A32045248BB7030520B5705802B6=0.000000,PreventsFromAttacking_23_5A5E14E44C3D17A7A3FE449E887CAB12=False),StatAffected_34_F783641C4EA304A29ABDDA945C1399E4=NewEnumerator0),Move3_7_BE0263184D8FD95A11746497F3836EE5=(MoveName_2_43F0BF544EAAF8A690427CB947E7131F=\"\",MoveType_22_07E95F2C41F3C9341B7904971492E67C=NewEnumerator0,ElementType_23_2FAF1B2B499571551749F6B39F4BC37D=NewEnumerator0,SubType_30_AE9CCCF34C44A8E40556BC935A44D0E8=NewEnumerator13,PhysicalSpecialStatus_8_5DC943EA407D54B86BB243AB74D2061F=NewEnumerator0,Damage_11_DDB65D3849CE29C5B91384868780960B=0.000000,StatusEffect_26_96750FA3440CC08E8E62D4B3652D80CF=(StatusEffectName_6_FA334B9A46A1625B9465C486DECB7109=\"\",StatusEffectType_18_502EF54F491DF29148F612953C32058B=NewEnumerator6,ChancetoActivate_29_0596FFD440B899CCBD8DD2B916E60F25=0.000000,StatusEffectDialogueText_7_EF66845C403B2941A9B0E48788D56C2D=\"\",StatusEffectSymbol_10_B772178E429378675266F495F7CB57D9=None,DamageOverType_21_2B1F28EA4CCA2CC5EF204AA0E2DBF95A=False,DOTDamage_27_E554A32045248BB7030520B5705802B6=0.000000,PreventsFromAttacking_23_5A5E14E44C3D17A7A3FE449E887CAB12=False),StatAffected_34_F783641C4EA304A29ABDDA945C1399E4=NewEnumerator0),Move4_8_3C9EA81B4DD2C43837432D9247CA531D=(MoveName_2_43F0BF544EAAF8A690427CB947E7131F=\"\",MoveType_22_07E95F2C41F3C9341B7904971492E67C=NewEnumerator0,ElementType_23_2FAF1B2B499571551749F6B39F4BC37D=NewEnumerator0,SubType_30_AE9CCCF34C44A8E40556BC935A44D0E8=NewEnumerator13,PhysicalSpecialStatus_8_5DC943EA407D54B86BB243AB74D2061F=NewEnumerator0,Damage_11_DDB65D3849CE29C5B91384868780960B=0.000000,StatusEffect_26_96750FA3440CC08E8E62D4B3652D80CF=(StatusEffectName_6_FA334B9A46A1625B9465C486DECB7109=\"\",StatusEffectType_18_502EF54F491DF29148F612953C32058B=NewEnumerator6,ChancetoActivate_29_0596FFD440B899CCBD8DD2B916E60F25=0.000000,StatusEffectDialogueText_7_EF66845C403B2941A9B0E48788D56C2D=\"\",StatusEffectSymbol_10_B772178E429378675266F495F7CB57D9=None,DamageOverType_21_2B1F28EA4CCA2CC5EF204AA0E2DBF95A=False,DOTDamage_27_E554A32045248BB7030520B5705802B6=0.000000,PreventsFromAttacking_23_5A5E14E44C3D17A7A3FE449E887CAB12=False),StatAffected_34_F783641C4EA304A29ABDDA945C1399E4=NewEnumerator0)),Battled_89_F480929841A407ED2344FA97712C4968=False)"))
      (Default|AssignPartyIDs (Variables|/Game/Blueprints/Avatar/BP_Character.BP_Character_C|GetMonsterRoster _asbp_character_2))
      (Default|SetOrder (Variables|/Game/Blueprints/Avatar/BP_Character.BP_Character_C|GetMonsterRoster _asbp_character_2)))))

(event Custom|LoadGame
  (bind _storagesystem (Variables|Default|GetStoragesystem))
  (bind _returnvalue (SaveGame|LoadGamefromSlot (Variables|Default|GetSave1)))
  (bind _asbp_save_game (Utilities|Casting|CastToBP_SaveGame _returnvalue))
  (Variables|Default|SetBeingLoaded true)
  (Game|OpenLevel(byName) (Utilities|String|StringToName (Variables|/Game/Blueprints/SaveLoad/BP_SaveGame.BP_SaveGame_C|GetLevelName _asbp_save_game)) false)
  (bind _asbp_character (Utilities|Casting|CastToBP_Character (Game|GetPlayerCharacter 0)))
  (Transformation|SetActorTransform _asbp_character (Variables|/Game/Blueprints/SaveLoad/BP_SaveGame.BP_SaveGame_C|GetPlayerTransform _asbp_save_game))
  (Utilities|IsValid _storagesystem
    (:Is%20Valid
      (Variables|/Game/Blueprints/InventorySystem/BP_MonsterStorage.BP_MonsterStorage_C|SetMonsters _storagesystem (Variables|/Game/Blueprints/SaveLoad/BP_SaveGame.BP_SaveGame_C|GetMonsterStruct _asbp_save_game))
      (Variables|/Game/Blueprints/InventorySystem/BP_Inventory.BP_Inventory_C|SetStructInventory (Variables|/Game/Blueprints/Avatar/BP_Character.BP_Character_C|GetBP_Inventory _asbp_character) (Variables|/Game/Blueprints/SaveLoad/BP_SaveGame.BP_SaveGame_C|GetInventory _asbp_save_game))
      (Variables|/Game/Blueprints/MonsterAssets/BP_Component_MonsterRoster.BP_Component_MonsterRoster_C|SetMonsterRosterStruct (Variables|/Game/Blueprints/Avatar/BP_Character.BP_Character_C|GetMonsterRoster _asbp_character) (Variables|/Game/Blueprints/SaveLoad/BP_SaveGame.BP_SaveGame_C|GetMonsterRoster _asbp_save_game))
      (Default|SetOrder (Variables|/Game/Blueprints/Avatar/BP_Character.BP_Character_C|GetMonsterRoster _asbp_character)))))

(event Custom|RestartLevel
  (SaveGame|DeleteGameinSlot (Variables|Default|GetSave1))
  (Development|ExecuteConsoleCommand "RestartLevel" 0))

(event Custom|Load%20Storage%20System
  (bind _storagesystem (Variables|Default|GetStoragesystem))
  (bind _returnvalue (SaveGame|LoadGamefromSlot (Variables|Default|GetSave1)))
  (bind _asbp_save_game (Utilities|Casting|CastToBP_SaveGame _returnvalue))
  (Variables|Default|SetAs%20BP%20Save%20Game _asbp_save_game)
  (bind _asbp_character (Utilities|Casting|CastToBP_Character (Game|GetPlayerCharacter 0)))
  (Transformation|SetActorTransform _asbp_character (Variables|/Game/Blueprints/SaveLoad/BP_SaveGame.BP_SaveGame_C|GetPlayerTransform (Variables|Default|GetAs%20BP%20Save%20Game)))
  (Variables|/Game/Blueprints/InventorySystem/BP_Inventory.BP_Inventory_C|SetStructInventory (Variables|/Game/Blueprints/Avatar/BP_Character.BP_Character_C|GetBP_Inventory _asbp_character) (Variables|/Game/Blueprints/SaveLoad/BP_SaveGame.BP_SaveGame_C|GetInventory (Variables|Default|GetAs%20BP%20Save%20Game)))
  (Variables|/Game/Blueprints/MonsterAssets/BP_Component_MonsterRoster.BP_Component_MonsterRoster_C|SetMonsterRosterStruct (Variables|/Game/Blueprints/Avatar/BP_Character.BP_Character_C|GetMonsterRoster _asbp_character) (Variables|/Game/Blueprints/SaveLoad/BP_SaveGame.BP_SaveGame_C|GetMonsterRoster (Variables|Default|GetAs%20BP%20Save%20Game)))
  (Default|SetOrder (Variables|/Game/Blueprints/Avatar/BP_Character.BP_Character_C|GetMonsterRoster _asbp_character))
  (Utilities|IsValid _storagesystem
    (:Is%20Valid
      (Variables|/Game/Blueprints/InventorySystem/BP_MonsterStorage.BP_MonsterStorage_C|SetMonsters _storagesystem (Variables|/Game/Blueprints/SaveLoad/BP_SaveGame.BP_SaveGame_C|GetMonsterStruct (Variables|Default|GetAs%20BP%20Save%20Game)))
      (Variables|Default|SetBeingLoaded false))
    (:Is%20Not%20Valid
      (Development|PrintString "Not valid NG" true true "(R=0.000000,G=0.660000,B=1.000000,A=1.000000)" 1e+01))))

(event Custom|CustomEvent:%20Tick
  (params (DeltaSeconds :type Float%20%28single-precision%29))
  ;[1 1 1] Timer Setup: Countdown (Failed)
)

(fn PlayMusic
  (params (VolumeMultiplier :type Float%20%28single-precision%29) (bPersistAcrossLevelTransition :type Boolean) (Sound :type Sound%20Base%20Object%20Reference))
  (bind _returnvalue (Audio|CreateSound2D Sound VolumeMultiplier 1.0 0.0 0 bPersistAcrossLevelTransition false))
  (bind _output_get (Variables|Default|SetMusic _returnvalue))
  (Audio|Components|Audio|Play _output_get 0.0))

(fn StopMusic
  (Audio|Components|Audio|Stop (Variables|Default|GetMusic)))

(fn FadeOut
  (Audio|Components|Audio|FadeOut (Variables|Default|GetMusic) 2.0 0.1 "Linear" :!class /Script/Engine.AudioComponent)
  (bind _returnvalue (Utilities|Time|SetTimerbyEvent (EventDispatchers|CreateEvent :!event Fadein) 2.0))
  (Variables|Default|SetFadeOutTimer _returnvalue))

(fn SwitchMusic
  (params (NewSound :type Sound%20Base%20Object%20Reference) (Fading :type Boolean))
  (bind _output_get (Variables|Default|SetNew%20Sound NewSound))
  (if (not Fading)
    (Audio|Components|Audio|SetSound (Variables|Default|GetMusic) _output_get)))

(fn PlaySoundFX
  (params (Sound :type Sound%20Base%20Object%20Reference))
  (bind _returnvalue (Audio|CreateSound2D Sound (Variables|Default|GetSoundVolume) 1.0 0.0 0))
  (bind _output_get (Variables|Default|SetSoundFXComponent _returnvalue))
  (Audio|Components|Audio|Play _output_get 0.0))

(fn Fadein
  (bind _music (Variables|Default|GetMusic))
  (Audio|Components|Audio|SetSound _music (Variables|Default|GetNew%20Sound))
  (Audio|Components|Audio|FadeIn _music 1.0 (Variables|Default|GetMusicVolume) 0.0 "Linear" :!class /Script/Engine.AudioComponent))