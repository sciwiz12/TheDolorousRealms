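; Moving platform that travels toward an end point when a BP_Character enters its PlayerTouch trigger.
; BeginPlay caches Platform and EndPoint world locations and sets the play rate; the Platform_Move timeline lerps between them, applying the result as a relative location.
; Entering also applies a glow material and plays a whoosh.
; Leaving restores the brown material and clears sound mix modifiers, without reversing the timeline.
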(event OnComponentBeginOverlap(PlayerTouch)
  (params (OverlappedComponent :type Primitive%20Component%20Object%20Reference) (OtherActor :type Actor%20Object%20Reference) (OtherComp :type Primitive%20Component%20Object%20Reference) (OtherBodyIndex :type Integer) (bFromSweep :type Boolean) (SweepResult :type Hit%20Result%20Structure%20%28by%20ref%29))
  (Utilities|Casting|CastToBP_Character OtherActor)
  (Rendering|Material|SetMaterial (Variables|Default|GetPlatform) 0 "/Game/ArtAssets/Materials/Mat_glow.Mat_glow")
  (Audio|PlaySound2D "/Game/AudioAssets/SFX/woosh_low_long01-98755.woosh_low_long01-98755" 1.0 1.0 0.0 0 0)
  (bind _newtrack_0 (Timeline|Platform_Move Play)
    (:Update
      (Transformation|SetRelativeLocation (Variables|Default|GetPlatform) (Math|Vector|Lerp(Vector) (Variables|Default|GetStart_Loc) (Variables|Default|GetEnd_Loc) _newtrack_0) false false))))

(event OnComponentEndOverlap(PlayerTouch)
  (params (OverlappedComponent :type Primitive%20Component%20Object%20Reference) (OtherActor :type Actor%20Object%20Reference) (OtherComp :type Primitive%20Component%20Object%20Reference) (OtherBodyIndex :type Integer))
  (Utilities|Casting|CastToBP_Character OtherActor)
  (Rendering|Material|SetMaterial (Variables|Default|GetPlatform) 0 "/Game/ArtAssets/Textures/Colors/Brown_color.Brown_color")
  (Class|GameplayStatics|ClearSoundMixModifiers))

(event EventBeginPlay
  (CallFunction|SetLocations))

(fn ConstructionScript)

(fn SetLocations
  (Variables|Default|SetStart_Loc (Transformation|GetWorldLocation (Variables|Default|GetPlatform)))
  (Variables|Default|SetEnd_Loc (Transformation|GetWorldLocation (Variables|Default|GetEnd_Point)))
  (Components|Timeline|SetPlayRate (Variables|Default|GetPlatform_Move) (Variables|Default|GetPlayRate)))