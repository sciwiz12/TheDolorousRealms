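; BP_Door is a Paper2D door that opens when a BP_Character overlaps its trigger box, optionally requiring a key.
; If locked, it checks the character's KeyRing for KeyNeeded and prints a "Find Key" message when it is missing.
; Opening plays the flipbook once and disables collision on Box1, with no closing logic.
; Disconnected inventory item nodes remain in the graph and never run.
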(event OnComponentBeginOverlap(Box)
  (params (OverlappedComponent :type Primitive%20Component%20Object%20Reference) (OtherActor :type Actor%20Object%20Reference) (OtherComp :type Primitive%20Component%20Object%20Reference) (OtherBodyIndex :type Integer) (bFromSweep :type Boolean) (SweepResult :type Hit%20Result%20Structure%20%28by%20ref%29))
  (bind _asbp_character (Utilities|Casting|CastToBP_Character OtherActor))
  (if (Variables|Default|GetLocked?)
    (if (Utilities|Array|ContainsItem (Variables|/Game/Blueprints/Avatar/BP_Character.BP_Character_C|GetKeyRing _asbp_character) (Variables|Default|GetKeyNeeded))
      (CallFunction|OpenDoor)
      (Variables|Default|SetDoorOpen? true)
      (else
        (Development|PrintString "Find Key")))
    (else
      (CallFunction|OpenDoor))))

(event OnComponentEndOverlap(Box)
  (params (OverlappedComponent :type Primitive%20Component%20Object%20Reference) (OtherActor :type Actor%20Object%20Reference) (OtherComp :type Primitive%20Component%20Object%20Reference) (OtherBodyIndex :type Integer)))

(event Custom|OpenDoor
  (Components|Timeline|SetPlayRate (Variables|Default|GetPaperFlipbook) 1.0)
  (Components|Timeline|SetLooping (Variables|Default|GetPaperFlipbook) false)
  (Collision|SetCollisionEnabled (Variables|Default|GetBox1) "NoCollision"))

(event EventBeginPlay)

(event Collision|EventActorBeginOverlap
  (params (OtherActor :type Actor%20Object%20Reference)))

(event EventTick
  (params (DeltaSeconds :type Float%20%28single-precision%29)))

(fn ConstructionScript)