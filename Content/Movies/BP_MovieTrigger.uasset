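; BP_MovieTrigger is a trigger actor that plays a movie in a fullscreen-style widget when the player character enters it.
; On collision overlap with a BP_Character, it checks for an existing top-level GUI_Movies widget and creates one only if none is present.
; It passes its MediaPlayer, MediaSource and Material to the new widget before adding it to the viewport.
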(event OnComponentBeginOverlap(CollisionComponent)
  (params (OverlappedComponent :type Primitive%20Component%20Object%20Reference) (OtherActor :type Actor%20Object%20Reference) (OtherComp :type Primitive%20Component%20Object%20Reference) (OtherBodyIndex :type Integer) (bFromSweep :type Boolean) (SweepResult :type Hit%20Result%20Structure%20%28by%20ref%29))
  (Utilities|Casting|CastToBP_Character OtherActor)
  (bind _foundwidgets (Widget|GetAllWidgetsOfClass "/Game/Blueprints/GUIs/GUI_Movies.GUI_Movies_C" true))
  (Utilities|IsValid (Utilities|Array|Get(acopy) _foundwidgets)
    (:Is%20Not%20Valid
      (bind _returnvalue (UserInterface|CreateWidget "/Game/Blueprints/GUIs/GUI_Movies.GUI_Movies_C" (Game|GetPlayerController 0)))
      (Variables|/Game/Blueprints/GUIs/GUI_Movies.GUI_Movies_C|SetMediaPlayer _returnvalue (Variables|Default|GetMediaPlayer))
      (Variables|/Game/Blueprints/GUIs/GUI_Movies.GUI_Movies_C|SetMedia%20Source _returnvalue (Variables|Default|GetMedia%20Source))
      (Variables|/Game/Blueprints/GUIs/GUI_Movies.GUI_Movies_C|SetMaterial _returnvalue (Variables|Default|GetMaterial))
      (UserInterface|Viewport|AddtoViewport _returnvalue 0))))

(event EventBeginPlay)

(event Collision|EventActorBeginOverlap
  (params (OtherActor :type Actor%20Object%20Reference)))

(event EventTick
  (params (DeltaSeconds :type Float%20%28single-precision%29)))

(fn ConstructionScript)