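; BP_TimerMode is a work-in-progress countdown timer prototype, meant to lead to a lose screen when time runs out.
; Only Tick does any work, printing a timer's remaining time every frame, though no live code starts a timer.
; Disconnected experiments hold minute/second countdowns, a timer event, the timer widget and a bad-end screen that pauses the game.
; GoToLoseScreen is an empty stub with its logic left unwired.
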(event EventTick
  (params (DeltaSeconds :type Float%20%28single-precision%29))
  ;[1 1 1] Timer Ver 3.0
  (|CallParentFunction DeltaSeconds)
  (Development|PrintString (Utilities|String|ToString(Float) (Utilities|Time|GetTimerRemainingTimebyHandle))))

(event EventBeginPlay
  ;[1 1 1] Timer Ver 3.0
)

(fn ConstructionScript)

(fn GotoLoseScreen)