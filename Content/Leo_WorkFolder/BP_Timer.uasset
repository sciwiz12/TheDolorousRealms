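; BP_Timer is an actor that serves as a level countdown, apparently triggering the lose condition when time runs out.
; BeginPlay starts a one-shot five-minute timer and stores its handle, though the delegate's target function is not shown.
; GoToLoseScreen, the likely callback, displays the GUI_BadEnd widget, shows the mouse cursor and pauses the game.
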(event Collision|EventActorBeginOverlap
  (params (OtherActor :type Actor%20Object%20Reference)))

(event EventTick
  (params (DeltaSeconds :type Float%20%28single-precision%29))
  (|CallParentFunction DeltaSeconds))

(event EventBeginPlay
  (bind _returnvalue (Utilities|Time|SetTimerbyEvent (EventDispatchers|CreateEvent :!event GotoLoseScreen) 3e+02))
  (bind _output_get (Variables|Default|SetTimer _returnvalue)))

(fn ConstructionScript)

(fn GotoLoseScreen
  (bind _returnvalue (UserInterface|CreateWidget "/Game/Blueprints/GUIs/GUI_BadEnd.GUI_BadEnd_C"))
  (UserInterface|Viewport|AddtoViewport _returnvalue 0)
  (Variables|/Script/Engine.PlayerController|SetbShowMouseCursor (Game|GetPlayerController 0) true)
  (Game|SetGamePaused true))