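; Level manager for the Greed level (Level 4) that places the player character when play begins.
; On BeginPlay it runs the parent logic, then casts the first player's character to BP_Character.
; It moves that character to the manager's own location without sweeping and applies a fixed rotation, so the manager actor doubles as the spawn marker.
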(event EventBeginPlay
  (|CallParentFunction)
  (bind _asbp_character (Utilities|Casting|CastToBP_Character (Game|GetPlayerCharacter 0)))
  (Transformation|SetActorLocation _asbp_character (Transformation|GetActorLocation self) false false)
  (Transformation|SetActorRotation _asbp_character "0,180.000000, 0"))

(event Collision|EventActorBeginOverlap
  (params (OtherActor :type Actor%20Object%20Reference))
  (|CallParentFunction OtherActor) ; This node is disabled and will not be called.\nDrag off pins to build functionality.
)

(event EventTick
  (params (DeltaSeconds :type Float%20%28single-precision%29))
  (|CallParentFunction DeltaSeconds) ; This node is disabled and will not be called.\nDrag off pins to build functionality.
)

(fn ConstructionScript
  (|CallParentFunction))