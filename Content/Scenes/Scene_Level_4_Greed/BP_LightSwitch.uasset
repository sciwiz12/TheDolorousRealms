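; BP_LightSwitch is an interactable switch in the Greed level scene that toggles a red light with the E key.
; A box overlap with BP_Character shows a text prompt and enables input for player 0, and leaving hides the prompt and disables input.
; Each press plays a select sound, toggles the light's visibility and flips IsOn, with both branches making the same toggle call.
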(event OnComponentBeginOverlap(Box)
  (params (OverlappedComponent :type Primitive%20Component%20Object%20Reference) (OtherActor :type Actor%20Object%20Reference) (OtherComp :type Primitive%20Component%20Object%20Reference) (OtherBodyIndex :type Integer) (bFromSweep :type Boolean) (SweepResult :type Hit%20Result%20Structure%20%28by%20ref%29))
  (Utilities|Casting|CastToBP_Character OtherActor)
  (Rendering|SetVisibility (Variables|Default|GetTextRender) true false)
  (Input|EnableInput (Game|GetPlayerController 0)))

(event OnComponentEndOverlap(Box)
  (params (OverlappedComponent :type Primitive%20Component%20Object%20Reference) (OtherActor :type Actor%20Object%20Reference) (OtherComp :type Primitive%20Component%20Object%20Reference) (OtherBodyIndex :type Integer))
  (Utilities|Casting|CastToBP_Character OtherActor)
  (Rendering|SetVisibility (Variables|Default|GetTextRender) false false)
  (Input|DisableInput (Game|GetPlayerController 0)))

(event Input|KeyboardEvents|E
  (params (Key :type Key%20Structure :default "None"))
  (:Pressed
    (if (Variables|Default|GetisOn?)
      (Audio|PlaySound2D "/Game/AudioAssets/SoundEffects/Select.Select" 1.0 1.0 0.0 0 0)
      (Rendering|ToggleVisibility (Variables|/Script/Engine.Light|GetLightComponent (Variables|Default|GetRedLight)) false)
      (Variables|Default|SetisOn? false)
      (else
        (Audio|PlaySound2D "/Game/AudioAssets/SoundEffects/Select.Select" 1.0 1.0 0.0 0 0)
        (Rendering|ToggleVisibility (Variables|/Script/Engine.Light|GetLightComponent (Variables|Default|GetRedLight)) false)
        (Variables|Default|SetisOn? true)))))

(fn ConstructionScript)